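; Falling particle sprite actor that drifts down from its spawn point and destroys itself when done.
; On BeginPlay it jitters its start position, picks one of four flower particle sprites at random and plays the FallWave timeline at half speed.
; Each update sets a swept location from that start, combining the timeline's height track with a rotated, horizontally scaled flutter vector.
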(event EventBeginPlay
  (Variables|Default|SetInitPos (+ (Transformation|GetActorLocation) (Math|Vector|MakeVector (Math|Random|RandomFloatinRange -8.0 7.0) (Math|Random|RandomFloatinRange -4.0 3.0) -2.0)))
  (Components|Timeline|SetPlayRate (Variables|Default|GetFallWave) 0.5)
  (Rendering|Components|Sprite|SetSprite (Variables|Default|GetRenderComponent) (Utilities|Select :Index (Math|Random|RandomIntegerinRange 0 3) :Option%200 "/Game/Assets/Textures/T_FlowerParticles_Sprite_0.T_FlowerParticles_Sprite_0" :Option%201 "/Game/Assets/Textures/T_FlowerParticles_Sprite_1.T_FlowerParticles_Sprite_1" :Option%202 "/Game/Assets/Textures/T_FlowerParticles_Sprite_2.T_FlowerParticles_Sprite_2" :Option%203 "/Game/Assets/Textures/T_FlowerParticles_Sprite_3.T_FlowerParticles_Sprite_3"))
  (bind (_direction _flutter_down _z) (Timeline|FallWave PlayFromStart)
    (:Update
      (Transformation|SetActorLocation (+ (Variables|Default|GetInitPos) (* (Math|Vector|RotateVector _flutter_down "0,90.000000, 0") "64.000000,64.000000,0.000000") (Math|Vector|MakeVector 0.0 0.0 _z)) true false))
    (:Finished
      (Actor|DestroyActor))))

(fn ConstructionScript)