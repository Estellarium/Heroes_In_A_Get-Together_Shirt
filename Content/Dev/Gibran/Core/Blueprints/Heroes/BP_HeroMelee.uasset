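; Melee hero Blueprint whose primary action performs a short-range attack, gated by the Ability 1 cooldown.
; Action1 spawns a BP_MeleeAttack at the shooting component, triggers it with Attack1Data, then starts the cooldown.
; It also spawns a one-shot flipbook BP_SpriteVFX at the Arrow, randomly mirrored on X for variety.
; Tick draws a debug cone from the shooting component, with both debug-mode check branches left empty.
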(event EventBeginPlay
  (|CallParentFunction) ; This node is disabled and will not be called.\nDrag off pins to build functionality.
)

(event Collision|EventActorBeginOverlap
  (params (OtherActor :type Actor%20Object%20Reference)))

(event EventTick
  (params (DeltaSeconds :type Float%20%28single-precision%29))
  (bind _bp_shooting_component (Variables|Default|GetBP_Shooting_Component))
  (|CallParentFunction DeltaSeconds)
  (Utilities|IsDebugModeOn?
    (:Debug%20Mode%20On
      _)
    (:Debug%20Mode%20Off
      _))
  (Class|KismetSystemLibrary|DrawDebugConeinDegrees (Transformation|GetWorldLocation _bp_shooting_component) (Math|Vector|GetForwardVector _bp_shooting_component) 1.2e+02 9e+01 45.0 12 "(R=1.000000,G=0.000000,B=0.365907,A=1.000000)" 0.0 3.0))

(event EventAction1
  (bind _arrow (Variables|Default|GetArrow))
  (bind _bp_shooting_component (Variables|Default|GetBP_Shooting_Component))
  (if (not (Variables|Default|GetInAbility1Cooldown))
    (bind _returnvalue (Game|SpawnActorfromClass "/Game/Dev/Gibran/Core/Blueprints/BP_MeleeAttack.BP_MeleeAttack_C" (Math|Transform|MakeTransform (Transformation|GetWorldLocation _bp_shooting_component) (Math|Rotator|MakeRotator 0.0 0.0 (.yaw (Transformation|GetWorldRotation _bp_shooting_component))) "2.000000,2.000000,1.000000") "AlwaysSpawn" 0 0))
    (Default|TriggerAttack _returnvalue (Variables|Default|GetAttack1Data))
    (bind _returnvalue_2 (Game|SpawnActorfromClass "/Game/Dev/Gibran/Core/Blueprints/BP_SpriteVFX.BP_SpriteVFX_C" (Math|Transform|MakeTransform (Transformation|GetWorldLocation _arrow) (Math|Rotator|MakeRotator 0.0 0.0 (.yaw (Transformation|GetWorldRotation _arrow))) (Math|Vector|MakeVector (Math|Float|SelectFloat 1.0 -1.0 (Math|Random|RandomBool)) 1.0 1.0)) "Undefined" 0 0))
    (Default|TriggerEffect(Flipbook) _returnvalue_2 "/Game/Dev/Gibran/TestAssets/Flipbooks/VFX/3_2.3_2" 1.0 false)
    (CallFunction|StartAbility1Cooldown)))

(fn ConstructionScript
  (|CallParentFunction))