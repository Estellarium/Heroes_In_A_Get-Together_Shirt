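; Playable hero Blueprint for Ben, a support character who interacts with objects and heals the hero group.
; While not fainted, Tick sphere-traces ahead of the shooting component for BPI_InteractableObject actors, tracking the focused one and showing its prompt widget.
; Action1 triggers the focused actor's interaction and starts its cooldown.
; Action2 heals the group, more strongly when Enhanced, plays the healing animation, starts its cooldown and records the heal stat.
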(event Custom|Interact
  (bind _focusedinteractableactor (Variables|Default|GetFocusedInteractableActor))
  ;[1 1 1] Interaction with objects
  (Utilities|IsValid _focusedinteractableactor
    (:Is%20Valid
      (Class|BPIInteractableObject|Interact(Message) _focusedinteractableactor self))))

(event Custom|UnfocusInteractable
  (bind _interactionpromptwidget (Variables|Default|GetInteractionPromptWidget))
  ;[1 1 1] Interaction with objects
  (Utilities|IsValid _interactionpromptwidget
    (:Is%20Valid
      (Widget|RemovefromParent _interactionpromptwidget))
    (:Is%20Not%20Valid
      _))
  (Variables|Default|SetFocusedInteractableActor 0))

(event EventTick
  (params (DeltaSeconds :type Float%20%28single-precision%29))
  (bind _bp_shooting_component (Variables|Default|GetBP_Shooting_Component))
  (bind _returnvalue (Transformation|GetWorldLocation _bp_shooting_component))
  (|CallParentFunction DeltaSeconds)
  (if (not (Variables|Default|GetFainted))
    ;[1 1 1] Interaction with objects
    (bind (_outhit _returnvalue_2) (Collision|SphereTraceForObjects _returnvalue (+ _returnvalue (* (Math|Vector|GetForwardVector _bp_shooting_component) 3e+02)) 2e+01 (Utilities|Array|MakeArray "ObjectTypeQuery1" "ObjectTypeQuery2") false (Utilities|Array|MakeArray self (Variables|Default|GetHeroGroupRef)) "None"))
    (if _returnvalue_2
      (if (Utilities|DoesObjectImplementInterface (.HitActor (Collision|BreakHitResult _outhit)) "/Game/Dev/Gibran/Core/Interfaces/BPI_InteractableObject.BPI_InteractableObject_C")
        (if (not (== (.HitActor (Collision|BreakHitResult _outhit)) (Variables|Default|GetFocusedInteractableActor)))
          (Utilities|IsValid (Variables|Default|GetInteractionPromptWidget)
            (:Is%20Valid
              (Widget|RemovefromParent (Variables|Default|GetInteractionPromptWidget)))
            (:Is%20Not%20Valid
              _))
          (Variables|Default|SetFocusedInteractableActor (.HitActor (Collision|BreakHitResult _outhit)))
          (bind _returnvalue_3 (UserInterface|CreateWidget "/Game/Dev/Gibran/Core/UI/HUD/WBP_InteractionPromptBase.WBP_InteractionPromptBase_C"))
          (bind _output_get (Variables|Default|SetInteractionPromptWidget _returnvalue_3))
          (UserInterface|Viewport|AddtoViewport _output_get 0)
          (bind (_prompttext _promptimage) (Class|BPIInteractableObject|GetInteractionPrompt(Message) (.HitActor (Collision|BreakHitResult _outhit))))
          (Default|SetPromptData _returnvalue_3 _prompttext _promptimage))
        (else
          (Utilities|IsValid (Variables|Default|GetInteractionPromptWidget) :!label _label
            (:Is%20Valid
              (Widget|RemovefromParent (Variables|Default|GetInteractionPromptWidget)))
            (:Is%20Not%20Valid
              _))
          (Variables|Default|SetFocusedInteractableActor 0)))
      (else
        (goto _label)))))

(event EventAction1
  (Utilities|IsValid (Variables|Default|GetFocusedInteractableActor)
    (:Is%20Valid
      (CallFunction|Interact)
      (CallFunction|StartAbility1Cooldown))))

(event EventAction2
  (bind _herogroupref (Variables|Default|GetHeroGroupRef))
  (if (Variables|Default|GetEnhanced)
    (Default|TakeGroupHealing _herogroupref 5e+01)
    (else
      (Default|TakeGroupHealing _herogroupref 1e+01)))
  (Default|ExecuteAnimation (Variables|Default|GetBP_SpriteAnimationComponent) "/Game/Dev/Gibran/TestAssets/Flipbooks/Characters/Ben_Healing.Ben_Healing")
  (CallFunction|StartAbility2Cooldown)
  (Default|AddStatBenHeals (Variables|Default|GetGameInstanceRef)))

(event EventStartEnhancement
  (Class|Image|SetBrushResourceObject (Variables|/Game/Dev/Gibran/Core/UI/HUD/WBP_EnhancementMeter.WBP_EnhancementMeter_C|GetEnhacementIcon (Variables|Default|GetEnhancementMeterRef)) "/Game/Dev/Gibran/TestAssets/Sprites/UI/Icons/Icon_Heal.Icon_Heal"))

(event EventEndEnhancement)

(fn ConstructionScript
  (|CallParentFunction))