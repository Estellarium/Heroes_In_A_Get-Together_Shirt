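; Base class for heroes in a hero group, providing health, damage, healing, fainting, two ability cooldowns and timed enhancement pickups, with actions and enhancement effects left to child classes.
; Separate torso and legs flipbooks are fed to a sprite animation component and show color flashes and a timeline-driven faint rotation.
; Damage passes a shield overlap check and hit cooldown, then health changes update the group total.
; Timelines rescaled to durations drive cooldowns and the enhancement meter.
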(event Custom|TriggerHeroEnhancement
  (params (Duration :type Float%20%28double-precision%29))
  ;[0 0 0] Enhancement Pickup
  (if (not (Variables|PowerUp|GetEnhanced))
    (Variables|PowerUp|SetEnhanced true)
    (CallFunction|TimelinePlayrateinSeconds (Variables|Default|GetEnhancementTimeline) Duration)
    (bind _meter (Default|CreateMeter (Variables|/Game/Dev/Gibran/Core/Blueprints/Heroes/BP_HeroGroup.BP_HeroGroup_C|GetEnhancementsRef (Variables|Default|GetHeroGroupRef)) (Variables|PowerUp|GetEnhancementColor)))
    (Variables|PowerUp|SetEnhancementMeterRef _meter)
    (CallFunction|StartEnhancement)
    (bind _duration (Timeline|EnhancementTimeline PlayFromStart)
      (:Update
        (Progress|SetPercent (Variables|/Game/Dev/Gibran/Core/UI/HUD/WBP_EnhancementMeter.WBP_EnhancementMeter_C|GetEnhancementTime (Variables|PowerUp|GetEnhancementMeterRef)) _duration))
      (:Finished
        (Default|EndMeter (Variables|PowerUp|GetEnhancementMeterRef))
        (Variables|PowerUp|SetEnhancementMeterRef 0)
        (Variables|PowerUp|SetEnhanced false)
        (CallFunction|EndEnhancement)))))

(event Custom|EndEnhancement
  ;[0 0 0] Override in child
)

(event Custom|StartAbility1Cooldown
  ;[0 0 0] Ability Cooldowns
  (CallFunction|TimelinePlayrateinSeconds (Variables|Default|GetAbility1CooldownTm) (Variables|Abilities|GetAbility1Cooldown))
  (Variables|Abilities|SetInAbility1Cooldown true)
  (bind _cooldownprogress (Timeline|Ability1CooldownTm PlayFromStart)
    (:Update
      (Variables|Abilities|SetAbility1CooldownProgress _cooldownprogress))
    (:Finished
      (Variables|Abilities|SetInAbility1Cooldown false))))

(event Custom|StartEnhancement
  ;[0 0 0] Override in child
)

(event Custom|Faint
  (bind _torsoflipbook (Variables|Default|GetTorsoFlipbook))
  (bind _legsflipbook (Variables|Default|GetLegsFlipbook))
  ;[0.08854 0 0] Fainting
  (Variables|Health|SetFainted true)
  (Sprite|SetSpriteColor _torsoflipbook "(R=0.000000,G=0.000000,B=0.000000,A=1.000000)")
  (Audio|Components|Audio|Stop _torsoflipbook)
  (Sprite|SetSpriteColor _legsflipbook "(R=0.000000,G=0.000000,B=0.000000,A=1.000000)")
  (Audio|Components|Audio|Stop _legsflipbook)
  (Default|UpdateTotalHealth (Variables|Default|GetHeroGroupRef))
  (Default|AddStatHeroFainted (CallFunction|GetHeroesGameInstance))
  (bind _rotation (Timeline|FaintTimeline Play)
    (:Update
      (Variables|Health|SetFaintRotation _rotation))))

(event Custom|Action1
  ;[0 0 0] Actions to be implemented by child classes
)

(event Custom|Action2
  ;[0 0 0] Actions to be implemented by child classes
)

(event Custom|ReceiveHealing
  (params (HealAmmount :type Float%20%28double-precision%29))
  ;[0 0 0] Receiving Healing
  (Variables|Health|SetHealth (Math|Float|Clamp(Float) (+ (Variables|Health|GetHealth) HealAmmount) 0.0 (Variables|Health|GetMaxHealth)))
  (Utilities|FlipbookColorFlash (Variables|Default|GetTorsoFlipbook) "(R=0.260107,G=1.000000,B=0.000000,A=1.000000)" 0.2
    (:__
      (Utilities|FlipbookColorFlash (Variables|Default|GetLegsFlipbook) "(R=0.260107,G=1.000000,B=0.000000,A=1.000000)" 0.2
        (:__
          (Default|UpdateTotalHealth (Variables|Default|GetHeroGroupRef))
          (if (Variables|Health|GetFainted)
            (CallFunction|Unfaint)))))))

(event Custom|Unfaint
  (bind _torsoflipbook (Variables|Default|GetTorsoFlipbook))
  (bind _legsflipbook (Variables|Default|GetLegsFlipbook))
  ;[0.08854 0 0] Fainting
  (Variables|Health|SetFainted false)
  (Sprite|SetSpriteColor _torsoflipbook "(R=1.000000,G=1.000000,B=1.000000,A=1.000000)")
  (Audio|Components|Audio|Play _torsoflipbook)
  (Sprite|SetSpriteColor _legsflipbook "(R=1.000000,G=1.000000,B=1.000000,A=1.000000)")
  (Audio|Components|Audio|Play _legsflipbook)
  (Default|UpdateTotalHealth (Variables|Default|GetHeroGroupRef))
  (bind _rotation (Timeline|FaintTimeline Reverse)
    (:Update
      (Variables|Health|SetFaintRotation _rotation))))

(event Custom|StartAbility2Cooldown
  ;[0 0 0] Ability Cooldowns
  (CallFunction|TimelinePlayrateinSeconds (Variables|Default|GetAbility2CooldownTm) (Variables|Abilities|GetAbility2Cooldown))
  (Variables|Abilities|SetInAbility2Cooldown true)
  (bind _cooldownprogress (Timeline|Ability2CooldownTm PlayFromStart)
    (:Update
      (Variables|Abilities|SetAbility2CooldownProgress _cooldownprogress))
    (:Finished
      (Variables|Abilities|SetInAbility2Cooldown false))))

(event EventBeginPlay
  (bind _bp_spriteanimationcomponent (Variables|Default|GetBP_SpriteAnimationComponent))
  ;[0.0625 0.0625 0.0625] Begin Play
  (Utilities|FlowControl|Sequence
    (:then_0
      (Variables|Default|SetGameModeRef (CallFunction|GetHeroesGameMode))
      (Variables|Default|SetGameInstanceRef (CallFunction|GetHeroesGameInstance)))
    (:then_1
      (Rendering|Components|TextRender|SetText (Variables|Default|GetNumberText) (Utilities|Text|ToText(Integer) (Variables|Default|GetNumber)))
      (Rendering|Components|Sprite|SetSprite (Variables|Default|GetIcon) (Variables|Default|GetIconTxt))
      (Sprite|SetFlipbook (Variables|Default|GetTorsoFlipbook) (Variables|Default|GetIdleFlipbook))
      (Sprite|SetFlipbook (Variables|Default|GetLegsFlipbook) (Variables|Default|GetRunFlipbook))
      (Variables|Health|SetHealth (Variables|Health|GetMaxHealth)))
    (:then_2
      (Variables|/Game/Dev/Gibran/Core/Blueprints/Components/BP_SpriteAnimationComponent.BP_SpriteAnimationComponent_C|SetTorsoFlipbookRef _bp_spriteanimationcomponent (Variables|Default|GetTorsoFlipbook))
      (Variables|/Game/Dev/Gibran/Core/Blueprints/Components/BP_SpriteAnimationComponent.BP_SpriteAnimationComponent_C|SetLegsFlipbookRef _bp_spriteanimationcomponent (Variables|Default|GetLegsFlipbook))
      (Variables|/Game/Dev/Gibran/Core/Blueprints/Components/BP_SpriteAnimationComponent.BP_SpriteAnimationComponent_C|SetActorRef _bp_spriteanimationcomponent self)
      (CallFunction|StartAbility1Cooldown)
      (CallFunction|StartAbility2Cooldown))))

(event EventTick
  (params (DeltaSeconds :type Float%20%28single-precision%29))
  (bind _faintrotation (Variables|Health|GetFaintRotation))
  (bind _torsoflipbook (Variables|Default|GetTorsoFlipbook))
  (bind _capsule (Variables|Default|GetCapsule))
  (bind _legsflipbook (Variables|Default|GetLegsFlipbook))
  (bind _bp_spriteanimationcomponent (Variables|Default|GetBP_SpriteAnimationComponent))
  (bind _returnvalue (Transformation|GetWorldRotation _torsoflipbook))
  (bind _returnvalue_2 (Transformation|GetWorldRotation _legsflipbook))
  (bind _returnvalue_3 (+ 0.0 _faintrotation))
  ;[0.0625 0.0625 0.0625] Tick
  (Transformation|SetWorldRotation _torsoflipbook (Math|Rotator|MakeRotator (.roll _returnvalue) (.pitch _returnvalue) _returnvalue_3) false false)
  (Transformation|SetWorldRotation _legsflipbook (Math|Rotator|MakeRotator (.roll _returnvalue_2) (.pitch _returnvalue_2) _returnvalue_3) false false)
  (Variables|/Game/Dev/Gibran/Core/Blueprints/Components/BP_SpriteAnimationComponent.BP_SpriteAnimationComponent_C|SetDirection _bp_spriteanimationcomponent (Variables|Default|GetDirection))
  (Variables|/Game/Dev/Gibran/Core/Blueprints/Components/BP_SpriteAnimationComponent.BP_SpriteAnimationComponent_C|SetSpeed _bp_spriteanimationcomponent (Variables|/Game/Dev/Gibran/Core/Blueprints/Heroes/BP_HeroGroup.BP_HeroGroup_C|GetGroupSpeed (Variables|Default|GetHeroGroupRef)))
  (Utilities|FlowControl|Sequence
    (:then_0
      (Utilities|FlowControl|FlipFlop
        (:A
          (Transformation|AddRelativeLocation _capsule "0.010000, 0, 0" false false))
        (:B
          (Transformation|AddRelativeLocation _capsule "-0.010000, 0, 0" false false))))
    (:then_1
      (if (Variables|Health|GetFainted)
        (Sprite|SetSpriteColor (Variables|Default|GetTorsoFlipbook) "(R=0.000000,G=0.000000,B=0.000000,A=1.000000)")
        (Sprite|SetSpriteColor (Variables|Default|GetLegsFlipbook) "(R=0.000000,G=0.000000,B=0.000000,A=1.000000)")))))

(event EventTakeDamage
  (params (DamageCauser :type Actor%20Object%20Reference) (DamageInstigator :type Actor%20Object%20Reference) (Damage :type Float%20%28double-precision%29) (KnockbackStrength :type Float%20%28double-precision%29) (DamageType :type E_DamageType%20Enum :default "NewEnumerator11") (Direction :type Vector :default "0, 0, 0"))
  ;[0.07812 0 0] Taking Damage
  (Utilities|CheckforShieldBlocking DamageCauser
    (:NotBlocked
      (bind _output_get (Variables|Default|SetDamageReceived Damage))
      (if (not (Variables|Health|GetFainted))
        (if (not (Variables|Health|GetInDamageCooldown))
          (Utilities|FlowControl|Sequence
            (:then_0
              (Variables|Health|SetInDamageCooldown true)
              (Utilities|FlowControl|Delay (Variables|Health|GetDamageCooldown))
              (Variables|Health|SetInDamageCooldown false))
            (:then_1
              (Utilities|FlipbookDamageFlash (Variables|Default|GetTorsoFlipbook) 0.2
                (:__
                  (Utilities|FlipbookDamageFlash (Variables|Default|GetLegsFlipbook) 0.2
                    (:__
                      (Audio|PlaySoundatLocation (Variables|Default|GetDamageSound) (Transformation|GetActorLocation) "0, 0, 0" 1.0 1.0 0.0 0 0 0 0)
                      (bind _output_get_2 (Variables|Health|SetHealth (Math|Float|Clamp(Float) (- (Variables|Health|GetHealth) (Variables|Default|GetDamageReceived)) 0.0 (Variables|Health|GetMaxHealth))))
                      (Default|UpdateTotalHealth (Variables|Default|GetHeroGroupRef))
                      (Default|AddStatDamageReceived (CallFunction|GetHeroesGameInstance) (Variables|Default|GetDamageReceived))
                      (if (<= _output_get_2 0.0)
                        (Utilities|FlowControl|Delay 0.2)
                        (CallFunction|Faint)))))))
            (:then_2
              (Development|PrintText (Utilities|Text|FormatText "Hero {name} took {dmg} of damage" (Variables|Default|GetName) _output_get) (CallFunction|ReadDebugTag "Damage") true "(R=1.000000,G=0.000000,B=0.144855,A=1.000000)" 4.0 "HeroDamage"))))))))

(fn ConstructionScript)

(fn ToggleTalkingIcon
  (params (Visible :type Boolean))
  (Rendering|SetVisibility (Variables|Default|GetTalkingIcon) Visible false))