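; Sprite animation component that drives separate legs and torso Paper2D flipbooks for an actor, with extra handling for heroes.
; Tick swaps idle and walking flipbooks based on velocity, direction or speed, and mirrors both layers through X scale.
; Facing follows Direction or X velocity, or, for heroes in a group, the group's rotation direction and the hero's Y side.
; ExecuteAnimation overrides only the torso for the action flipbook's duration, leaving legs animating independently.
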(event Custom|ExecuteAnimation
  (params (Flipbook :type Paper%20Flipbook%20Object%20Reference))
  (bind _torsoflipbookref (Variables|Default|GetTorsoFlipbookRef))
  ;[0 0 0] Flipbook Action Animation
  (Utilities|IsValid Flipbook
    (:Is%20Valid
      (Variables|Default|SetExecutingAction true)
      (bind _output_get (Variables|Default|SetActionFlipbook Flipbook))
      (Components|Timeline|SetNewTime _torsoflipbookref 0.0)
      (Sprite|SetFlipbook _torsoflipbookref _output_get)
      (Utilities|FlowControl|Delay (Class|PaperFlipbook|GetTotalDuration Flipbook))
      (Variables|Default|SetExecutingAction false))))

(event EventBeginPlay
  (bind _actorref (Variables|Default|GetActorRef))
  (Utilities|FlowControl|Delay 0.001)
  (Utilities|IsValid _actorref
    (:Is%20Valid
      (if (Utilities|ClassIsChildOf (Utilities|GetClass _actorref) "/Game/Dev/Gibran/Core/Blueprints/Heroes/BP_HeroBase.BP_HeroBase_C")
        (bind _asbp_hero_base (Utilities|Casting|CastToBP_HeroBase _actorref))
        (Variables|Default|SetHero%20Group%20Ref (Variables|/Game/Dev/Gibran/Core/Blueprints/Heroes/BP_HeroBase.BP_HeroBase_C|GetHeroGroupRef _asbp_hero_base))))))

(event EventTick
  (params (DeltaSeconds :type Float%20%28single-precision%29))
  (bind _legsflipbookref (Variables|Default|GetLegsFlipbookRef))
  (bind _torsoflipbookref (Variables|Default|GetTorsoFlipbookRef))
  (bind _direction (Variables|Default|GetDirection))
  (bind _actionflipbook (Variables|Default|GetActionFlipbook))
  (bind _hero_group_ref (Variables|Default|GetHero%20Group%20Ref))
  (bind _actorref (Variables|Default|GetActorRef))
  (bind _legsflipbookref_2 (Variables|Default|GetLegsFlipbookRef))
  (bind _torsoflipbookref_2 (Variables|Default|GetTorsoFlipbookRef))
  (bind _returnvalue (Transformation|GetActorLocation _hero_group_ref))
  (bind _returnvalue_2 (Transformation|GetActorLocation _actorref))
  (bind _returnvalue_3 (Transformation|GetWorldScale _legsflipbookref))
  (bind _returnvalue_4 (Transformation|GetWorldScale _torsoflipbookref))
  (bind _returnvalue_5 (Math|Float|Absolute(Float) (.x _returnvalue_3)))
  (bind _returnvalue_6 (Math|Float|Absolute(Float) (.x _returnvalue_4)))
  (Utilities|FlowControl|Sequence
    (:then_0
      ;[0 0 0] Idle or Movement
      (if (Math|Boolean|ORBoolean (> (Math|Vector|VectorLength (Variables|Default|GetVelocity)) 0.0) (!= (Variables|Default|GetDirection) 0.0) (!= (Variables|Default|GetSpeed) 0.0))
        (Sprite|SetFlipbook _legsflipbookref_2 (Variables|Default|GetLegsWalkingFlipbook))
        (Sprite|SetFlipbook _torsoflipbookref_2 (select (Variables|Default|GetExecutingAction) _actionflipbook (Variables|Default|GetTorsoWalkingFlipbook)))
        (else
          (Sprite|SetFlipbook _legsflipbookref_2 (Variables|Default|GetLegsIdleFlipbook))
          (Sprite|SetFlipbook _torsoflipbookref_2 (select (Variables|Default|GetExecutingAction) _actionflipbook (Variables|Default|GetTorsoIdleFlipbook))))))
    (:then_1
      ;[0 0 0] Flipping the Flipbook
      (Utilities|IsValid (Variables|Default|GetHero%20Group%20Ref)
        (:Is%20Valid
          ;;[0 0 0] Hero especific rotation
          (Math|Float|CompareFloat (Variables|/Game/Dev/Gibran/Core/Blueprints/Heroes/BP_HeroGroup.BP_HeroGroup_C|GetGroupRotationDirection _hero_group_ref) 0.0
            (:>
              (Math|Float|CompareFloat (.y _returnvalue_2) (.y _returnvalue)
                (:>
                  (Transformation|SetWorldScale3D _torsoflipbookref (Math|Vector|MakeVector (* _returnvalue_6 -1.0) (.y _returnvalue_4) (.z _returnvalue_4)) :!label _label)
                  (Transformation|SetWorldScale3D _legsflipbookref (Math|Vector|MakeVector (* _returnvalue_5 -1.0) (.y _returnvalue_3) (.z _returnvalue_3))))
                (:<
                  (Transformation|SetWorldScale3D _torsoflipbookref (Math|Vector|MakeVector _returnvalue_6 (.y _returnvalue_4) (.z _returnvalue_4)) :!label _label_2)
                  (Transformation|SetWorldScale3D _legsflipbookref (Math|Vector|MakeVector _returnvalue_5 (.y _returnvalue_3) (.z _returnvalue_3))))))
            (:<
              (Math|Float|CompareFloat (.y _returnvalue_2) (.y _returnvalue)
                (:>
                  (goto _label_2))
                (:<
                  (goto _label))))))
        (:Is%20Not%20Valid
          (Math|Float|CompareFloat (.X (Math|Vector|BreakVector (select (!= _direction 0.0) (Math|Vector|MakeVector _direction 0.0 0.0) (Variables|Default|GetVelocity)))) 0.0
            (:>
              (goto _label_2))
            (:<
              (goto _label))))))))