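; Ranged hero Blueprint (Hanna) with two projectile attacks, extending a parent hero class.
; Each action plays the attack animation, fires a DT_Projectiles row through BPShootingComponent, spawns a tinted flipbook VFX with sound, and starts its cooldown.
; When Enhanced, both actions become multi-ray spreads, wider for the second, which also shakes the camera.
; Enhancement start sets the meter icon to arrows, and debug arrows visualise the shooting direction.
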(event EventAction2
  (bind _bp_shooting_component (Variables|Default|GetBP_Shooting_Component))
  (bind _arrow (Variables|Default|GetArrow))
  (Default|ExecuteAnimation (Variables|Default|GetBP_SpriteAnimationComponent) "/Game/Dev/Gibran/TestAssets/Flipbooks/Characters/Han_Attacking.Han_Attacking")
  (if (Variables|Default|GetEnhanced)
    (Variables|/Game/Bin/Blueprints/Character/BP_Shooting_Component.BP_Shooting_Component_C|SetShootRays _bp_shooting_component 5)
    (Variables|/Game/Bin/Blueprints/Character/BP_Shooting_Component.BP_Shooting_Component_C|SetShootAngle _bp_shooting_component 7e+01)
    (else
      (Variables|/Game/Bin/Blueprints/Character/BP_Shooting_Component.BP_Shooting_Component_C|SetShootRays _bp_shooting_component 1)
      (Variables|/Game/Bin/Blueprints/Character/BP_Shooting_Component.BP_Shooting_Component_C|SetShootAngle _bp_shooting_component 0.0)))
  (Default|FShootOnceProjectilefromDatatable _bp_shooting_component (Utilities|Struct|MakeDataTableRowHandle "/Game/Dev/Gibran/Core/DataTables/DT_Projectiles.DT_Projectiles" "HannaProjectile2"))
  (Audio|PlaySoundatLocation "/Game/Dev/Gibran/TestAssets/Sounds/Combat/swoosh_1_Cue.swoosh_1_Cue" (Transformation|GetActorLocation) "0, 0, 0" 2.0 2.0 0.0 0 0 0 0)
  (bind _returnvalue (Game|SpawnActorfromClass "/Game/Dev/Gibran/Core/Blueprints/BP_SpriteVFX.BP_SpriteVFX_C" (Math|Transform|MakeTransform (Transformation|GetWorldLocation _arrow) (Math|Rotator|MakeRotator 0.0 0.0 (.yaw (Transformation|GetWorldRotation _arrow))) "1.000000,1.000000,1.000000") "Undefined" 0 0))
  (Default|TriggerEffect(Flipbook) _returnvalue "/Game/Dev/Gibran/TestAssets/Flipbooks/VFX/3_Sprite.3_Sprite" 2.0 false)
  (Sprite|SetSpriteColor (Variables|/Game/Dev/Gibran/Core/Blueprints/BP_SpriteVFX.BP_SpriteVFX_C|GetPaperFlipbook _returnvalue) "(R=0.000000,G=1.000000,B=0.497386,A=1.000000)")
  (Game|Feedback|ClientStartCameraShake (Game|GetPlayerController 0) "/Game/Dev/Gibran/Core/Blueprints/CameraShakes/TestCameraShake.TestCameraShake_C" 0.25 "CameraLocal" "0, 0, 0")
  (CallFunction|StartAbility2Cooldown))

(event EventAction1
  (bind _bp_shooting_component (Variables|Default|GetBP_Shooting_Component))
  (bind _arrow (Variables|Default|GetArrow))
  (bind _bp_shooting_component_2 (Variables|Default|GetBP_Shooting_Component))
  (bind _returnvalue (Transformation|GetWorldLocation _bp_shooting_component))
  (Default|ExecuteAnimation (Variables|Default|GetBP_SpriteAnimationComponent) "/Game/Dev/Gibran/TestAssets/Flipbooks/Characters/Han_Attacking.Han_Attacking")
  (if (Variables|Default|GetEnhanced)
    (Variables|/Game/Bin/Blueprints/Character/BP_Shooting_Component.BP_Shooting_Component_C|SetShootRays _bp_shooting_component_2 3)
    (Variables|/Game/Bin/Blueprints/Character/BP_Shooting_Component.BP_Shooting_Component_C|SetShootAngle _bp_shooting_component_2 3e+01)
    (else
      (Variables|/Game/Bin/Blueprints/Character/BP_Shooting_Component.BP_Shooting_Component_C|SetShootRays _bp_shooting_component_2 1)
      (Variables|/Game/Bin/Blueprints/Character/BP_Shooting_Component.BP_Shooting_Component_C|SetShootAngle _bp_shooting_component_2 0.0)))
  (Default|FShootOnceProjectilefromDatatable _bp_shooting_component_2 (Utilities|Struct|MakeDataTableRowHandle "/Game/Dev/Gibran/Core/DataTables/DT_Projectiles.DT_Projectiles" "HannaProjectile1"))
  (Audio|PlaySoundatLocation "/Game/Dev/Gibran/TestAssets/Sounds/Combat/swoosh_1_Cue.swoosh_1_Cue" (Transformation|GetActorLocation) "0, 0, 0" 1.0 1.0 0.0 0 0 0 0)
  (bind _returnvalue_2 (Game|SpawnActorfromClass "/Game/Dev/Gibran/Core/Blueprints/BP_SpriteVFX.BP_SpriteVFX_C" (Math|Transform|MakeTransform (Transformation|GetWorldLocation _arrow) (Math|Rotator|MakeRotator 0.0 0.0 (.yaw (Transformation|GetWorldRotation _arrow))) "0.500000,0.500000,0.500000") "Undefined" 0 0))
  (Default|TriggerEffect(Flipbook) _returnvalue_2 "/Game/Dev/Gibran/TestAssets/Flipbooks/VFX/3_Sprite.3_Sprite" 2.0 false)
  (Sprite|SetSpriteColor (Variables|/Game/Dev/Gibran/Core/Blueprints/BP_SpriteVFX.BP_SpriteVFX_C|GetPaperFlipbook _returnvalue_2) "(R=0.624931,G=1.000000,B=0.000000,A=1.000000)")
  (Utilities|FlowControl|Sequence
    (:then_0
      (Utilities|IsDebugModeOn?
        (:Debug%20Mode%20On
          (Rendering|Debug|DrawDebugArrow _returnvalue (+ _returnvalue (* (Math|Vector|GetForwardVector _bp_shooting_component) 5e+02)) 2.0 "(R=1.000000,G=0.024480,B=0.000000,A=1.000000)" 1.0 3.0))))
    (:then_1
      (CallFunction|StartAbility1Cooldown))))

(event EventTick
  (params (DeltaSeconds :type Float%20%28single-precision%29))
  (bind _bp_shooting_component (Variables|Default|GetBP_Shooting_Component))
  (bind _returnvalue (Transformation|GetWorldLocation _bp_shooting_component))
  (|CallParentFunction DeltaSeconds)
  (Utilities|IsDebugModeOn?
    (:Debug%20Mode%20On
      _)
    (:Debug%20Mode%20Off
      _))
  (Rendering|Debug|DrawDebugArrow _returnvalue (+ _returnvalue (* (Math|Vector|GetForwardVector _bp_shooting_component) 2.5e+02)) 1e+01 "(R=0.000000,G=1.000000,B=0.185576,A=1.000000)" 0.0 3.0))

(event EventStartEnhancement
  (Class|Image|SetBrushResourceObject (Variables|/Game/Dev/Gibran/Core/UI/HUD/WBP_EnhancementMeter.WBP_EnhancementMeter_C|GetEnhacementIcon (Variables|Default|GetEnhancementMeterRef)) "/Game/Dev/Gibran/TestAssets/Sprites/UI/Icons/Icon_Arrows.Icon_Arrows"))

(event EventEndEnhancement)

(fn ConstructionScript
  (|CallParentFunction))