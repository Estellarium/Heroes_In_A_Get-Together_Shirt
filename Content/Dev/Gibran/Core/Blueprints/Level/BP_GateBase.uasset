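; Base interactable 2D gate that the player opens and closes, optionally requiring key items from the hero group's inventory.
; Interact counts inventory items matching the key name against the required quantity, unlocking on the first success and toggling afterwards.
; Each state change swaps the Paper2D tilemap and updates the prompt; opening and closing also swap the sprite and collision object type.
; The key check repeats on every interaction, and its match counter is never visibly reset.
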(event Custom|OpenGate
  (Variables|Default|SetOpen true)
  (Class|PaperTileMapComponent|SetTileMap (Variables|Default|GetPaperTileMap) (Variables|Default|GetOpenedTilemap))
  (Rendering|Components|Sprite|SetSprite (Variables|Default|GetPaperSprite) (Variables|Default|GetOpenedSprite))
  (Development|PrintString "Opened" (CallFunction|ReadDebugTag "GeneralDebug"))
  (Collision|SetCollisionObjectType (Variables|Default|GetCollisionBox) "ECC_WorldDynamic")
  (Variables|Default|SetInteractionPromptText "E to close")
  (Default|UnfocusInteractable (Variables|/Game/Dev/Gibran/Core/Blueprints/Heroes/BP_HeroGroupRemake.BP_HeroGroupRemake_C|GetHeroBenRef (Variables|Default|GetPlayerGroupRef))))

(event Custom|CloseGate
  (Variables|Default|SetOpen false)
  (Class|PaperTileMapComponent|SetTileMap (Variables|Default|GetPaperTileMap) (Variables|Default|GetClosedTilemap))
  (Rendering|Components|Sprite|SetSprite (Variables|Default|GetPaperSprite) (Variables|Default|GetClosedSprite))
  (Development|PrintString "Closed" (CallFunction|ReadDebugTag "GeneralDebug"))
  (Collision|SetCollisionObjectType (Variables|Default|GetCollisionBox) "ECC_WorldStatic")
  (Variables|Default|SetInteractionPromptText "E to open")
  (Default|UnfocusInteractable (Variables|/Game/Dev/Gibran/Core/Blueprints/Heroes/BP_HeroGroupRemake.BP_HeroGroupRemake_C|GetHeroBenRef (Variables|Default|GetPlayerGroupRef))))

(event Custom|Unlock
  (Variables|Default|SetLocked false)
  (Development|PrintString "Unlocked" (CallFunction|ReadDebugTag "GeneralDebug"))
  (Default|UnfocusInteractable (Variables|/Game/Dev/Gibran/Core/Blueprints/Heroes/BP_HeroGroupRemake.BP_HeroGroupRemake_C|GetHeroBenRef (Variables|Default|GetPlayerGroupRef)))
  (Variables|Default|SetInteractionPromptText "E to open")
  (Class|PaperTileMapComponent|SetTileMap (Variables|Default|GetPaperTileMap) (Variables|Default|GetClosedTilemap)))

(event EventBeginPlay
  (Variables|Default|SetPlayerGroupRef (CallFunction|GetHeroesGroup))
  (Class|PaperTileMapComponent|SetTileMap (Variables|Default|GetPaperTileMap) (Variables|Default|GetLockedTilemap)))

(event EventInteract
  (params (Instigator :type Actor%20Object%20Reference))
  (if (Variables|Default|GetRequiresKeyItem)
    (if (CallFunction|CheckforKeyItens (Variables|/Game/Dev/Gibran/Core/Blueprints/Heroes/BP_HeroGroupRemake.BP_HeroGroupRemake_C|GetInventory (Variables|Default|GetPlayerGroupRef)))
      (if (Variables|Default|GetLocked)
        (CallFunction|Unlock)
        (else
          (if (Variables|Default|GetOpen) :!label _label
            (CallFunction|CloseGate)
            (else
              (CallFunction|OpenGate))))))
    (else
      (goto _label))))

(fn ConstructionScript
  (Class|PaperTileMapComponent|SetTileMap (Variables|Default|GetPaperTileMap) (Variables|Default|GetLockedTilemap)))

(fn CheckforKeyItens
  (params (PlayerInventory :type Array%20of%20S%20Inventory%20Object%20Structures))
  (for _array_element PlayerInventory
    (if (== (.Name (Utilities|Struct|BreakS_InventoryObject _array_element)) (Variables|Default|GetKeyItemName))
      (Math|Integer|IncrementInt (LocalVariables|GetMatchingKeyItens))))
  (if (>= (LocalVariables|GetMatchingKeyItens) (Variables|Default|GetKeyItemQuantity))
    (return true)
    (else
      (return false))))

(fn GetInteractionPrompt
  (return (Utilities|Text|FormatText (Variables|Default|GetInteractionPromptText) (Variables|Default|GetKeyItemQuantity) (Variables|Default|GetKeyItemName)) (Variables|Default|GetInteractionPromptImage)))