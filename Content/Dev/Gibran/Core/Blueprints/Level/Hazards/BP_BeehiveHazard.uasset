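; BP_BeehiveHazard is a one-shot level hazard: a beehive that falls and releases bees when triggered.
; ActivationArea fires once when overlapped by a component with the Hero, Hero Projectile or Hero Melee collision profile.
; A sped-up timeline lerps the sprite from its starting relative location to FallLocation.
; On finish it swaps the sprite and spawns BeesAmmount BP_BeeHazard actors there, each holding a reference to the hive.
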(event OnComponentBeginOverlap(ActivationArea)
  (params (OverlappedComponent :type Primitive%20Component%20Object%20Reference) (OtherActor :type Actor%20Object%20Reference) (OtherComp :type Primitive%20Component%20Object%20Reference) (OtherBodyIndex :type Integer) (bFromSweep :type Boolean) (SweepResult :type Hit%20Result%20Structure%20%28by%20ref%29))
  (switch name (Collision|GetCollisionProfileName OtherComp)
    (:Hero
      _)
    (:HeroProjectile
      _)
    (:HeroMelee
      _))
  (Utilities|FlowControl|DoOnce false
    (:Completed
      (CallFunction|Activate))))

(event Custom|Activate
  (bind _beehivesprite (Variables|Default|GetBeehiveSprite))
  (Variables|Default|SetInitialLocation (Variables|/Script/Engine.SceneComponent|GetRelativeLocation (Variables|Default|GetBeehiveSprite)))
  (Components|Timeline|SetPlayRate (Variables|Default|GetFallTimeline) 2.0)
  (bind _alpha (Timeline|FallTimeline Play)
    (:Update
      (Transformation|SetRelativeLocation _beehivesprite (Math|Vector|Lerp(Vector) (Variables|Default|GetInitialLocation) (Variables|Default|GetFallLocation) _alpha) false false))
    (:Finished
      (Rendering|Components|Sprite|SetSprite _beehivesprite "/Game/Dev/Gibran/TestAssets/Sprites/Objects/Beehive2.Beehive2")
      (for _index (range 1 (Variables|Default|GetBeesAmmount))
        (Game|SpawnActorfromClass "/Game/Dev/Gibran/Core/Blueprints/Level/Hazards/BP_BeeHazard.BP_BeeHazard_C" (Math|Transform|MakeTransform (Transformation|GetWorldLocation _beehivesprite) "0, 0, 0" "1.000000,1.000000,1.000000") "Undefined" 0 self 0)))))

(fn ConstructionScript)