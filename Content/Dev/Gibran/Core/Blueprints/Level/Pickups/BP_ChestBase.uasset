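; BP_ChestBase is a base interactable chest pickup that bursts into coins when opened.
; Interact fires once, playing a timeline that scales the chest sprite relative to its original scale cached at construction.
; When the animation finishes, it spawns a random number of BP_Coin actors at its location and destroys itself.
; The construction script also applies the configurable sprite, and the interaction prompt reads "Open chest".
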(event EventInteract
  (params (Instigator :type Actor%20Object%20Reference))
  (bind _originalspritescale (Variables|Default|GetOriginalSpriteScale))
  (Utilities|FlowControl|DoOnce false
    (:Completed
      (bind _transform (Timeline|ChestOpenAnimation Play)
        (:Update
          (Transformation|SetRelativeScale3D (Variables|Default|GetChestSprite) (Math|Vector|MakeVector (* (.x _originalspritescale) (.x _transform)) (* (.y _originalspritescale) (.y _transform)) (* (.z _originalspritescale) (.z _transform)))))
        (:Finished
          (for _index (range 1 (Math|Random|RandomIntegerinRange (Variables|Default|GetMinCoinAmmount) (Variables|Default|GetMaxCoinAmmount)))
            (Game|SpawnActorfromClass "/Game/Dev/Gibran/Core/Blueprints/Level/Pickups/BP_Coin.BP_Coin_C" (Math|Transform|MakeTransform (Transformation|GetActorLocation) "0, 0, 0" "1.000000,1.000000,1.000000") "AlwaysSpawn" 0 0))
          (Actor|DestroyActor))))))

(fn ConstructionScript
  (bind _chestsprite (Variables|Default|GetChestSprite))
  (Rendering|Components|Sprite|SetSprite _chestsprite (Variables|Default|GetSprite))
  (Variables|Default|SetOriginalSpriteScale (Variables|/Script/Engine.SceneComponent|GetRelativeScale3D _chestsprite)))

(fn GetInteractionPrompt
  (return "Open chest" 0))