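; BP_Shooting_Component is a scene component that fires one volley of projectiles for its owner, with a configurable ray count.
; Two events ask the game mode to spawn them, from a class (faster, custom effects) or a customizable struct, with optional overrides.
; MakeBulletTransform offsets spawns forward and yaws each ray into a centered arc or an equal radial spread.
; BeginPlay clamps the arc angle to limit overlaps, zeroing it in radial mode.
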(event Custom|Shoot%20Once%20Projectille%20Structure
  (params (Override :type Struct%20Projectile%20Structure))
  ;[1 1 1] Spawn Projectile from a customizable Struct (slower, no custom effects)
  (for _index (range 1 (Variables|Default|GetShootRays))
    (Class|BPIGMProjectile|SpawnProjectilefromStruct(Message) (Game|GetGameMode) (select (== (Utilities|Struct|BreakStruct_Projectile Override) "Null") (Variables|Default|GetProjectile%20Struct) Override) (CallFunction|MakeBulletTransform _index) (Components|GetOwner))))

(event Custom|Shoot%20Once%20Projectile%20Class
  (params (Override :type BP%20Projectile%20Class%20Reference))
  ;[1 1 1] Spawn Projectile from a defined class (faster to spawn, custom effects from within class)
  (for _index (range 1 (Variables|Default|GetShootRays))
    (Class|BPIGMProjectile|SpawnProjectilefromClass(Message) (Game|GetGameMode) (select (== Override 0) (Variables|Default|GetProjectile%20Class) Override) (CallFunction|MakeBulletTransform _index) (Components|GetOwner))))

(event EventBeginPlay
  ;[1 1 1] Clamp shooting angle to avoid overlaps at 180+ angles
  (if (Variables|Default|GetEquirradial)
    (Variables|Default|SetShootAngle 0.0)
    (else
      (Variables|Default|SetShootAngle (Math|Float|Clamp(Float) (Variables|Default|GetShootAngle) 0.0 (Utilities|Operators|Divide 3.6e+02 (Math|Conversions|ToFloat(Integer) (Variables|Default|GetShootRays)) 0.5))))))

(fn MakeBulletTransform
  (params (Index :type Integer))
  (bind _returnvalue (Transformation|GetWorldTransform))
  (bind _shootrays (Variables|Default|GetShootRays))
  (bind _equirradial (Variables|Default|GetEquirradial))
  (bind (_location _rotation _scale) (Math|Transform|BreakTransform _returnvalue))
  (bind _returnvalue_2 (- _shootrays 1))
  ;[1 1 1] Equidistant angles
  ;[1 1 1] Spawn away from "socket"
  (return (Math|Transform|MakeTransform (+ _location (* (Math|Vector|GetForwardVector) (Variables|Default|GetShootDist))) (Math|Rotator|CombineRotators _rotation (Math|Rotator|MakeRotator 0.0 0.0 (- (* (- (Math|Conversions|ToFloat(Integer) Index) 1.0) (Math|Float|SelectFloat (/ 3.6e+02 (Math|Conversions|ToFloat(Integer) (Variables|Default|GetShootRays))) (select (== _returnvalue_2 0) 0.0 (/ (Variables|Default|GetShootAngle) _returnvalue_2)) _equirradial)) (Math|Float|SelectFloat 0.0 (* (Variables|Default|GetShootAngle) 0.5) _equirradial)))) _scale)))