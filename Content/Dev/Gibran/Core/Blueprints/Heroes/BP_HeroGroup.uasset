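; Player pawn that moves and turns a party of four hero child actors (ranged, melee, tank, healer-unlocker) as one unit.
; Each action input fires one hero's ability, picking tap or hold through a retriggerable delay.
; Projectile damage splits evenly across heroes, and zero total health triggers game over.
; Also handles HUD, pause, debug tools, timed speed enhancements and a level-intro camera timeline whose curve is swapped at runtime.
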(event Custom|TriggerGroupEnhancement
  (params (Duration :type Float%20%28double-precision%29))
  ;[0 0 0] Enhancements
  (if (not (Variables|PowerUp|GetEnhanced))
    (Variables|PowerUp|SetEnhanced true)
    (CallFunction|TimelinePlayrateinSeconds (Variables|Default|GetEnhancementTimeline) Duration)
    (bind _meter (Default|CreateMeter (Variables|PowerUp|GetEnhancementsRef) (Variables|PowerUp|GetEnhancementColor)))
    (Variables|PowerUp|SetEnhancementMeterRef _meter)
    (CallFunction|StartEnhancement)
    (bind _duration (Timeline|EnhancementTimeline PlayFromStart)
      (:Update
        (Progress|SetPercent (Variables|/Game/Dev/Gibran/Core/UI/HUD/WBP_EnhancementMeter.WBP_EnhancementMeter_C|GetEnhancementTime (Variables|PowerUp|GetEnhancementMeterRef)) _duration))
      (:Finished
        (Default|EndMeter (Variables|PowerUp|GetEnhancementMeterRef))
        (Variables|PowerUp|SetEnhancementMeterRef 0)
        (Variables|PowerUp|SetEnhanced false)
        (CallFunction|EndEnhancement)))))

(event Custom|EndEnhancement
  ;[0 0 0] Enhancements
  (Variables|Default|SetMovementSpeedMultiplier 1.0))

(event Custom|StartEnhancement
  ;[0 0 0] Enhancements
  (Variables|Default|SetMovementSpeedMultiplier 2.0)
  (Class|Image|SetBrushResourceObject (Variables|/Game/Dev/Gibran/Core/UI/HUD/WBP_EnhancementMeter.WBP_EnhancementMeter_C|GetEnhacementIcon (Variables|PowerUp|GetEnhancementMeterRef)) "/Game/Dev/Gibran/TestAssets/Sprites/UI/Icons/_1_-_Transparent_Icons_Sprite_60._1_-_Transparent_Icons_Sprite_60"))

(event Custom|LevelStartCameraAnimation
  (params (CameraAnimationCurve :type Curve%20Vector%20Object%20Reference))
  (bind _camera (Variables|Default|GetCamera))
  (bind _cameraanimtimeline (Variables|Default|GetCameraAnimTimeline))
  (Class|TimelineComponent|SetVectorCurve _cameraanimtimeline CameraAnimationCurve "PositionAndZoom")
  (Components|Timeline|SetTimelineLength _cameraanimtimeline (.MaxTime (Math|Curves|GetTimeRange CameraAnimationCurve)))
  (bind _positionandzoom (Timeline|CameraAnimTimeline Play)
    (:Update
      (Transformation|SetRelativeLocation _camera (Math|Vector|MakeVector 0.0 (.Y (Math|Vector|BreakVector _positionandzoom)) (.X (Math|Vector|BreakVector _positionandzoom))) false false)
      (Class|CameraComponent|SetOrthoWidth _camera (.Z (Math|Vector|BreakVector _positionandzoom))))))

(event Custom|Die
  ;[0.151 0 0] Game Over
  (bind _outactors (Actor|GetAllActorsOfClass "/Script/Engine.AmbientSound"))
  (for _array_element _outactors
    (Audio|Components|Audio|AdjustVolume (Variables|/Script/Engine.AmbientSound|GetAudioComponent _array_element) 1.0 0.0 "Linear" :!class /Script/Engine.AudioComponent))
  (Input|DisableInput (Game|GetPlayerController 0))
  (Widget|RemovefromParent (Variables|Default|GetHudRef))
  (Utilities|FlowControl|Delay 0.5)
  (Game|SetGamePaused true)
  (bind _returnvalue (UserInterface|CreateWidget "/Game/Dev/Gibran/Core/UI/WBP_GameOverScreen.WBP_GameOverScreen_C"))
  (UserInterface|Viewport|AddtoViewport _returnvalue 0))

(event Custom|TakeGroupHealing
  (params (HealAmmount :type Float%20%28double-precision%29))
  (Default|ReceiveHealing (Variables|Default|GetHeroHanRef) HealAmmount)
  (Default|ReceiveHealing (Variables|Default|GetHeroEthRef) HealAmmount)
  (Default|ReceiveHealing (Variables|Default|GetHeroShuRef) HealAmmount)
  (Default|ReceiveHealing (Variables|Default|GetHeroBenRef) HealAmmount))

(event EventBeginPlay
  ;[0.1667 0.1667 0.1667] Begin Play
  (Utilities|FlowControl|Sequence
    (:then_0
      (Variables|Default|SetGameModeRef (CallFunction|GetHeroesGameMode))
      (Variables|Default|SetGameInstanceRef (CallFunction|GetHeroesGameInstance)))
    (:then_1
      (Components|Movement|SetUpdatedComponent (Variables|Default|GetFloatingPawnMovement) (Variables|Default|GetBoxCollision)))
    (:then_2
      (|SetHeroReferences))
    (:then_3
      (Utilities|FlowControl|Delay 0.01)
      (Class|CameraComponent|SetOrthoWidth (Variables|Default|GetCamera) (.z (Math|Curves|GetVectorValue (Utilities|Struct|BreakS_LevelData (.Value (Utilities|Map|Find (Variables|/Game/Dev/Gibran/Core/HeroesGameInstance.HeroesGameInstance_C|GetLevelDataRef (Variables|Default|GetGameInstanceRef)) (Variables|/Game/Bin/Blueprints/_Core/GM_BulletHell.GM_BulletHell_C|GetCurrentLevel (Variables|Default|GetGameModeRef))))) (.MinTime (Math|Curves|GetTimeRange (Utilities|Struct|BreakS_LevelData (.Value (Utilities|Map|Find (Variables|/Game/Dev/Gibran/Core/HeroesGameInstance.HeroesGameInstance_C|GetLevelDataRef (Variables|Default|GetGameInstanceRef)) (Variables|/Game/Bin/Blueprints/_Core/GM_BulletHell.GM_BulletHell_C|GetCurrentLevel (Variables|Default|GetGameModeRef)))))))))))
    (:then_4
      (Utilities|FlowControl|Delay 5.0)
      (|CreateHUD))))

(event EventTakeDamage
  (params (DamageCauser :type Actor%20Object%20Reference) (DamageInstigator :type Actor%20Object%20Reference) (Damage :type Float%20%28double-precision%29) (KnockbackStrength :type Float%20%28double-precision%29) (DamageType :type E_DamageType%20Enum :default "NewEnumerator11") (Direction :type Vector :default "0, 0, 0"))
  (bind _returnvalue (/ Damage 4.0))
  ;[0.1823 0 0] Taking Group Damage
  (bind _asbp_projectile (Utilities|Casting|CastToBP_Projectile DamageCauser))
  (switch name (Collision|GetCollisionProfileName (Variables|/Game/Bin/Blueprints/Object/Projectiles/BP_Projectile.BP_Projectile_C|GetCapsule _asbp_projectile))
    (:EnemyProjectile
      _)
    (:EnemyMelee
      _))
  (Class|BPIDamageableActor|TakeDamage(Message) (Variables|Default|GetHeroHanRef) 0 0 _returnvalue 0.0 DamageType "0, 0, 0")
  (Class|BPIDamageableActor|TakeDamage(Message) (Variables|Default|GetHeroEthRef) 0 0 _returnvalue 0.0 DamageType "0, 0, 0")
  (Class|BPIDamageableActor|TakeDamage(Message) (Variables|Default|GetHeroShuRef) 0 0 _returnvalue 0.0 DamageType "0, 0, 0")
  (Class|BPIDamageableActor|TakeDamage(Message) (Variables|Default|GetHeroBenRef) 0 0 _returnvalue 0.0 DamageType "0, 0, 0")
  (Game|Feedback|ClientStartCameraShake (Game|GetPlayerController 0) "/Game/Dev/Gibran/Core/Blueprints/CameraShakes/DamageCameraShake.DamageCameraShake_C" 1.0 "CameraLocal" "0, 0, 0")
  (Audio|PlaySoundatLocation (Variables|Default|GetGroupDamageSound) (Transformation|GetActorLocation) "0, 0, 0" 1.0 1.0 0.0 0 0 0 0)
  (Default|AddStatDamageReceived (Variables|Default|GetGameInstanceRef) Damage))

(event EventTick
  (params (DeltaSeconds :type Float%20%28single-precision%29))
  (bind _boxcollision (Variables|Default|GetBoxCollision))
  ;[0.3385 0.3385 0.3385] Tick
  (Utilities|FlowControl|Sequence
    (:then_0
      (bind _returnvalue (Class|Pawn|ConsumeMovementInputVector))
      (Class|PawnMovementComponent|AddInputVector (Variables|Default|GetFloatingPawnMovement) _returnvalue false)
      (Variables|Default|SetGroupSpeed (+ (Math|Vector|VectorLength (Transformation|GetVelocity)) (Variables|Default|GetGroupRotatingSpeed) (Variables|Default|GetGroupWalkingSpeed)))
      (Utilities|SwitchDebugTag "GeneralDebug"
        (:Debug%20Tag%20On
          (|DistanceDebugging))))
    (:then_1
      (Development|PrintText (Utilities|Text|FormatText "Ethan: {eh} 
Hanna: {hh} 
Shura: {sh} 
Benjamin: {bh} 
Total: {th}" (Variables|/Game/Dev/Gibran/Core/Blueprints/Heroes/BP_HeroBase.BP_HeroBase_C|GetHealth (Variables|Default|GetHeroEthRef)) (Variables|/Game/Dev/Gibran/Core/Blueprints/Heroes/BP_HeroBase.BP_HeroBase_C|GetHealth (Variables|Default|GetHeroHanRef)) (Variables|/Game/Dev/Gibran/Core/Blueprints/Heroes/BP_HeroBase.BP_HeroBase_C|GetHealth (Variables|Default|GetHeroShuRef)) (Variables|/Game/Dev/Gibran/Core/Blueprints/Heroes/BP_HeroBase.BP_HeroBase_C|GetHealth (Variables|Default|GetHeroBenRef)) (Variables|Default|GetTotalHealth)) (CallFunction|ReadDebugTag "Damage") false "(R=0.000000,G=1.000000,B=0.126143,A=1.000000)" 0.0 "GroupHealth")
      (CallFunction|CalculateMaxMovingSpeed))
    (:then_2
      (Utilities|FlowControl|FlipFlop
        (:A
          (Transformation|AddRelativeLocation _boxcollision "0.100000, 0, 0" false false))
        (:B
          (Transformation|AddRelativeLocation _boxcollision "-0.100000, 0, 0" false false))))))

(event Input|ActionEvents|InputActionAction1
  (params (Key :type Key%20Structure :default "None"))
  (bind _herobenref (Variables|Default|GetHeroBenRef))
  (bind _fainted (Variables|/Game/Dev/Gibran/Core/Blueprints/Heroes/BP_HeroBase.BP_HeroBase_C|GetFainted _herobenref))
  ;[0 0 0] Action Inputs
  (:Pressed
    (Variables|Default|SetHero1AbilityHolded false)
    (Utilities|FlowControl|RetriggerableDelay (Variables|Default|GetAbilityHoldingThreshold))
    (Variables|Default|SetHero1AbilityHolded true))
  (:Released
    (if (Variables|Default|GetHero1AbilityHolded)
      (if (Math|Boolean|NORBoolean (Variables|/Game/Dev/Gibran/Core/Blueprints/Heroes/BP_HeroBase.BP_HeroBase_C|GetInAbility2Cooldown _herobenref) _fainted)
        (Default|Action2 _herobenref))
      (elif (Math|Boolean|NORBoolean (Variables|/Game/Dev/Gibran/Core/Blueprints/Heroes/BP_HeroBase.BP_HeroBase_C|GetInAbility1Cooldown _herobenref) _fainted)
        (Default|Action1 _herobenref)))))

(event Input|ActionEvents|InputActionAction2
  (params (Key :type Key%20Structure :default "None"))
  (bind _heroethref (Variables|Default|GetHeroEthRef))
  (bind _fainted (Variables|/Game/Dev/Gibran/Core/Blueprints/Heroes/BP_HeroBase.BP_HeroBase_C|GetFainted _heroethref))
  ;[0 0 0] Action Inputs
  (:Pressed
    (Variables|Default|SetHero2AbilityHolded false)
    (Utilities|FlowControl|RetriggerableDelay (Variables|Default|GetAbilityHoldingThreshold))
    (Variables|Default|SetHero2AbilityHolded true))
  (:Released
    (if (Variables|Default|GetHero2AbilityHolded)
      (if (Math|Boolean|NORBoolean (Variables|/Game/Dev/Gibran/Core/Blueprints/Heroes/BP_HeroBase.BP_HeroBase_C|GetInAbility2Cooldown _heroethref) _fainted)
        (Default|Action2 _heroethref))
      (elif (Math|Boolean|NORBoolean (Variables|/Game/Dev/Gibran/Core/Blueprints/Heroes/BP_HeroBase.BP_HeroBase_C|GetInAbility1Cooldown _heroethref) _fainted)
        (Default|Action1 _heroethref)))))

(event Input|ActionEvents|InputActionAction3
  (params (Key :type Key%20Structure :default "None"))
  (bind _heroshuref (Variables|Default|GetHeroShuRef))
  (bind _fainted (Variables|/Game/Dev/Gibran/Core/Blueprints/Heroes/BP_HeroBase.BP_HeroBase_C|GetFainted _heroshuref))
  ;[0 0 0] Action Inputs
  (:Pressed
    (Variables|Default|SetHero3AbilityHolded false)
    (Utilities|FlowControl|RetriggerableDelay (Variables|Default|GetAbilityHoldingThreshold))
    (Variables|Default|SetHero3AbilityHolded true))
  (:Released
    (if (Variables|Default|GetHero3AbilityHolded)
      (if (Math|Boolean|NORBoolean (Variables|/Game/Dev/Gibran/Core/Blueprints/Heroes/BP_HeroBase.BP_HeroBase_C|GetInAbility2Cooldown _heroshuref) _fainted)
        (Default|Action2 _heroshuref))
      (elif (Math|Boolean|NORBoolean (Variables|/Game/Dev/Gibran/Core/Blueprints/Heroes/BP_HeroBase.BP_HeroBase_C|GetInAbility1Cooldown _heroshuref) _fainted)
        (Default|Action1 _heroshuref)))))

(event Input|ActionEvents|InputActionAction4
  (params (Key :type Key%20Structure :default "None"))
  (bind _herohanref (Variables|Default|GetHeroHanRef))
  (bind _fainted (Variables|/Game/Dev/Gibran/Core/Blueprints/Heroes/BP_HeroBase.BP_HeroBase_C|GetFainted _herohanref))
  ;[0 0 0] Action Inputs
  (:Pressed
    (Variables|Default|SetHero4AbilityHolded false)
    (Utilities|FlowControl|RetriggerableDelay (Variables|Default|GetAbilityHoldingThreshold))
    (Variables|Default|SetHero4AbilityHolded true))
  (:Released
    (if (Variables|Default|GetHero4AbilityHolded)
      (if (Math|Boolean|NORBoolean (Variables|/Game/Dev/Gibran/Core/Blueprints/Heroes/BP_HeroBase.BP_HeroBase_C|GetInAbility2Cooldown _herohanref) _fainted)
        (Default|Action2 _herohanref))
      (elif (Math|Boolean|NORBoolean (Variables|/Game/Dev/Gibran/Core/Blueprints/Heroes/BP_HeroBase.BP_HeroBase_C|GetInAbility1Cooldown _herohanref) _fainted)
        (Default|Action1 _herohanref)))))

(event Input|ActionEvents|InputActionInteractions
  (params (Key :type Key%20Structure :default "None"))
  ;[0 0 0] Action Inputs
)

(event Input|ActionEvents|InputActionPauseGame
  (params (Key :type Key%20Structure :default "None"))
  (bind _returnvalue (Game|GetPlayerController 0))
  (:Released
    (Game|SetGamePaused true)
    (bind _returnvalue_2 (UserInterface|CreateWidget "/Game/Dev/Gibran/Core/UI/WBP_PauseMenu.WBP_PauseMenu_C"))
    (UserInterface|Viewport|AddtoViewport _returnvalue_2 0)
    (Input|SetInputModeUIOnly _returnvalue _returnvalue_2 "DoNotLock")
    (Variables|/Script/Engine.PlayerController|SetbShowMouseCursor _returnvalue true)))

(event Input|AxisEvents|InputAxisMoveUp/Down
  (params (AxisValue :type Float%20%28single-precision%29))
  ;[0 0 0] Movement Inputs
  (Variables|Default|SetGroupWalkingSpeed (Math|Float|Absolute(Float) AxisValue))
  (Pawn|Input|AddMovementInput (Math|Vector|GetForwardVector (Variables|Default|GetDirectionArrow)) AxisValue false))

(event Input|AxisEvents|InputAxisMoveLeft/Right
  (params (AxisValue :type Float%20%28single-precision%29))
  ;[0 0 0] Movement Inputs
  (Pawn|Input|AddControllerYawInput (* AxisValue (Variables|Default|GetMaxRotationRate)))
  (Variables|Default|SetGroupRotationDirection AxisValue)
  (Variables|Default|SetGroupRotatingSpeed (Math|Float|Absolute(Float) AxisValue))
  (Variables|/Game/Dev/Gibran/Core/Blueprints/Heroes/BP_HeroBase.BP_HeroBase_C|SetDirection (Variables|Default|GetHeroHanRef) AxisValue)
  (Variables|/Game/Dev/Gibran/Core/Blueprints/Heroes/BP_HeroBase.BP_HeroBase_C|SetDirection (Variables|Default|GetHeroEthRef) AxisValue)
  (Variables|/Game/Dev/Gibran/Core/Blueprints/Heroes/BP_HeroBase.BP_HeroBase_C|SetDirection (Variables|Default|GetHeroShuRef) AxisValue)
  (Variables|/Game/Dev/Gibran/Core/Blueprints/Heroes/BP_HeroBase.BP_HeroBase_C|SetDirection (Variables|Default|GetHeroBenRef) AxisValue))

(event Input|KeyboardEvents|Tab
  (params (Key :type Key%20Structure :default "None"))
  ;[0.1823 0.7199 1] Debug
  (:Released
    (Default|ToggleDebugMode (Variables|Default|GetGameInstanceRef))))

(event Input|KeyboardEvents|LeftCtrl
  (params (Key :type Key%20Structure :default "None")))

(event Input|KeyboardEvents|CtrlF
  (params (Key :type Key%20Structure :default "None"))
  (bind _returnvalue (Game|GetPlayerController 0))
  ;[0.1823 0.7199 1] Debug
  (:Released
    (Variables|/Game/Dev/Gibran/Core/HeroesGameInstance.HeroesGameInstance_C|SetDebugMode (Variables|Default|GetGameInstanceRef) true)
    (bind _returnvalue_2 (UserInterface|CreateWidget "/Game/Dev/Gibran/Core/UI/WBP_DebugMenu.WBP_DebugMenu_C" (Game|GetPlayerController 0)))
    (UserInterface|Viewport|AddtoViewport _returnvalue_2 10)
    (Widget|SetFocus _returnvalue_2)
    (Input|SetInputModeUIOnly _returnvalue _returnvalue_2 "DoNotLock")
    (Variables|/Script/Engine.PlayerController|SetbShowMouseCursor _returnvalue true)))

(event Input|KeyboardEvents|LeftShift
  (params (Key :type Key%20Structure :default "None")))

(event Input|KeyboardEvents|CtrlSpaceBar
  (params (Key :type Key%20Structure :default "None"))
  (bind _camera (Variables|Default|GetCamera))
  (:Released
    (Widget|RemovefromParent (Variables|/Game/Bin/Blueprints/_Core/GM_BulletHell.GM_BulletHell_C|GetLevelStartPopupRef (Variables|Default|GetGameModeRef)))
    (bind _positionandzoom (Timeline|CameraAnimTimeline SetNewTime)
      (:Update
        (Transformation|SetRelativeLocation _camera (Math|Vector|MakeVector 0.0 (.Y (Math|Vector|BreakVector _positionandzoom)) (.X (Math|Vector|BreakVector _positionandzoom))) false false)
        (Class|CameraComponent|SetOrthoWidth _camera (.Z (Math|Vector|BreakVector _positionandzoom)))))))

(fn ConstructionScript)

(fn UpdateTotalHealth
  (bind _hudref (Variables|Default|GetHudRef))
  (bind _output_get (Variables|Default|SetTotalHealth (Math|Float|Clamp(Float) (+ (Variables|/Game/Dev/Gibran/Core/Blueprints/Heroes/BP_HeroBase.BP_HeroBase_C|GetHealth (Variables|Default|GetHeroHanRef)) (Variables|/Game/Dev/Gibran/Core/Blueprints/Heroes/BP_HeroBase.BP_HeroBase_C|GetHealth (Variables|Default|GetHeroEthRef)) (Variables|/Game/Dev/Gibran/Core/Blueprints/Heroes/BP_HeroBase.BP_HeroBase_C|GetHealth (Variables|Default|GetHeroShuRef)) (Variables|/Game/Dev/Gibran/Core/Blueprints/Heroes/BP_HeroBase.BP_HeroBase_C|GetHealth (Variables|Default|GetHeroBenRef))) 0.0 8e+02)))
  (Utilities|IsValid _hudref
    (:Is%20Valid
      (Default|SetHealthBars _hudref)
      (Default|SetFaintedStats _hudref))
    (:Is%20Not%20Valid
      _))
  (if (<= _output_get 0.0)
    (CallFunction|Die)))

(fn SetMovementSpeeds)

(fn CalculateMaxMovingSpeed
  (bind _heroesnotfainted (LocalVariables|GetHeroesNotFainted))
  (if (Variables|/Game/Dev/Gibran/Core/Blueprints/Heroes/BP_HeroBase.BP_HeroBase_C|GetFainted (Variables|Default|GetHeroHanRef))
    _
    (else
      (Utilities|Array|Add _heroesnotfainted false)))
  (if (Variables|/Game/Dev/Gibran/Core/Blueprints/Heroes/BP_HeroBase.BP_HeroBase_C|GetFainted (Variables|Default|GetHeroEthRef))
    _
    (else
      (Utilities|Array|Add _heroesnotfainted false)))
  (if (Variables|/Game/Dev/Gibran/Core/Blueprints/Heroes/BP_HeroBase.BP_HeroBase_C|GetFainted (Variables|Default|GetHeroShuRef))
    _
    (else
      (Utilities|Array|Add _heroesnotfainted false)))
  (if (Variables|/Game/Dev/Gibran/Core/Blueprints/Heroes/BP_HeroBase.BP_HeroBase_C|GetFainted (Variables|Default|GetHeroBenRef))
    (Utilities|Array|Add _heroesnotfainted false))
  (Variables|/Script/Engine.FloatingPawnMovement|SetMaxSpeed (Variables|Default|GetFloatingPawnMovement) (* (Math|Float|MapRangeClamped (Math|Conversions|ToFloat(Integer) (Utilities|Array|Length (LocalVariables|GetHeroesNotFainted))) 0.0 4.0 0.0 (Variables|Default|GetMaxMovingSpeed)) (Variables|Default|GetMovementSpeedMultiplier))))