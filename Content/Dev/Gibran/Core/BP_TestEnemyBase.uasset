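; Test base enemy with a Paper2D flipbook that idles, chases the hero group and fires projectile attacks.
; Timers drive wander or spline patrol outside chase radius, and straight or circling AIMoveTo chases inside it.
; While chasing, it queues the first data-driven action passing its conditions, running multi-step volleys through ShootingComponent; only range checks work, as line-of-sight and health are stubs.
; Damage triggers flash and knockback; debug mode draws radii and moves.
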(event Custom|Wander
  ;[1 1 1] Wandering movement
  (if (not (Variables|Default|GetChasingPlayer))
    (CallFunction|Moveto (.RandomLocation (Class|NavigationSystemV1|GetRandomPointinNavigableRadius (Transformation|GetActorLocation) (Variables|Default|GetWanderRadius) 0 0)) (Variables|Default|GetIdleMovementUpdateTime))))

(event Custom|Patrol
  (bind _patrolpoints (Variables|Default|GetPatrolPoints))
  ;[1 1 1] Patrolling movement
  (if (not (Variables|Default|GetChasingPlayer))
    (if (>= (Variables|Default|GetLastSelectedSplinePoint) (- (Utilities|Array|Length _patrolpoints) 1))
      (Variables|Default|SetLastSelectedSplinePoint 0))
    (CallFunction|Moveto (Utilities|Array|Get(acopy) _patrolpoints (Variables|Default|GetLastSelectedSplinePoint)) (Variables|Default|GetIdleMovementUpdateTime))
    (Math|Integer|IncrementInt (Variables|Default|GetLastSelectedSplinePoint))))

(event Custom|MoveTo
  (params (Location :type Vector) (Duration :type Float%20%28double-precision%29))
  (Utilities|IsDebugModeOn?
    (:Debug%20Mode%20On
      (Rendering|Debug|DrawDebugArrow (Transformation|GetActorLocation) Location 5e+01 "(R=1.000000,G=1.000000,B=1.000000,A=1.000000)" Duration 5.0))
    (:Debug%20Mode%20Off
      _))
  (AI|AIMoveTo self Location 0 5.0 false))

(event Custom|ChaseStraight
  ;[1 1 1] Chase straight to player
  (if (Variables|Default|GetChasingPlayer)
    (CallFunction|Moveto (Transformation|GetActorLocation (Variables|Default|GetPlayerRef)) (Variables|Default|GetChaseMovementUpdateTime))))

(event Custom|ChaseCircle
  (bind _playerref (Variables|Default|GetPlayerRef))
  (bind _circlearoundradius (Variables|Default|GetCircleAroundRadius))
  (bind _chasemovementupdatetime (Variables|Default|GetChaseMovementUpdateTime))
  (bind _returnvalue (+ _circlearoundradius 2e+02))
  (bind _cylinder (Variables|/Game/Dev/Gibran/Core/BP_TestHeroGroup.BP_TestHeroGroup_C|GetCylinder _playerref))
  (bind _returnvalue_2 (Transformation|GetWorldLocation _cylinder))
  (bind _point (CallFunction|RandomPointBetweenCircles _returnvalue_2 _circlearoundradius _returnvalue))
  ;[1 1 1] Chase around the player
  (if (Variables|Default|GetChasingPlayer)
    (CallFunction|Moveto _point _chasemovementupdatetime)
    (Utilities|IsDebugModeOn?
      (:Debug%20Mode%20On
        (Rendering|Debug|DrawDebugCircle _point _circlearoundradius 24 "(R=0.684353,G=0.000000,B=1.000000,A=1.000000)" _chasemovementupdatetime 2.0 "0.000000,1.000000,0.000000" "1.000000,0.000000,0.000000"))
      (:Debug%20Mode%20Off
        _))
    (Utilities|FlowControl|Delay 1.0)
    (CallFunction|ChaseCircle)))

(event Custom|EvaluateActions
  (if (Variables|Default|GetChasingPlayer)
    (if (not (Variables|Actions|GetQueuingAction))
      (bind _array_element (Utilities|Array|ForEachLoopwithBreak (Variables|Actions|GetActions) :!label _label)
        (:LoopBody
          (bind _allconditionsmet (CallFunction|EvaluateActionConditions _array_element))
          (if _allconditionsmet
            (Variables|Actions|SetQueuedAction _array_element)
            (Variables|Actions|SetQueuingAction true)
            (goto _label Break)))
        (:Completed
          (if (Variables|Actions|GetQueuingAction)
            (CallFunction|ExecuteAction (Variables|Actions|GetQueuedAction))
            (Utilities|FlowControl|Delay (.QueueTime (Utilities|Struct|BreakS_ActionData (Variables|Actions|GetQueuedAction))))
            (Variables|Actions|SetQueuingAction false)))))))

(event EventBeginPlay
  (bind _idlemovementupdatetime (Variables|Default|GetIdleMovementUpdateTime))
  (bind _returnvalue (Actor|GetActorOfClass "/Game/Dev/Gibran/Core/BP_TestHeroGroup.BP_TestHeroGroup_C"))
  (Variables|Default|SetPlayerRef _returnvalue)
  (Utilities|FlowControl|Delay (Math|Random|RandomFloatinRange 0.0 0.5))
  (Utilities|Time|SetTimerbyEvent (delegate Custom|EvaluateActions) (Variables|Actions|GetActionUpdateTime) true)
  (bind _aswbp_enemy_health_bar (Utilities|Casting|CastToWBP_EnemyHealthBar (UserInterface|GetWidget (Variables|Default|GetHealthBarWidget))))
  (Variables|/Game/Dev/Gibran/Core/UI/WBP_EnemyHealthBar.WBP_EnemyHealthBar_C|SetEnemyRef _aswbp_enemy_health_bar self)
  (Default|UpdateHealthBar _aswbp_enemy_health_bar)
  (switch Utilities|FlowControl|Switch|SwitchonE_IdleMovementMode (Variables|Default|GetIdleMovementMode)
    (:NewEnumerator1
      (bind _returnvalue_2 (Utilities|Time|SetTimerbyEvent (delegate Custom|Wander) _idlemovementupdatetime true 0.5 1.0))
      (Variables|Timers|SetIdleMovementTimer _returnvalue_2))
    (:NewEnumerator2
      (bind _returnvalue_3 (Utilities|Time|SetTimerbyEvent (delegate Custom|Patrol) _idlemovementupdatetime true 0.5 1.0))
      (Variables|Timers|SetIdleMovementTimer _returnvalue_3))))

(event EventTakeDamage
  (params (DamageCauser :type Actor%20Object%20Reference) (DamageInstigator :type Actor%20Object%20Reference) (BaseDamage :type Float%20%28double-precision%29) (KnockbackStrength :type Float%20%28double-precision%29) (DamageType :type E_DamageType%20Enum :default "NewEnumerator0"))
  (Utilities|FlipbookDamageFlash (Variables|Default|GetPaperFlipbook) 0.2
    (:__
      (Utilities|InstantKnockback 0 (Math|Vector|NegateVector (Math|Vector|GetForwardVector (Variables|Default|GetDirection))) 5e+01 true))))

(event EventTick
  (params (DeltaSeconds :type Float%20%28single-precision%29))
  (bind _returnvalue (Transformation|GetActorLocation))
  (bind _chaseradius (Variables|Default|GetChaseRadius))
  (bind _chasemovementupdatetime (Variables|Default|GetChaseMovementUpdateTime))
  (bind _direction (Variables|Default|GetDirection))
  (Transformation|SetWorldRotation (Variables|Default|GetPaperFlipbook) "0.000000,0.000000,-90.000000" false false)
  (Transformation|SetWorldRotation _direction (Math|Rotator|FindLookatRotation (Transformation|GetWorldLocation _direction) (Transformation|GetActorLocation (Variables|Default|GetPlayerRef))) false false)
  (Utilities|IsDebugModeOn?
    (:Debug%20Mode%20On
      (CallFunction|ToggleDebugComponentsVisibility true)
      (Rendering|Debug|DrawDebugCircle _returnvalue (Variables|Default|GetWanderRadius) 24 "(R=0.114583,G=0.641977,B=1.000000,A=1.000000)" 0.0 1.0 "0.000000,1.000000,0.000000" "1.000000,0.000000,0.000000")
      (Rendering|Debug|DrawDebugCircle _returnvalue _chaseradius 24 "(R=1.000000,G=0.315589,B=0.000000,A=1.000000)" 0.0 1.0 "0.000000,1.000000,0.000000" "1.000000,0.000000,0.000000")
      (Rendering|Debug|DrawDebugCircle _returnvalue (Variables|Default|GetMeleeScanRadius) 24 "(R=1.000000,G=0.000000,B=0.049470,A=1.000000)" 0.0 1.0 "0.000000,1.000000,0.000000" "1.000000,0.000000,0.000000"))
    (:Debug%20Mode%20Off
      (CallFunction|ToggleDebugComponentsVisibility false)))
  (if (<= (Math|Vector|Distance(Vector) _returnvalue (Transformation|GetActorLocation (Variables|Default|GetPlayerRef))) _chaseradius)
    (Variables|Default|SetChasingPlayer true)
    (Utilities|FlowControl|DoOnce false :!label _label
      (:Completed
        (switch Utilities|FlowControl|Switch|SwitchonE_ChaseMovementMode (Variables|Default|GetChaseMovementMode)
          (:NewEnumerator3
            (bind _returnvalue_2 (Utilities|Time|SetTimerbyEvent (delegate Custom|ChaseCircle) _chasemovementupdatetime))
            (Variables|Timers|SetChaseMovementTimer _returnvalue_2))
          (:NewEnumerator4
            (bind _returnvalue_3 (Utilities|Time|SetTimerbyEvent (delegate Custom|ChaseStraight) _chasemovementupdatetime true))
            (Variables|Timers|SetChaseMovementTimer _returnvalue_3)))))
    (else
      (Variables|Default|SetChasingPlayer false)
      (Utilities|Time|ClearandInvalidateTimerbyHandle (Variables|Timers|GetChaseMovementTimer))
      (goto _label Reset))))

(event Game|Damage|EventPointDamage
  (params (Damage :type Float%20%28single-precision%29) (DamageType :type Damage%20Type%20Object%20Reference) (HitLocation :type Vector :default "0, 0, 0") (HitNormal :type Vector :default "0, 0, 0") (HitComponent :type Primitive%20Component%20Object%20Reference) (BoneName :type Name :default "None") (ShotFromDirection :type Vector :default "0, 0, 0") (InstigatedBy :type Controller%20Object%20Reference) (DamageCauser :type Actor%20Object%20Reference) (HitInfo :type Hit%20Result%20Structure%20%28by%20ref%29)))

(event Custom|ExecuteAction
  (params (ActionData :type S%20Action%20Data%20Structure))
  (bind (_actionname _type _canskipqueuing _queuetime _targets _duration _conditions _rangeconditions _lineofsightconditions _projectileactiondata) (Utilities|Struct|BreakS_ActionData ActionData))
  (bind _shootingcomponent (Variables|Default|GetShootingComponent))
  (switch Utilities|FlowControl|Switch|SwitchonE_ActionType _type
    (:NewEnumerator0
      (Variables|Default|SetActionStepIndex 0)
      (Variables|Default|SetActionSubStepIndex 0 :!label _label)
      (Variables|/Game/Bin/Blueprints/Character/BP_Shooting_Component.BP_Shooting_Component_C|SetShootRays _shootingcomponent (.Rays (Utilities|Struct|BreakS_ActionProjectileBurst (Utilities|Array|Get(acopy) _projectileactiondata (Variables|Default|GetActionStepIndex)))))
      (Variables|/Game/Bin/Blueprints/Character/BP_Shooting_Component.BP_Shooting_Component_C|SetShootAngle _shootingcomponent (.Angle (Utilities|Struct|BreakS_ActionProjectileBurst (Utilities|Array|Get(acopy) _projectileactiondata (Variables|Default|GetActionStepIndex)))))
      (Variables|/Game/Bin/Blueprints/Character/BP_Shooting_Component.BP_Shooting_Component_C|SetEquirradial _shootingcomponent (.Equiradial (Utilities|Struct|BreakS_ActionProjectileBurst (Utilities|Array|Get(acopy) _projectileactiondata (Variables|Default|GetActionStepIndex)))))
      (if (Utilities|IsValidClass (.ProjectileClass (Utilities|Struct|BreakS_ActionProjectileBurst (Utilities|Array|Get(acopy) _projectileactiondata (Variables|Default|GetActionStepIndex)))))
        (Default|ShootOnceProjectileClass _shootingcomponent (.ProjectileClass (Utilities|Struct|BreakS_ActionProjectileBurst (Utilities|Array|Get(acopy) _projectileactiondata (Variables|Default|GetActionStepIndex)))) :!label _label_2)
        (Utilities|FlowControl|Delay (.FireRate (Utilities|Struct|BreakS_ActionProjectileBurst (Utilities|Array|Get(acopy) _projectileactiondata (Variables|Default|GetActionStepIndex)))))
        (bind _result (Math|Integer|IncrementInt (Variables|Default|GetActionSubStepIndex))
          (:%20%20
            (if (>= _result (.Ammount (Utilities|Struct|BreakS_ActionProjectileBurst (Utilities|Array|Get(acopy) _projectileactiondata (Variables|Default|GetActionStepIndex)))))
              (Utilities|FlowControl|Delay (.DelayUntilNext (Utilities|Struct|BreakS_ActionProjectileBurst (Utilities|Array|Get(acopy) _projectileactiondata (Variables|Default|GetActionStepIndex)))))
              (Math|Integer|IncrementInt (Variables|Default|GetActionStepIndex)
                (:%20%20
                  (if (>= (Variables|Default|GetActionStepIndex) (Utilities|Array|Length _projectileactiondata))
                    (Variables|Default|SetActionStepIndex 0)
                    (Variables|Default|SetActionSubStepIndex 0)
                    (else
                      (goto _label)))))
              (else
                (goto _label_2)))))))))

(fn ConstructionScript
  (bind _patrolspline (Variables|Default|GetPatrolSpline))
  (for _index (range 1 (Spline|GetNumberOfSplinePoints _patrolspline))
    (Utilities|Array|Add (Variables|Default|GetPatrolPoints) (Spline|GetLocationatSplinePoint _patrolspline (- _index 1) "World"))))

(fn FCallFunctionbyName
  (params (FunctionName :type String))
  (bind _returnvalue (Utilities|Time|SetTimerbyFunctionName 0 FunctionName 0.0001))
  (Utilities|Time|ClearandInvalidateTimerbyHandle _returnvalue))

(fn EvaluateRangeConditions
  (params (RangeConditions :type S%20Range%20Conditions%20Structure))
  (bind _targetspecifications (Utilities|Struct|BreakS_RangeConditions RangeConditions))
  (bind _locdistances (LocalVariables|GetlocDistances))
  (bind (_targetspecifications_2 _mindistance _maxdistance _rule) (Utilities|Struct|BreakS_RangeConditions RangeConditions))
  (bind (_foundalltargets _singletarget _multipletargets) (CallFunction|GetTargetsfromSpecifications _targetspecifications))
  (if _foundalltargets
    (LocalVariables|SetlocTargets _multipletargets)
    (LocalVariables|SetlocTarget _singletarget)
    (switch Utilities|FlowControl|Switch|SwitchonE_ActionTarget (.Target (Utilities|Struct|BreakS_ActionTargetSpecifications _targetspecifications))
      (:NewEnumerator2
        (LocalVariables|SetlocDistance (Math|Vector|Distance(Vector) (Transformation|GetActorLocation) (Transformation|GetActorLocation (Variables|Default|GetPlayerRef))))
        (switch Utilities|FlowControl|Switch|SwitchonE_NumberRangePreference _rule :!label _label
          (:NewEnumerator0
            (LocalVariables|SetlocSuccess (>= (LocalVariables|GetlocDistance) _mindistance)))
          (:NewEnumerator1
            (LocalVariables|SetlocSuccess (Math|Float|InRange(Float) (LocalVariables|GetlocDistance) _mindistance _maxdistance)))
          (:NewEnumerator2
            (LocalVariables|SetlocSuccess (<= (LocalVariables|GetlocDistance) _maxdistance))))
        (return (LocalVariables|GetlocSuccess)))
      (:NewEnumerator0
        (LocalVariables|SetlocDistance (Math|Vector|Distance(Vector) (Transformation|GetActorLocation) (Transformation|GetActorLocation (LocalVariables|GetlocTarget))) :!label _label_2)
        (goto _label))
      (:NewEnumerator8
        (goto _label_2))
      (:NewEnumerator1
        (bind _output_get (LocalVariables|SetlocSuccess true))
        (return _output_get))
      (:NewEnumerator3
        _)
      (:NewEnumerator4
        _)
      (:NewEnumerator7
        (goto _label_2))
      (:NewEnumerator5
        _)
      (:NewEnumerator6
        (goto _label_2)))
    (for _array_element (LocalVariables|GetlocTargets)
      (Utilities|Array|Add (LocalVariables|GetlocDistances) (Math|Vector|Distance(Vector) (Transformation|GetActorLocation _array_element) (Transformation|GetActorLocation))))
    (switch Utilities|FlowControl|Switch|SwitchonE_NumberRangePreference _rule
      (:NewEnumerator0
        (LocalVariables|SetlocSuccess (>= (.MinValue (Math|Float|MinOfFloatArray _locdistances)) _mindistance))
        (return (LocalVariables|GetlocSuccess)))
      (:NewEnumerator1
        (bind _array_element_2 (Utilities|Array|ForEachLoopwithBreak _locdistances :!label _label_3)
          (:LoopBody
            (if (Math|Float|InRange(Float) _array_element_2 _mindistance _maxdistance)
              (LocalVariables|SetlocSuccess true)
              (else
                (LocalVariables|SetlocSuccess false)
                (goto _label_3 Break))))
          (:Completed
            (return (LocalVariables|GetlocSuccess)))))
      (:NewEnumerator2
        (LocalVariables|SetlocSuccess (<= (.MaxValue (Math|Float|MaxOfFloatArray _locdistances)) _maxdistance))
        (return (LocalVariables|GetlocSuccess))))
    (else
      (return false))))

(fn EvaluateLineOfSightConditions
  (return false))

(fn EvaluatePlayerHealthConditions
  (return false))

(fn EvaluateActionConditions
  (params (ActionData :type S%20Action%20Data%20Structure))
  (bind (_actionname _type _canskipqueuing _queuetime _targets _duration _conditions _rangeconditions) (Utilities|Struct|BreakS_ActionData ActionData))
  (bind _array_element (Utilities|Array|ForEachLoopwithBreak _conditions :!label _label)
    (:LoopBody
      (switch Utilities|FlowControl|Switch|SwitchonE_ConditionTypes _array_element
        (:NewEnumerator0
          (bind _success (CallFunction|EvaluateRangeConditions _rangeconditions))
          (if _success
            (LocalVariables|SetlocSucces true)
            (else
              (LocalVariables|SetlocSucces false)
              (goto _label Break))))
        (:NewEnumerator1
          (CallFunction|EvaluateLineOfSightConditions))
        (:NewEnumerator2
          (CallFunction|EvaluatePlayerHealthConditions))))
    (:Completed
      (return (LocalVariables|GetlocSucces)))))

(fn ToggleDebugComponentsVisibility
  (params (Visibility :type Boolean))
  (Rendering|SetVisibility (Variables|Default|GetDirection) Visibility false)
  (Rendering|SetVisibility (Variables|Default|GetHealthBarWidget) Visibility false))

(fn GetTargetsfromSpecifications
  (params (TargetSpecifications :type S%20Action%20Target%20Specifications%20Structure))
  (bind (_target _targethero _targetenemyclass _targetenemy _targetactorclass _targetactor _quantitypreference _minquantity _maxquantity _quantityrangepreference _maxrange) (Utilities|Struct|BreakS_ActionTargetSpecifications TargetSpecifications))
  (bind (_target_2 _targethero_2 _targetenemyclass_2 _targetenemy_2 _targetactorclass_2 _targetactor_2 _quantitypreference_2 _minquantity_2 _maxquantity_2 _quantityrangepreference_2) (Utilities|Struct|BreakS_ActionTargetSpecifications TargetSpecifications))
  (switch Utilities|FlowControl|Switch|SwitchonE_ActionTarget _target
    (:NewEnumerator2
      (LocalVariables|SetLocSingleTarget (Variables|Default|GetPlayerRef))
      (bind _output_get (LocalVariables|SetlocFoundAllTargets true :!label _label))
      (return _output_get (LocalVariables|GetLocSingleTarget) 0))
    (:NewEnumerator0
      (bind (_foundactor _closestactor) (CallFunction|ClosestActorOfClass "/Game/Dev/Gibran/Core/BP_TestHeroBase.BP_TestHeroBase_C" (Transformation|GetActorLocation) _maxrange))
      (if _foundactor
        (LocalVariables|SetLocSingleTarget _closestactor)
        (goto _label)))
    (:NewEnumerator8
      (bind _array_element (Utilities|Array|ForEachLoopwithBreak (Actor|GetComponentsByClass (Variables|Default|GetPlayerRef) "/Script/Engine.ChildActorComponent") :!label _label_2)
        (:LoopBody
          (if (== (Variables|/Script/Engine.ChildActorComponent|GetChildActorClass _array_element) (.TargetHero (Utilities|Struct|BreakS_ActionTargetSpecifications TargetSpecifications)))
            (LocalVariables|SetLocSingleTarget (Variables|/Script/Engine.ChildActorComponent|GetChildActor _array_element))
            (goto _label_2 Break)))
        (:Completed
          (bind _output_get_2 (LocalVariables|SetlocFoundAllTargets true :!label _label_3))
          (return _output_get_2 (LocalVariables|GetLocSingleTarget) 0))))
    (:NewEnumerator1
      (LocalVariables|SetLocSingleTarget self)
      (goto _label_3))
    (:NewEnumerator3
      (bind _outactors (Actor|GetAllActorsOfClass (Utilities|GetClass self)))
      (LocalVariables|SetlocAnalisingActors _outactors)
      (if (Utilities|Array|IsEmpty (LocalVariables|GetlocAnalisingActors)) :!label _label_4
        (bind _output_get_3 (LocalVariables|SetlocFoundAllTargets false))
        (return _output_get_3 0 0)
        (else
          (switch Utilities|FlowControl|Switch|SwitchonE_QuantityPreference _quantitypreference_2
            (:NewEnumerator0
              (bind _output_get_4 (LocalVariables|SetLocSingleTarget (Utilities|Array|Get(acopy) (LocalVariables|GetlocAnalisingActors))))
              (bind _output_get_5 (LocalVariables|SetlocFoundAllTargets true))
              (return _output_get_5 _output_get_4 0))
            (:NewEnumerator1
              (switch Utilities|FlowControl|Switch|SwitchonE_NumberRangePreference _quantityrangepreference_2
                (:NewEnumerator0
                  (if (>= (Utilities|Array|Length (LocalVariables|GetlocAnalisingActors)) _minquantity_2)
                    _
                    (else
                      (bind _output_get_6 (LocalVariables|SetlocFoundAllTargets false :!label _label_5))
                      (return _output_get_6 0 0))))
                (:NewEnumerator1
                  (if (>= (Utilities|Array|Length (LocalVariables|GetlocAnalisingActors)) _minquantity_2)
                    (if (>= (Utilities|Array|Length (LocalVariables|GetlocAnalisingActors)) _maxquantity_2)
                      (Utilities|Array|Resize (LocalVariables|GetlocAnalisingActors) _maxquantity_2))
                    (else
                      (goto _label_5))))
                (:NewEnumerator2
                  (if (and (> (Utilities|Array|Length (LocalVariables|GetlocAnalisingActors)) 0) (<= (Utilities|Array|Length (LocalVariables|GetlocAnalisingActors)) _maxquantity_2))
                    (Utilities|Array|Resize (LocalVariables|GetlocAnalisingActors) _maxquantity_2)
                    (else
                      (goto _label_5)))))
              (bind _output_get_7 (LocalVariables|SetLocMultipleTargets (LocalVariables|GetlocAnalisingActors)))
              (bind _output_get_8 (LocalVariables|SetlocFoundAllTargets true))
              (return _output_get_8 0 _output_get_7))
            (:NewEnumerator2
              (bind _output_get_9 (LocalVariables|SetLocMultipleTargets (LocalVariables|GetlocAnalisingActors)))
              (bind _output_get_10 (LocalVariables|SetlocFoundAllTargets true))
              (return _output_get_10 0 _output_get_9))))))
    (:NewEnumerator4
      (bind _outactors_2 (Actor|GetAllActorsOfClass _targetenemyclass))
      (LocalVariables|SetlocAnalisingActors _outactors_2)
      (goto _label_4))
    (:NewEnumerator7
      (LocalVariables|SetLocSingleTarget _targetenemy)
      (bind _output_get_11 (LocalVariables|SetlocFoundAllTargets true :!label _label_6))
      (return _output_get_11 (LocalVariables|GetLocSingleTarget) 0))
    (:NewEnumerator5
      (bind _outactors_3 (Actor|GetAllActorsOfClass _targetactorclass))
      (LocalVariables|SetlocAnalisingActors _outactors_3)
      (goto _label_4))
    (:NewEnumerator6
      (LocalVariables|SetLocSingleTarget _targetactor)
      (goto _label_6))))

(fn HasActionsThatSkipQueue
  (for _array_element (Variables|Actions|GetActions)
    (if (.CanSkipQueuing (Utilities|Struct|BreakS_ActionData _array_element))
      (Variables|Default|SetHasSkipableActions true))))