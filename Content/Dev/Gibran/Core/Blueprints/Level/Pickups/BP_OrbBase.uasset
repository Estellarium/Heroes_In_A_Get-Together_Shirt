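; Base pickup orb that scatters on spawn and is collected when a hero overlaps it.
; On BeginPlay it picks a random direction and distance, then a timeline lerps it there with smooth or linear easing.
; Tick keeps the sprite's rotation fixed and, if FloatToHero is set, drifts it toward the closest hero when the hero group is within pickup radius.
; Overlap plays a sound and calls OrbPickup, meant for child overrides, which destroys the orb by default.
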(event OnComponentBeginOverlap(Capsule)
  (params (OverlappedComponent :type Primitive%20Component%20Object%20Reference) (OtherActor :type Actor%20Object%20Reference) (OtherComp :type Primitive%20Component%20Object%20Reference) (OtherBodyIndex :type Integer) (bFromSweep :type Boolean) (SweepResult :type Hit%20Result%20Structure%20%28by%20ref%29))
  (bind _asbp_hero_base (Utilities|Casting|CastToBP_HeroBase OtherActor))
  (Audio|PlaySound2D (Variables|Default|GetPickupSound) 1.0 1.0 0.0 0 0)
  (CallFunction|OrbPickup _asbp_hero_base))

(event Custom|OrbPickup
  (params (Hero :type BP%20Hero%20Base%20Object%20Reference))
  ;[1 1 1] Override in child
  (Actor|DestroyActor))

(event EventBeginPlay
  (bind _output_get (Variables|Default|SetStartLocation (Transformation|GetActorLocation)))
  (Transformation|SetActorRotation (Math|Rotator|MakeRotator 0.0 0.0 (.Yaw (Math|Rotator|BreakRotator (Math|Random|RandomRotator false)))))
  (Variables|Default|SetTargetLocation (+ _output_get (* (Transformation|GetActorForwardVector) (Math|Random|RandomFloatinRange (Variables|Default|GetSpreadMinRadius) (Variables|Default|GetSpreadMaxRadius)))))
  (Variables|Default|SetHeroGroupRef (CallFunction|GetHeroesGroup))
  (bind (_direction _alphasmooth _alphalinear) (Timeline|InitialMovementTimeline Play)
    (:Update
      (Transformation|SetActorLocation (Math|Vector|Lerp(Vector) (Variables|Default|GetStartLocation) (Variables|Default|GetTargetLocation) (select (Variables|Default|GetSmoothMovement) _alphasmooth _alphalinear)) false false))))

(event EventTick
  (params (DeltaSeconds :type Float%20%28single-precision%29))
  (bind _returnvalue (Transformation|GetActorLocation))
  (bind _returnvalue_2 (Transformation|GetActorLocation))
  (bind _floatpickupradius (Variables|Default|GetFloatPickupRadius))
  (Transformation|SetWorldRotation (Variables|Default|GetPaperSprite) "0, 0,-90.000000" false false)
  (if (Variables|Default|GetFloatToHero)
    (if (<= (Math|Vector|Distance(Vector) _returnvalue_2 (Transformation|GetActorLocation (Variables|Default|GetHeroGroupRef))) _floatpickupradius)
      (Transformation|SetActorRotation (Math|Rotator|MakeRotator 0.0 0.0 (.yaw (Math|Rotator|FindLookatRotation _returnvalue (Transformation|GetActorLocation (.ClosestActor (CallFunction|ClosestActorOfClass "/Game/Dev/Gibran/Core/Blueprints/Heroes/BP_HeroBase.BP_HeroBase_C" _returnvalue_2 _floatpickupradius)))))))
      (Transformation|SetActorLocation (+ _returnvalue (* (Transformation|GetActorForwardVector) 2.0)) false false))))

(fn ConstructionScript)