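; Base power-up pickup that grants a timed enhancement to a hero or hero group on overlap, then destroys itself.
; The construction script applies the configured sprite, and a timeline started on BeginPlay drives its floating offset along relative Y.
; Overlaps count only when the actor's exact class matches the Classes map entry for Target.
; Casts then route Duration to either BP_HeroBase's hero enhancement or BP_HeroGroup's group enhancement.
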(event OnComponentBeginOverlap(CollisionBox)
  (params (OverlappedComponent :type Primitive%20Component%20Object%20Reference) (OtherActor :type Actor%20Object%20Reference) (OtherComp :type Primitive%20Component%20Object%20Reference) (OtherBodyIndex :type Integer) (bFromSweep :type Boolean) (SweepResult :type Hit%20Result%20Structure%20%28by%20ref%29))
  (bind _duration (Variables|Default|GetDuration))
  (if (== (Utilities|GetClass OtherActor) (.Value (Utilities|Map|Find (Variables|Default|GetClasses) (Variables|Default|GetTarget))))
    (bind _asbp_hero_base (Utilities|Casting|CastToBP_HeroBase OtherActor)
      (:then
        (Default|TriggerHeroEnhancement _asbp_hero_base _duration))
      (:CastFailed
        (bind _asbp_hero_group_remake (Utilities|Casting|CastToBP_HeroGroup OtherActor))
        (Default|TriggerGroupEnhancement _asbp_hero_group_remake _duration)))
    (Actor|DestroyActor)))

(event EventBeginPlay
  (bind _height (Timeline|FloatingTimeline Play)
    (:Update
      (Transformation|SetRelativeLocation (Variables|Default|GetPickupSprite) (Math|Vector|MakeVector 0.0 (Math|Float|Lerp 0.0 -4e+01 _height) 0.0) false false))))

(fn ConstructionScript
  (Rendering|Components|Sprite|SetSprite (Variables|Default|GetPickupSprite) (Variables|Default|GetSprite)))