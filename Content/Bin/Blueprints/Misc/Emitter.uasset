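; Emitter actor that repeatedly spawns a Particle actor at its own location and rotation at irregular intervals.
; On BeginPlay it sets a one-shot timer with a random delay of a few seconds or more.
; When the timer fires, Emit spawns the actor regardless of collision, clears the handle and restarts the timer, re-rolling the delay each cycle instead of using a fixed loop.
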(event Custom|Emit
  (bind _returnvalue (Transformation|GetActorTransform))
  (Game|SpawnActorfromClass "/Game/Bin/Blueprints/Misc/Particle.Particle_C" (Math|Transform|MakeTransform (.location _returnvalue) (.rotation _returnvalue) "1.000000,1.000000,1.000000") "AlwaysSpawn" 0 0)
  (Utilities|Time|ClearandInvalidateTimerbyHandle (Variables|Default|GetTimer))
  (CallFunction|StartTimer))

(event Custom|Start%20Timer
  (bind _returnvalue (Utilities|Time|SetTimerbyEvent (delegate Custom|Emit) (Math|Random|RandomFloatinRange 5.0 2e+01)))
  (Variables|Default|SetTimer _returnvalue))

(event EventBeginPlay
  (CallFunction|StartTimer))

(fn ConstructionScript)