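; Debug test actor that visually and numerically checks the RandomWeightedInteger and RandomPointInCircle helpers.
; On BeginPlay it draws 1000 weighted picks among four options, plotting each as a colored debug point at a random spot inside that option's circle and counting hits.
; It then prints each option's weight, expected count from SumOfWeights and actual frequency for comparison.
; Tick redraws the four circle outlines along the actor's Y axis.
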(event EventBeginPlay
  (bind _returnvalue (Transformation|GetActorLocation))
  (bind _map (Utilities|Map|MakeMap 0 1e+01 1 5.0 2 2.5 3 15.0))
  (bind _sum (CallFunction|SumOfWeights _map))
  (for _index (range 0 999)
    (bind _output_get (Variables|Default|SetChosenNum (CallFunction|RandomWeightedInteger _map)))
    (Rendering|Debug|DrawDebugPoint (Utilities|Select :Index _output_get :Option%200 (CallFunction|RandomPointinCircle (Math|Vector|MakeVector (.x _returnvalue) (+ (.y _returnvalue) 0.0) (.z _returnvalue)) 2e+02) :Option%201 (CallFunction|RandomPointinCircle (Math|Vector|MakeVector (.x _returnvalue) (+ (.y _returnvalue) 4e+02) (.z _returnvalue)) 2e+02) :Option%202 (CallFunction|RandomPointinCircle (Math|Vector|MakeVector (.x _returnvalue) (+ (.y _returnvalue) 8e+02) (.z _returnvalue)) 2e+02) :Option%203 (CallFunction|RandomPointinCircle (Math|Vector|MakeVector (.x _returnvalue) (+ (.y _returnvalue) 1.2e+03) (.z _returnvalue)) 2e+02)) 5.0 (Utilities|Select :Index _output_get :Option%200 "(R=0.019608,G=1.000000,B=0.000000,A=1.000000)" :Option%201 "(R=0.000000,G=0.876143,B=1.000000,A=1.000000)" :Option%202 "(R=0.984314,G=0.000000,B=1.000000,A=1.000000)" :Option%203 "(R=1.000000,G=0.823529,B=0.000000,A=1.000000)") 3e+01)
    (switch int _output_get
      (:0
        (Math|Integer|IncrementInt (Variables|Default|GetNum0Chosen)))
      (:1
        (Math|Integer|IncrementInt (Variables|Default|GetNum1Chosen)))
      (:2
        (Math|Integer|IncrementInt (Variables|Default|GetNum2Chosen)))
      (:3
        (Math|Integer|IncrementInt (Variables|Default|GetNum3Chosen)))))
  (Development|PrintText (Utilities|Text|FormatText " 
Number 1 weight: {w1}, expected: {e1}, frequency: {f1} 
Number 2 weight: {w2}, expected: {e2}, frequency: {f2} 
Number 3 weight: {w3}, expected: {e3}, frequency: {f3} 
Number 4 weight: {w4}, expected: {e4}, frequency: {f4}" (Math|Float|MakeLiteralFloat 1e+01) (/ 1e+03 (/ _sum 1e+01)) (Variables|Default|GetNum0Chosen) (Math|Float|MakeLiteralFloat 5.0) (/ 1e+03 (/ _sum 5.0)) (Variables|Default|GetNum1Chosen) (Math|Float|MakeLiteralFloat 2.5) (/ 1e+03 (/ _sum 2.5)) (Variables|Default|GetNum2Chosen) (Math|Float|MakeLiteralFloat 15.0) (/ 1e+03 (/ _sum 15.0)) (Variables|Default|GetNum3Chosen)) true true "(R=0.000000,G=0.660000,B=1.000000,A=1.000000)" 3e+01))

(event EventTick
  (params (DeltaSeconds :type Float%20%28single-precision%29))
  (bind _returnvalue (Transformation|GetActorLocation))
  (Rendering|Debug|DrawDebugCircle (Math|Vector|MakeVector (.x _returnvalue) (+ (.y _returnvalue) 0.0) (.z _returnvalue)) 2e+02 48 "(R=0.000000,G=1.000000,B=0.004274,A=1.000000)" 0.0 3.0 "0.000000,1.000000,0.000000" "1.000000,0.000000,0.000000")
  (Rendering|Debug|DrawDebugCircle (Math|Vector|MakeVector (.x _returnvalue) (+ (.y _returnvalue) 4e+02) (.z _returnvalue)) 2e+02 48 "(R=0.000000,G=0.930072,B=1.000000,A=1.000000)" 0.0 3.0 "0.000000,1.000000,0.000000" "1.000000,0.000000,0.000000")
  (Rendering|Debug|DrawDebugCircle (Math|Vector|MakeVector (.x _returnvalue) (+ (.y _returnvalue) 8e+02) (.z _returnvalue)) 2e+02 48 "(R=1.000000,G=0.000000,B=0.733442,A=1.000000)" 0.0 3.0 "0.000000,1.000000,0.000000" "1.000000,0.000000,0.000000")
  (Rendering|Debug|DrawDebugCircle (Math|Vector|MakeVector (.x _returnvalue) (+ (.y _returnvalue) 1.2e+03) (.z _returnvalue)) 2e+02 48 "(R=1.000000,G=0.867631,B=0.000000,A=1.000000)" 0.0 3.0 "0.000000,1.000000,0.000000" "1.000000,0.000000,0.000000"))

(fn ConstructionScript)