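; Base projectile actor with a sprite or flipbook, configured through SetVariables with difficulty-based damage and reused via Activate and Deactivate.
; A timeline with a swappable vector curve, stretched by speed and lifespan and rotated to the actor's facing, drives its trajectory.
; While active, a gate passes capsule overlaps to apply random-range damage and knockback, with shields blocking damage.
; Expiry or destroy-on-impact hits notify the GameMode instead of destroying the actor.
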(event OnComponentBeginOverlap(Capsule)
  (params (OverlappedComponent :type Primitive%20Component%20Object%20Reference) (OtherActor :type Actor%20Object%20Reference) (OtherComp :type Primitive%20Component%20Object%20Reference) (OtherBodyIndex :type Integer) (bFromSweep :type Boolean) (SweepResult :type Hit%20Result%20Structure%20%28by%20ref%29))
  (bind _parent (Variables|PostSpawn|GetParent))
  (Utilities|IsValid OtherActor
    (:Is%20Valid
      (switch name (Collision|GetCollisionProfileName OtherComp)
        (:Hero
          (Variables|Default|SetHitCharacter true :!label _label))
        (:Enemy
          (goto _label))
        (:HeroShield
          (Variables|Default|SetHitCharacter false))
        (:Destructible
          (goto _label)))
      (Utilities|FlowControl|Gate true
        (:Exit
          (Utilities|IsValid OtherActor
            (:Is%20Valid
              (if (not (== (Utilities|GetClass OtherActor) 0))
                (if (Variables|Default|GetHitCharacter)
                  (bind _output_get (Variables|Default|SetAppliedDamage (Math|Random|RandomFloatinRange (Variables|Stats|GetMinDamage) (Variables|Stats|GetMaxDamage))))
                  (Class|BPIDamageableActor|TakeDamage(Message) OtherActor self (select (Utilities|IsValid _parent) (Game|GetInstigatorController _parent) 0) _output_get (Variables|Stats|GetKnockback%20Strength) (Variables|Stats|GetDamageType) (Transformation|GetActorForwardVector))
                  (CallFunction|SwitchDamageStat (Collision|GetCollisionObjectType (Variables|Default|GetCapsule)) (Variables|Default|GetAppliedDamage))
                  (Development|PrintText (Utilities|Text|FormatText "Projectile applied damage: 
Base damage: {bd} 
Damage variance: {dv} 
Applied damage: {ad}" (Variables|Stats|GetMinDamage) (Variables|Stats|GetMaxDamage) (Variables|Default|GetAppliedDamage)) (CallFunction|ReadDebugTag "Damage") false "(R=1.000000,G=0.207221,B=0.000000,A=1.000000)" 1e+01 "ProjectileAppliedDamage"))
                (if (Variables|Default|GetDestroyOnImpact) :!label _label_2
                  (CallFunction|OnDeath)
                  (Development|PrintText (Utilities|Text|FormatText "Actor {ActorName} damaged" (Utilities|GetDisplayName OtherActor)) (CallFunction|ReadDebugTag "Damage") true "(R=0.475202,G=0.000000,B=1.000000,A=1.000000)" 2.0 "ProjectileHit"))))
            (:Is%20Not%20Valid
              (goto _label_2))))))))

(event Custom|Set%20New%20Sprite
  (params (NewSprite :type Paper%20Sprite%20Object%20Reference) (InColor :type Color%20Structure))
  (bind _spritecomponent (Variables|Default|GetSpriteComponent))
  (Rendering|Components|Sprite|SetSprite _spritecomponent NewSprite)
  (Sprite|SetSpriteColor _spritecomponent (Math|Conversions|ToLinearColor(Color) InColor)))

(event Custom|Deactivate
  (bind _parent (Variables|PostSpawn|GetParent))
  (Utilities|FlowControl|Sequence
    (:then_0
      (bind _movementcurve (Timeline|Movement Stop)
        (:Update
          (CallFunction|Update (CallFunction|CalculateLocation _movementcurve)))
        (:Finished
          (CallFunction|OnDeath))))
    (:then_1
      (Utilities|FlowControl|Gate true) ; enters at Close
    )))

(event Custom|Activate
  (bind _parent (Variables|PostSpawn|GetParent))
  (Variables|PostSpawn|SetInitPos (Transformation|GetActorLocation))
  (Utilities|FlowControl|Sequence
    (:then_0
      (bind _movementcurve (Timeline|Movement PlayFromStart)
        (:Update
          (CallFunction|Update (CallFunction|CalculateLocation _movementcurve)))
        (:Finished
          (CallFunction|OnDeath))))
    (:then_1
      (Utilities|FlowControl|Gate true) ; enters at Open
    )))

(event Custom|Update
  (params (NewLocation :type Vector))
  (Transformation|SetActorLocation NewLocation false false))

(event Custom|OnDeath
  (Development|PrintString "died")
  (Utilities|FlowControl|Delay 0.001)
  (CallFunction|DestroyBullet))

(event Custom|Set%20New%20Flipbook
  (params (NewFlipbook :type Paper%20Flipbook%20Object%20Reference) (InColor :type Color%20Structure))
  (bind _flipbookcomponent (Variables|Default|GetFlipbookComponent))
  (Sprite|SetFlipbook _flipbookcomponent NewFlipbook)
  (Sprite|SetSpriteColor _flipbookcomponent (Math|Conversions|ToLinearColor(Color) InColor)))

(event Custom|DestroyBullet
  (Class|BPIGMProjectile|ProjectileDied(Message) (Game|GetGameMode) self))

(event EventBeginPlay
  (bind _movement (Variables|Default|GetMovement))
  (Class|TimelineComponent|SetVectorCurve _movement (Variables|Stats|GetTrajectory) "MovementCurve")
  (Components|Timeline|SetPlayRate _movement (/ 1.0 (Variables|Stats|GetLifespan)))
  (CallFunction|SetNewSprite (Variables|Appearence|GetSprite) (Variables|Appearence|GetColor))
  (Variables|Stats|SetSpeed (* (Variables|Stats|GetSpeed) (CallFunction|ScaleAverage))))

(fn ConstructionScript
  (bind _color (Variables|Appearence|GetColor))
  (CallFunction|SetNewSprite (Variables|Appearence|GetSprite) _color)
  (CallFunction|SetNewFlipbook (Variables|Appearence|GetFlipbook) _color))

(fn CalculateLocation
  (params (Vector%20Track :type Vector))
  (bind _lifespan (Variables|Stats|GetLifespan))
  (bind _speed (Variables|Stats|GetSpeed))
  (bind _returnvalue (* _lifespan _speed Vector%20Track))
  (bind (_x _y _z) (Math|Vector|BreakVector _returnvalue))
  (return (+ (Variables|PostSpawn|GetInitPos) (Math|Vector|RotateVectorAroundAxis (+ (Math|Vector|RotateVector (Math|Vector|MakeVector _x 0.0 0.0) (Math|Rotator|MakeRotator 0.0 0.0 (.yaw (Transformation|GetActorRotation)))) (* (Transformation|GetActorUpVector) _y 0.5)) _z "0, 0,1.000000"))))

(fn ScaleAverage
  (bind _root (Variables|Default|GetRoot))
  (bind _returnvalue (Transformation|GetWorldScale _root))
  (bind (_x _y) (Math|Vector|BreakVector _returnvalue))
  (return (/ (+ _x _y) 2.0)))

(fn SetVariables
  (params (Params :type Struct%20Projectile%20Structure))
  (bind (_name _sprite _color _trajectory _speed _lifespan _damagedata _collisionprofile _destroyonimpact _scale) (Utilities|Struct|BreakStruct_Projectile Params))
  (bind _heroes_game_instance (CallFunction|GetHeroesGameInstance))
  (bind _movement (Variables|Default|GetMovement))
  (bind (_damagevaluesperdifficulty _damagetype) (Utilities|Struct|BreakS_DamageData _damagedata))
  (bind _currentdifficulty (Variables|/Game/Dev/Gibran/Core/HeroesGameInstance.HeroesGameInstance_C|GetCurrentDifficulty _heroes_game_instance))
  (bind _value (Utilities|Map|Find _damagevaluesperdifficulty _currentdifficulty))
  (bind (_basemindamage _basemaxdamage _knockbackstrength) (Utilities|Struct|BreakS_DamageDataValues _value))
  (Variables|Appearence|SetName _name)
  (CallFunction|SetNewSprite _sprite _color)
  (Class|TimelineComponent|SetVectorCurve _movement _trajectory "MovementCurve")
  (Components|Timeline|SetPlayRate _movement (/ 1.0 _lifespan))
  (Variables|Stats|SetSpeed _speed)
  (Variables|Stats|SetMinDamage _basemindamage)
  (Variables|Stats|SetMaxDamage _basemaxdamage)
  (Variables|Stats|SetKnockback%20Strength _knockbackstrength)
  (Variables|Stats|SetDamageType _damagetype)
  (Collision|SetCollisionProfileName (Variables|Default|GetCapsule) _collisionprofile true :!class /Script/Engine.PrimitiveComponent)
  (Variables|Default|SetDestroyOnImpact _destroyonimpact)
  (Transformation|SetActorScale3D (+ _scale "1.000000,1.000000,1.000000")))