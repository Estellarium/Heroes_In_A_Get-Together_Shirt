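; BP_DestructibleBase is a destructible sprite actor with durability that drops when it takes damage.
; Non-lethal hits flash the sprite and play a timeline whose FlipFlop jitters it back and forth, ignoring further damage until finished.
; At zero durability it spawns a double-scale BP_SpriteVFX playing the destruction flipbook, then destroys itself.
; Tick prints current durability as debug text.
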(event Custom|Destroy
  (bind _returnvalue (Game|SpawnActorfromClass "/Game/Dev/Gibran/Core/Blueprints/BP_SpriteVFX.BP_SpriteVFX_C" (Math|Transform|MakeTransform (Transformation|GetActorLocation) "0, 0, 0" (* (Transformation|GetActorScale3D) 2.0)) "AlwaysSpawn" 0 0))
  (Default|TriggerEffect(Flipbook) _returnvalue (Variables|Default|GetDestructionFlipbook) 1.0 false)
  (Actor|DestroyActor))

(event EventTakeDamage
  (params (DamageCauser :type Actor%20Object%20Reference) (DamageInstigator :type Actor%20Object%20Reference) (BaseDamage :type Float%20%28double-precision%29) (KnockbackStrength :type Float%20%28double-precision%29) (DamageType :type E_DamageType%20Enum :default "NewEnumerator11") (Direction :type Vector :default "0, 0, 0"))
  (bind _papersprite (Variables|Default|GetPaperSprite))
  (if (not (Variables|Default|GetIsTakingDamage))
    (bind _output_get (Variables|Default|SetCurrentDurability (Math|Float|Clamp(Float) (- (Variables|Default|GetCurrentDurability) BaseDamage) 0.0 (Variables|Default|GetMaxDurability))))
    (Variables|Default|SetIsTakingDamage true)
    (if (<= _output_get 0.0)
      (CallFunction|Destroy)
      (else
        (Utilities|SpriteColorFlash (Variables|Default|GetPaperSprite) "(R=1.000000,G=0.391402,B=0.000000,A=1.000000)" 0.2
          (:__
            (Timeline|DamageTimeline PlayFromStart
              (:Update
                (Utilities|FlowControl|FlipFlop
                  (:A
                    (Transformation|AddRelativeLocation _papersprite "1.000000,1.000000, 0" false false))
                  (:B
                    (Transformation|AddRelativeLocation _papersprite "-1.000000,-1.000000, 0" false false))))
              (:Finished
                (Variables|Default|SetIsTakingDamage false)))))))))

(event EventBeginPlay
  (Variables|Default|SetCurrentDurability (Variables|Default|GetMaxDurability)))

(event EventTick
  (params (DeltaSeconds :type Float%20%28single-precision%29))
  (Development|PrintText (Utilities|Text|FormatText "Detsructible durability: {dur}" (Variables|Default|GetCurrentDurability)) true true "(R=1.000000,G=0.645574,B=0.000000,A=1.000000)" 5.0 "Destructible"))

(fn ConstructionScript)