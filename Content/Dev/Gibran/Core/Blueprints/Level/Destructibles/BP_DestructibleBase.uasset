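; BP_DestructibleBase is a base destructible obstacle with durability, drawn with a Paper2D sprite and tilemap.
; TakeDamage can restrict durability loss to BP_HeroMelee ("Ethan"), optionally only through melee attacks flagged to destroy obstacles.
; Rejected and non-lethal hits flash orange, play a sound and shake via a timeline, whose end clears the damage lock set by valid hits.
; At zero durability it spawns BP_SpriteVFX with DestructionFX and destroys itself.
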(event Custom|Destroy
  (bind _returnvalue (Game|SpawnActorfromClass "/Game/Dev/Gibran/Core/Blueprints/BP_SpriteVFX.BP_SpriteVFX_C" (Math|Transform|MakeTransform (Transformation|GetActorLocation) "0, 0, 0" (Transformation|GetActorScale3D)) "AlwaysSpawn" 0 0))
  (Default|TriggerEffect(Struct) _returnvalue (Variables|Default|GetDestructionFX))
  (Actor|DestroyActor))

(event EventTakeDamage
  (params (DamageCauser :type Actor%20Object%20Reference) (DamageInstigator :type Actor%20Object%20Reference) (Damage :type Float%20%28double-precision%29) (KnockbackStrength :type Float%20%28double-precision%29) (DamageType :type E_DamageType%20Enum :default "NewEnumerator11") (Direction :type Vector :default "0, 0, 0"))
  (bind _papersprite (Variables|Default|GetPaperSprite))
  (bind _papertilemap (Variables|Default|GetPaperTileMap))
  (if (not (Variables|Default|GetIsTakingDamage))
    (if (Variables|Default|GetRequiresEthan)
      (if (== (Utilities|GetClass DamageInstigator) "/Game/Dev/Gibran/Core/Blueprints/Heroes/BP_HeroMelee.BP_HeroMelee_C")
        (if (Variables|Default|GetRequiresDestructionAttack)
          (bind _asbp_melee_attack (Utilities|Casting|CastToBP_MeleeAttack DamageCauser)
            (:then
              (if (Variables|/Game/Dev/Gibran/Core/Blueprints/BP_MeleeAttack.BP_MeleeAttack_C|GetDestroysObstacles _asbp_melee_attack)
                (bind _output_get (Variables|Default|SetCurrentDurability (Math|Float|Clamp(Float) (- (Variables|Default|GetCurrentDurability) Damage) 0.0 (Variables|Default|GetMaxDurability)) :!label _label))
                (Variables|Default|SetIsTakingDamage true)
                (if (<= _output_get 0.0)
                  (CallFunction|Destroy)
                  (else
                    (Utilities|SpriteColorFlash (Variables|Default|GetPaperSprite) "(R=1.000000,G=0.392157,B=0.000000,A=1.000000)" 0.2 "(R=1.000000,G=1.000000,B=1.000000,A=1.000000)" :!label _label_2
                      (:__
                        (Utilities|TilemapColorFlash (Variables|Default|GetPaperTileMap) "(R=1.000000,G=0.392157,B=0.000000,A=1.000000)" 0.2
                          (:_
                            (Audio|PlaySoundatLocation (Variables|Default|GetDamageSound) (Transformation|GetActorLocation) "0, 0, 0" 1.0 1.0 0.0 0 0 0 0)
                            (Timeline|DamageTimeline PlayFromStart
                              (:Update
                                (Utilities|FlowControl|FlipFlop
                                  (:A
                                    (Transformation|AddRelativeLocation _papersprite "1.000000,1.000000, 0" false false)
                                    (Transformation|AddRelativeLocation _papertilemap "1.000000,1.000000, 0" false false))
                                  (:B
                                    (Transformation|AddRelativeLocation _papersprite "-1.000000,-1.000000, 0" false false)
                                    (Transformation|AddRelativeLocation _papertilemap "-1.000000,-1.000000, 0" false false))))
                              (:Finished
                                (Variables|Default|SetIsTakingDamage false)))))))))
                (else
                  (goto _label_2))))
            (:CastFailed
              (goto _label_2)))
          (else
            (goto _label)))
        (else
          (goto _label_2)))
      (else
        (goto _label)))))

(event EventBeginPlay
  (Variables|Default|SetCurrentDurability (Variables|Default|GetMaxDurability)))

(event EventTick
  (params (DeltaSeconds :type Float%20%28single-precision%29)))

(fn ConstructionScript)