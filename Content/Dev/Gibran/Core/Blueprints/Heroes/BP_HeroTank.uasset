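; Tank hero Blueprint that blocks enemy projectile and melee attacks with a base shield and an enhanced shield.
; Starting enhancement shows the enhanced shield, enables its collision profile and sets the meter icon; ending it hides and disables that shield.
; Each shield's overlap handler records the blocked attacker, flashes its sprite and plays a metal sound, clearing the record otherwise.
; Tick alternately nudges the base shield collision back and forth slightly.
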(event OnComponentBeginOverlap(BaseShieldCollision)
  (params (OverlappedComponent :type Primitive%20Component%20Object%20Reference) (OtherActor :type Actor%20Object%20Reference) (OtherComp :type Primitive%20Component%20Object%20Reference) (OtherBodyIndex :type Integer) (bFromSweep :type Boolean) (SweepResult :type Hit%20Result%20Structure%20%28by%20ref%29))
  (bind _returnvalue (Collision|GetCollisionProfileName OtherComp))
  (Development|PrintText (Utilities|Text|FormatText "Shield hit object of type {ot}" _returnvalue) (CallFunction|ReadDebugTag "Damage") true "(R=1.000000,G=0.277917,B=0.000000,A=1.000000)" 2.0 "ShieldHit")
  (switch name _returnvalue
    (:Default
      (Variables|Default|SetBlockedAttack 0 :!label _label))
    (:EnemyProjectile
      (Utilities|SpriteColorFlash (Variables|Default|GetBaseShieldSprite) "(R=0.196010,G=1.000000,B=0.000000,A=1.000000)" 0.2 "(R=1.000000,G=0.160000,B=0.000000,A=1.000000)" :!label _label_2
        (:__
          (Variables|Default|SetBlockedAttack OtherActor)
          (Audio|PlaySoundatLocation "/Game/Dev/Gibran/TestAssets/Sounds/Combat/metal_hit_floor_medium_1_Cue.metal_hit_floor_medium_1_Cue" (Transformation|GetActorLocation) "0, 0, 0" 1.0 1.0 0.0 0 0 0 0))))
    (:EnemyMelee
      (goto _label_2))
    (:Enemy
      (goto _label))))

(event OnComponentBeginOverlap(EnhShieldCollision)
  (params (OverlappedComponent :type Primitive%20Component%20Object%20Reference) (OtherActor :type Actor%20Object%20Reference) (OtherComp :type Primitive%20Component%20Object%20Reference) (OtherBodyIndex :type Integer) (bFromSweep :type Boolean) (SweepResult :type Hit%20Result%20Structure%20%28by%20ref%29))
  (bind _returnvalue (Collision|GetCollisionProfileName OtherComp))
  (Development|PrintText (Utilities|Text|FormatText "Shield hit object of type {ot}" _returnvalue) (CallFunction|ReadDebugTag "Damage") true "(R=1.000000,G=0.277917,B=0.000000,A=1.000000)" 2.0 "ShieldHit")
  (switch name _returnvalue
    (:Default
      (Variables|Default|SetBlockedAttack 0 :!label _label))
    (:EnemyProjectile
      (Utilities|SpriteColorFlash (Variables|Default|GetEnhShieldSprite) "(R=0.196010,G=1.000000,B=0.000000,A=1.000000)" 0.2 "(R=1.000000,G=0.160000,B=0.000000,A=1.000000)" :!label _label_2
        (:__
          (Variables|Default|SetBlockedAttack OtherActor)
          (Audio|PlaySoundatLocation "/Game/Dev/Gibran/TestAssets/Sounds/Combat/metal_hit_floor_medium_1_Cue.metal_hit_floor_medium_1_Cue" (Transformation|GetActorLocation) "0, 0, 0" 1.0 1.0 0.0 0 0 0 0))))
    (:EnemyMelee
      (goto _label_2))
    (:Enemy
      (goto _label))))

(event EventBeginPlay
  (|CallParentFunction)
  (Variables|Default|SetShieldMeshRef (Variables|Default|GetBaseShieldCollision)))

(event Collision|EventActorBeginOverlap
  (params (OtherActor :type Actor%20Object%20Reference)))

(event EventTick
  (params (DeltaSeconds :type Float%20%28single-precision%29))
  (bind _baseshieldcollision (Variables|Default|GetBaseShieldCollision))
  (|CallParentFunction DeltaSeconds)
  (Utilities|FlowControl|FlipFlop
    (:A
      (Transformation|AddRelativeLocation _baseshieldcollision "0.100000, 0, 0" false false))
    (:B
      (Transformation|AddRelativeLocation _baseshieldcollision "-0.100000, 0, 0" false false))))

(event EventAction1)

(event EventStartEnhancement
  (CallFunction|ToggleEnhancedShield true)
  (Class|Image|SetBrushResourceObject (Variables|/Game/Dev/Gibran/Core/UI/HUD/WBP_EnhancementMeter.WBP_EnhancementMeter_C|GetEnhacementIcon (Variables|Default|GetEnhancementMeterRef)) "/Game/Dev/Gibran/TestAssets/Sprites/UI/Icons/Icon_Shield1.Icon_Shield1"))

(event EventEndEnhancement
  (CallFunction|ToggleEnhancedShield false))

(fn ConstructionScript
  (|CallParentFunction))

(fn ToggleEnhancedShield
  (params (Activate :type Boolean))
  (bind _enhshieldcollision (Variables|Default|GetEnhShieldCollision))
  (Rendering|SetVisibility (Variables|Default|GetEnhShieldSprite) Activate false)
  (if Activate
    (Collision|SetCollisionProfileName _enhshieldcollision "HeroShield" true :!class /Script/Engine.PrimitiveComponent)
    (else
      (Collision|SetCollisionProfileName _enhshieldcollision "NoCollision" true :!class /Script/Engine.PrimitiveComponent))))