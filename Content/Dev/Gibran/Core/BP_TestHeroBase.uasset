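; BP_TestHeroBase is a test base hero with a 2D flipbook sprite, a number label and an icon, all set on BeginPlay.
; Events switch between idle and run flipbooks, flip the sprite by X scale, and flash it on damage.
; InitShooting starts a looping timer that fires the shooting component at BulletsPerSecond.
; Tick locks the sprite's world rotation; logic driving animation from parent actor velocity is disconnected.
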(event Custom|SpriteRun
  (Sprite|SetFlipbook (Variables|Default|GetFlipbook) (Variables|Default|GetRunFlipbook)))

(event Custom|SpriteStop
  (Sprite|SetFlipbook (Variables|Default|GetFlipbook) (Variables|Default|GetIdleFlipbook)))

(event Custom|SpriteFlip
  (params (Scale :type Float%20%28double-precision%29))
  (Transformation|SetRelativeScale3D (Variables|Default|GetFlipbook) (Math|Vector|MakeVector Scale 2.655821 2.655821)))

(event Custom|Init%20Shooting
  (Utilities|Time|SetTimerbyEvent (delegate Custom|Shoot) (/ 1.0 (Variables|Default|GetBulletsPerSecond)) true))

(event Custom|Shoot
  (Default|ShootOnceProjectileClass (Variables|Default|GetBP_Shooting_Component)))

(event EventBeginPlay
  (Rendering|Components|TextRender|SetText (Variables|Default|GetNumberText) (Utilities|Text|ToText(Integer) (Variables|Default|GetNumber)))
  (Rendering|Components|Sprite|SetSprite (Variables|Default|GetIcon) (Variables|Default|GetIconTxt))
  (Sprite|SetFlipbook (Variables|Default|GetFlipbook) (Variables|Default|GetIdleFlipbook)))

(event EventTick
  (params (DeltaSeconds :type Float%20%28single-precision%29))
  (Transformation|SetWorldRotation (Variables|Default|GetFlipbook) "0.000000,0.000000,-90.000000" false false))

(event EventTakeDamage
  (params (DamageCauser :type Actor%20Object%20Reference) (DamageInstigator :type Actor%20Object%20Reference) (BaseDamage :type Float%20%28double-precision%29) (KnockbackStrength :type Float%20%28double-precision%29) (DamageType :type E_DamageType%20Enum :default "NewEnumerator0"))
  (Utilities|FlipbookDamageFlash (Variables|Default|GetFlipbook) 0.2))

(fn ConstructionScript)