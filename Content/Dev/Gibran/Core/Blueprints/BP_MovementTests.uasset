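; Debug test actor that visualizes random point sampling between two radii, apparently for movement target selection.
; Tick draws inner and outer radius circles around the actor.
; BeginPlay plots 1000 temporary debug points from RandomPointInSliceBetweenCirclesSimple, using a start offset along world X and the actor as target, to show the slice distribution.
; Disconnected calls to the complex slice, full-circle and between-circles variants remain as unused alternatives.
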(event EventBeginPlay
  (bind _returnvalue (Transformation|GetActorLocation))
  (bind (_x _y _z) (Math|Vector|BreakVector _returnvalue))
  (for _index (range 0 999)
    (Rendering|Debug|DrawDebugPoint (CallFunction|RandomPointinSliceBetweenCircles(Simple) (Math|Vector|MakeVector (+ _x 4e+02) _y _z) _returnvalue (Variables|Default|GetInnerRadius) (Variables|Default|GetOuterRadius) 3e+01) 5.0 "(R=1.000000,G=0.704562,B=0.000000,A=1.000000)" 3e+01)))

(event EventTick
  (params (DeltaSeconds :type Float%20%28single-precision%29))
  (bind _returnvalue (Transformation|GetActorLocation))
  (Rendering|Debug|DrawDebugCircle _returnvalue (Variables|Default|GetInnerRadius) 48 "(R=0.000000,G=1.000000,B=0.004274,A=1.000000)" 0.0 3.0 "0.000000,1.000000,0.000000" "1.000000,0.000000,0.000000")
  (Rendering|Debug|DrawDebugCircle _returnvalue (Variables|Default|GetOuterRadius) 48 "(R=0.000000,G=0.195574,B=1.000000,A=1.000000)" 0.0 3.0 "0.000000,1.000000,0.000000" "1.000000,0.000000,0.000000"))

(fn ConstructionScript)