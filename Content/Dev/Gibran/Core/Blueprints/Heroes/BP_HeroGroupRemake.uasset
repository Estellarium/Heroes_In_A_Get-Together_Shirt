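; Player pawn that moves and steers a party of four heroes (range, melee, tank, healer/unlocker) as one group, using child actors and floating movement.
; Four action inputs each drive one hero, with a retriggerable delay separating tap and hold abilities, gated by cooldown and fainting.
; Enemy projectile or melee damage is forwarded to every hero.
; Summed health feeds the HUD and triggers game over at zero; Tick adds debug readouts and jiggles the collision box.
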(event OnComponentBeginOverlap(BoxCollision)
  (params (OverlappedComponent :type Primitive%20Component%20Object%20Reference) (OtherActor :type Actor%20Object%20Reference) (OtherComp :type Primitive%20Component%20Object%20Reference) (OtherBodyIndex :type Integer) (bFromSweep :type Boolean) (SweepResult :type Hit%20Result%20Structure%20%28by%20ref%29))
  (Utilities|IsValid OtherComp))

(event Custom|Die
  (bind _outactors (Actor|GetAllActorsOfClass "/Script/Engine.AmbientSound"))
  (for _array_element _outactors
    (Audio|Components|Audio|AdjustVolume (Variables|/Script/Engine.AmbientSound|GetAudioComponent _array_element) 1.0 0.0 "Linear" :!class /Script/Engine.AudioComponent))
  (Input|DisableInput (Game|GetPlayerController 0))
  (Widget|RemovefromParent (Variables|Default|GetHudRef))
  (Utilities|FlowControl|Delay 0.5)
  (Game|SetGamePaused true)
  (bind _returnvalue (UserInterface|CreateWidget "/Game/Dev/Gibran/Core/UI/WBP_GameOverScreen.WBP_GameOverScreen_C"))
  (UserInterface|Viewport|AddtoViewport _returnvalue 0))

(event EventBeginPlay
  (bind _self self)
  (Utilities|FlowControl|Sequence
    (:then_0
      (Components|Movement|SetUpdatedComponent (Variables|Default|GetFloatingPawnMovement) (Variables|Default|GetBoxCollision)))
    (:then_1
      (bind _asbp_hero_range (Utilities|Casting|CastToBP_HeroRange (Variables|/Script/Engine.ChildActorComponent|GetChildActor (Variables|Default|GetcHeroHan))))
      (bind _output_get (Variables|Default|SetHeroHanRef _asbp_hero_range))
      (Variables|/Game/Dev/Gibran/Core/Blueprints/Heroes/BP_HeroBase.BP_HeroBase_C|SetHeroGroupRef _output_get _self)
      (bind _asbp_hero_melee (Utilities|Casting|CastToBP_HeroMelee (Variables|/Script/Engine.ChildActorComponent|GetChildActor (Variables|Default|GetcHeroEth))))
      (bind _output_get_2 (Variables|Default|SetHeroEthRef _asbp_hero_melee))
      (Variables|/Game/Dev/Gibran/Core/Blueprints/Heroes/BP_HeroBase.BP_HeroBase_C|SetHeroGroupRef _output_get_2 _self)
      (bind _asbp_hero_tank (Utilities|Casting|CastToBP_HeroTank (Variables|/Script/Engine.ChildActorComponent|GetChildActor (Variables|Default|GetcHeroShu))))
      (bind _output_get_3 (Variables|Default|SetHeroShuRef _asbp_hero_tank))
      (Variables|/Game/Dev/Gibran/Core/Blueprints/Heroes/BP_HeroBase.BP_HeroBase_C|SetHeroGroupRef _output_get_3 _self)
      (bind _asbp_hero_heal_unlocker (Utilities|Casting|CastToBP_HeroHealUnlocker (Variables|/Script/Engine.ChildActorComponent|GetChildActor (Variables|Default|GetcHeroBen))))
      (bind _output_get_4 (Variables|Default|SetHeroBenRef _asbp_hero_heal_unlocker))
      (Variables|/Game/Dev/Gibran/Core/Blueprints/Heroes/BP_HeroBase.BP_HeroBase_C|SetHeroGroupRef _output_get_4 _self))
    (:then_2
      (Utilities|FlowControl|Delay 5.0)
      (bind _returnvalue (UserInterface|CreateWidget "/Game/Dev/Gibran/Core/UI/WBP_HeroBarsHud.WBP_HeroBarsHud_C"))
      (UserInterface|Viewport|AddtoViewport _returnvalue 0)
      (Variables|Default|SetHudRef _returnvalue)
      (CallFunction|UpdateTotalHealth))))

(event EventTakeDamage
  (params (DamageCauser :type Actor%20Object%20Reference) (DamageInstigator :type Actor%20Object%20Reference) (BaseDamage :type Float%20%28double-precision%29) (KnockbackStrength :type Float%20%28double-precision%29) (DamageType :type E_DamageType%20Enum :default "NewEnumerator11") (Direction :type Vector :default "0, 0, 0"))
  (bind _asbp_projectile (Utilities|Casting|CastToBP_Projectile DamageCauser))
  (switch name (Collision|GetCollisionProfileName (Variables|/Game/Bin/Blueprints/Object/Projectiles/BP_Projectile.BP_Projectile_C|GetCapsule _asbp_projectile))
    (:EnemyProjectile
      _)
    (:EnemyMelee
      _))
  (Class|BPIDamageableActor|TakeDamage(Message) (Variables|Default|GetHeroHanRef) 0 0 BaseDamage 0.0 DamageType "0, 0, 0")
  (Class|BPIDamageableActor|TakeDamage(Message) (Variables|Default|GetHeroEthRef) 0 0 BaseDamage 0.0 DamageType "0, 0, 0")
  (Class|BPIDamageableActor|TakeDamage(Message) (Variables|Default|GetHeroShuRef) 0 0 BaseDamage 0.0 DamageType "0, 0, 0")
  (Class|BPIDamageableActor|TakeDamage(Message) (Variables|Default|GetHeroBenRef) 0 0 BaseDamage 0.0 DamageType "0, 0, 0"))

(event EventTick
  (params (DeltaSeconds :type Float%20%28single-precision%29))
  (bind _boxcollision (Variables|Default|GetBoxCollision))
  (Utilities|FlowControl|Sequence
    (:then_0
      (bind _returnvalue (Class|Pawn|ConsumeMovementInputVector))
      (Class|PawnMovementComponent|AddInputVector (Variables|Default|GetFloatingPawnMovement) _returnvalue false)
      (Utilities|IsDebugModeOn?
        (:Debug%20Mode%20On
          (|DistanceDebugging))))
    (:then_1
      (Development|PrintText (Utilities|Text|FormatText "Ethan: {eh} 
Hanna: {hh} 
Shura: {sh} 
Benjamin: {bh} 
Total: {th}" (Variables|/Game/Dev/Gibran/Core/Blueprints/Heroes/BP_HeroBase.BP_HeroBase_C|GetHealth (Variables|Default|GetHeroEthRef)) (Variables|/Game/Dev/Gibran/Core/Blueprints/Heroes/BP_HeroBase.BP_HeroBase_C|GetHealth (Variables|Default|GetHeroHanRef)) (Variables|/Game/Dev/Gibran/Core/Blueprints/Heroes/BP_HeroBase.BP_HeroBase_C|GetHealth (Variables|Default|GetHeroShuRef)) (Variables|/Game/Dev/Gibran/Core/Blueprints/Heroes/BP_HeroBase.BP_HeroBase_C|GetHealth (Variables|Default|GetHeroBenRef)) (Variables|Default|GetTotalHealth)) true false "(R=0.000000,G=1.000000,B=0.126143,A=1.000000)" 0.0 "GroupHealth"))
    (:then_2
      (Utilities|FlowControl|FlipFlop
        (:A
          (Transformation|AddRelativeLocation _boxcollision "0.100000, 0, 0" false false))
        (:B
          (Transformation|AddRelativeLocation _boxcollision "-0.100000, 0, 0" false false))))))

(event Input|ActionEvents|InputActionAction1
  (params (Key :type Key%20Structure :default "None"))
  (bind _herobenref (Variables|Default|GetHeroBenRef))
  (bind _fainted (Variables|/Game/Dev/Gibran/Core/Blueprints/Heroes/BP_HeroBase.BP_HeroBase_C|GetFainted _herobenref))
  (:Pressed
    (Variables|Default|SetHero1AbilityHolded false)
    (Utilities|FlowControl|RetriggerableDelay (Variables|Default|GetAbilityHoldingThreshold))
    (Variables|Default|SetHero1AbilityHolded true))
  (:Released
    (if (Variables|Default|GetHero1AbilityHolded)
      (if (Math|Boolean|NORBoolean (Variables|/Game/Dev/Gibran/Core/Blueprints/Heroes/BP_HeroBase.BP_HeroBase_C|GetInAbility2Cooldown _herobenref) _fainted)
        (Default|Action2 _herobenref))
      (elif (Math|Boolean|NORBoolean (Variables|/Game/Dev/Gibran/Core/Blueprints/Heroes/BP_HeroBase.BP_HeroBase_C|GetInAbility1Cooldown _herobenref) _fainted)
        (Default|Action1 _herobenref)))))

(event Input|ActionEvents|InputActionAction2
  (params (Key :type Key%20Structure :default "None"))
  (bind _heroethref (Variables|Default|GetHeroEthRef))
  (bind _fainted (Variables|/Game/Dev/Gibran/Core/Blueprints/Heroes/BP_HeroBase.BP_HeroBase_C|GetFainted _heroethref))
  (:Pressed
    (Variables|Default|SetHero2AbilityHolded false)
    (Utilities|FlowControl|RetriggerableDelay (Variables|Default|GetAbilityHoldingThreshold))
    (Variables|Default|SetHero2AbilityHolded true))
  (:Released
    (if (Variables|Default|GetHero2AbilityHolded)
      (if (Math|Boolean|NORBoolean (Variables|/Game/Dev/Gibran/Core/Blueprints/Heroes/BP_HeroBase.BP_HeroBase_C|GetInAbility2Cooldown _heroethref) _fainted)
        (Default|Action2 _heroethref))
      (elif (Math|Boolean|NORBoolean (Variables|/Game/Dev/Gibran/Core/Blueprints/Heroes/BP_HeroBase.BP_HeroBase_C|GetInAbility1Cooldown _heroethref) _fainted)
        (Default|Action1 _heroethref)))))

(event Input|ActionEvents|InputActionAction3
  (params (Key :type Key%20Structure :default "None"))
  (bind _heroshuref (Variables|Default|GetHeroShuRef))
  (bind _fainted (Variables|/Game/Dev/Gibran/Core/Blueprints/Heroes/BP_HeroBase.BP_HeroBase_C|GetFainted _heroshuref))
  (:Pressed
    (Variables|Default|SetHero3AbilityHolded false)
    (Utilities|FlowControl|RetriggerableDelay (Variables|Default|GetAbilityHoldingThreshold))
    (Variables|Default|SetHero3AbilityHolded true))
  (:Released
    (if (Variables|Default|GetHero3AbilityHolded)
      (if (Math|Boolean|NORBoolean (Variables|/Game/Dev/Gibran/Core/Blueprints/Heroes/BP_HeroBase.BP_HeroBase_C|GetInAbility2Cooldown _heroshuref) _fainted)
        (Default|Action2 _heroshuref))
      (elif (Math|Boolean|NORBoolean (Variables|/Game/Dev/Gibran/Core/Blueprints/Heroes/BP_HeroBase.BP_HeroBase_C|GetInAbility1Cooldown _heroshuref) _fainted)
        (Default|Action1 _heroshuref)))))

(event Input|ActionEvents|InputActionAction4
  (params (Key :type Key%20Structure :default "None"))
  (bind _herohanref (Variables|Default|GetHeroHanRef))
  (bind _fainted (Variables|/Game/Dev/Gibran/Core/Blueprints/Heroes/BP_HeroBase.BP_HeroBase_C|GetFainted _herohanref))
  (:Pressed
    (Variables|Default|SetHero4AbilityHolded false)
    (Utilities|FlowControl|RetriggerableDelay (Variables|Default|GetAbilityHoldingThreshold))
    (Variables|Default|SetHero4AbilityHolded true))
  (:Released
    (if (Variables|Default|GetHero4AbilityHolded)
      (if (Math|Boolean|NORBoolean (Variables|/Game/Dev/Gibran/Core/Blueprints/Heroes/BP_HeroBase.BP_HeroBase_C|GetInAbility2Cooldown _herohanref) _fainted)
        (Default|Action2 _herohanref))
      (elif (Math|Boolean|NORBoolean (Variables|/Game/Dev/Gibran/Core/Blueprints/Heroes/BP_HeroBase.BP_HeroBase_C|GetInAbility1Cooldown _herohanref) _fainted)
        (Default|Action1 _herohanref)))))

(event Input|AxisEvents|InputAxisMoveUp/Down
  (params (AxisValue :type Float%20%28single-precision%29))
  (Pawn|Input|AddMovementInput (Math|Vector|GetForwardVector (Variables|Default|GetDirectionArrow)) AxisValue false))

(event Input|AxisEvents|InputAxisMoveLeft/Right
  (params (AxisValue :type Float%20%28single-precision%29))
  (Pawn|Input|AddControllerYawInput (* AxisValue (Variables|Default|GetMaxRotationRate))))

(event Input|KeyboardEvents|Tab
  (params (Key :type Key%20Structure :default "None"))
  (:Released
    (Default|ToggleDebugMode (CallFunction|GetHeroesGameMode))))

(event Input|KeyboardEvents|LeftCtrl
  (params (Key :type Key%20Structure :default "None"))
  (:Released
    (bind _returnvalue (UserInterface|CreateWidget "/Game/Dev/Gibran/Core/UI/WBP_LanguageTest.WBP_LanguageTest_C"))
    (UserInterface|Viewport|AddtoViewport _returnvalue 0)))

(fn ConstructionScript)

(fn UpdateTotalHealth
  (bind _hudref (Variables|Default|GetHudRef))
  (bind _output_get (Variables|Default|SetTotalHealth (Math|Float|Clamp(Float) (+ (Variables|/Game/Dev/Gibran/Core/Blueprints/Heroes/BP_HeroBase.BP_HeroBase_C|GetHealth (Variables|Default|GetHeroHanRef)) (Variables|/Game/Dev/Gibran/Core/Blueprints/Heroes/BP_HeroBase.BP_HeroBase_C|GetHealth (Variables|Default|GetHeroEthRef)) (Variables|/Game/Dev/Gibran/Core/Blueprints/Heroes/BP_HeroBase.BP_HeroBase_C|GetHealth (Variables|Default|GetHeroShuRef)) (Variables|/Game/Dev/Gibran/Core/Blueprints/Heroes/BP_HeroBase.BP_HeroBase_C|GetHealth (Variables|Default|GetHeroBenRef))) 0.0 8e+02)))
  (Utilities|IsValid _hudref
    (:Is%20Valid
      (Default|SetHealthBars _hudref))
    (:Is%20Not%20Valid
      _))
  (if (<= _output_get 0.0)
    (CallFunction|Die)))

(fn SetMovementSpeeds)