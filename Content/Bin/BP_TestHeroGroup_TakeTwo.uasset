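; Test hero-group character that drives four heroes as one formation, with Hero2 and Hero4 set up for shooting on BeginPlay.
; A movement mode selects Twinstick, where move axes translate and analog axes rotate CenterRoot at a constant rate, or Tank, where both feed shared movement-plus-yaw logic.
; Tick stretches two spline meshes between opposite heroes.
; Several action inputs are overridden to do nothing, and construction derives rate multipliers and center distance.
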(event EventBeginPlay
  (|CallParentFunction)
  (Default|InitShooting (Variables|Default|GetHero2))
  (Variables|Default|SetAllHeroes (Utilities|Array|MakeArray (Variables|Default|GetHero1) (Variables|Default|GetHero2) (Variables|Default|GetHero3) (Variables|Default|GetHero4)))
  (Variables|Default|SetAllHeroesAsComponents (Utilities|Array|MakeArray (Variables|Default|GetcHero1) (Variables|Default|GetcHero2) (Variables|Default|GetcHero3) (Variables|Default|GetcHero4))))

(event EventTick
  (params (DeltaSeconds :type Float%20%28single-precision%29))
  (|CallParentFunction DeltaSeconds)
  (SplineMesh|SetStartandEnd (Variables|Default|GetSplineMesh) (Variables|/Script/Engine.SceneComponent|GetRelativeLocation (Variables|Default|GetcHero1)) "0, 0, 0" (Variables|/Script/Engine.SceneComponent|GetRelativeLocation (Variables|Default|GetcHero3)) "0, 0, 0" true :!class /Script/Engine.SplineMeshComponent)
  (SplineMesh|SetStartandEnd (Variables|Default|GetSplineMesh1) (Variables|/Script/Engine.SceneComponent|GetRelativeLocation (Variables|Default|GetcHero2)) "0, 0, 0" (Variables|/Script/Engine.SceneComponent|GetRelativeLocation (Variables|Default|GetcHero4)) "0, 0, 0" true :!class /Script/Engine.SplineMeshComponent))

(event Input|ActionEvents|InputActionaMoveLeft
  (params (Key :type Key%20Structure))
  ;[1 1 1] Overrides
  (:Pressed
    (if true :!label _label
      _))
  (:Released
    (goto _label)))

(event Input|ActionEvents|InputActionaMoveRight
  (params (Key :type Key%20Structure))
  ;[1 1 1] Overrides
  (:Pressed
    (if true :!label _label
      _))
  (:Released
    (goto _label)))

(event Input|ActionEvents|InputActionAction4
  (params (Key :type Key%20Structure))
  ;[1 1 1] Overrides
  (:Pressed
    (if true :!label _label
      _))
  (:Released
    (goto _label)))

(event Input|ActionEvents|InputActionAction2
  (params (Key :type Key%20Structure))
  ;[1 1 1] Overrides
  (:Pressed
    (if true :!label _label
      _))
  (:Released
    (goto _label)))

(event Input|AxisEvents|InputAxisMoveLeft/Right
  (params (AxisValue :type Float%20%28single-precision%29))
  (bind _returnvalue (Math|Float|Sign(Float) AxisValue))
  (switch Utilities|FlowControl|Switch|SwitchonMovemode (Variables|Default|GetMovementMode)
    (:NewEnumerator1
      (Pawn|Input|AddMovementInput (Math|Vector|Normalize (Math|Vector|MakeVector AxisValue (stale Input|AxisEvents|InputAxisMoveUp/Down AxisValue) 0.0)) 1.0 false))
    (:NewEnumerator2
      (Pawn|Input|AddMovementInput (+ (Math|Vector|Normalize (Math|Vector|MakeVector AxisValue (stale Input|AxisEvents|InputAxisMoveUp/Down AxisValue) 0.0)) (Math|Vector|Normalize (Math|Vector|MakeVector (stale Input|AxisEvents|InputAxisAnalogLeft/Right AxisValue) (stale Input|AxisEvents|InputAxisAnalogUp/Down AxisValue) 0.0))) (* (Math|Vector|VectorLength (+ (Math|Vector|Normalize (Math|Vector|MakeVector AxisValue (stale Input|AxisEvents|InputAxisMoveUp/Down AxisValue) 0.0)) (Math|Vector|Normalize (Math|Vector|MakeVector (stale Input|AxisEvents|InputAxisAnalogLeft/Right AxisValue) (stale Input|AxisEvents|InputAxisAnalogUp/Down AxisValue) 0.0)))) (Variables|Default|GetMovingRateMultiplier) 0.02) false)
      (Pawn|Input|AddControllerYawInput (* (/ (* (- (Math|Vector|DotProduct (Math|Vector|Normalize (Math|Vector|MakeVector AxisValue (stale Input|AxisEvents|InputAxisMoveUp/Down AxisValue) 0.0)) (Math|Vector|Normalize (Math|Vector|MakeVector (stale Input|AxisEvents|InputAxisAnalogLeft/Right AxisValue) (stale Input|AxisEvents|InputAxisAnalogUp/Down AxisValue) 0.0))) 1.0) (select (== (select (== (Math|Float|Sign(Float) (stale Input|AxisEvents|InputAxisMoveUp/Down AxisValue)) 0.0) (Math|Float|Sign(Float) (stale Input|AxisEvents|InputAxisAnalogUp/Down AxisValue)) (Math|Float|Sign(Float) (stale Input|AxisEvents|InputAxisMoveUp/Down AxisValue))) 0.0) (select (== _returnvalue 0.0) (Math|Float|Sign(Float) (stale Input|AxisEvents|InputAxisAnalogLeft/Right AxisValue)) _returnvalue) (select (== (Math|Float|Sign(Float) (stale Input|AxisEvents|InputAxisMoveUp/Down AxisValue)) 0.0) (Math|Float|Sign(Float) (stale Input|AxisEvents|InputAxisAnalogUp/Down AxisValue)) (Math|Float|Sign(Float) (stale Input|AxisEvents|InputAxisMoveUp/Down AxisValue))))) 8.0) (Variables|Default|GetTurningRateMultiplier))))))

(event Input|AxisEvents|InputAxisMoveUp/Down
  (params (AxisValue :type Float%20%28single-precision%29))
  (bind _returnvalue (Math|Float|Sign(Float) AxisValue))
  (switch Utilities|FlowControl|Switch|SwitchonMovemode (Variables|Default|GetMovementMode)
    (:NewEnumerator1
      (Pawn|Input|AddMovementInput (Math|Vector|Normalize (Math|Vector|MakeVector (stale Input|AxisEvents|InputAxisMoveLeft/Right AxisValue) AxisValue 0.0)) 1.0 false))
    (:NewEnumerator2
      (Pawn|Input|AddMovementInput (+ (Math|Vector|Normalize (Math|Vector|MakeVector (stale Input|AxisEvents|InputAxisMoveLeft/Right AxisValue) AxisValue 0.0)) (Math|Vector|Normalize (Math|Vector|MakeVector (stale Input|AxisEvents|InputAxisAnalogLeft/Right AxisValue) (stale Input|AxisEvents|InputAxisAnalogUp/Down AxisValue) 0.0))) (* (Math|Vector|VectorLength (+ (Math|Vector|Normalize (Math|Vector|MakeVector (stale Input|AxisEvents|InputAxisMoveLeft/Right AxisValue) AxisValue 0.0)) (Math|Vector|Normalize (Math|Vector|MakeVector (stale Input|AxisEvents|InputAxisAnalogLeft/Right AxisValue) (stale Input|AxisEvents|InputAxisAnalogUp/Down AxisValue) 0.0)))) (Variables|Default|GetMovingRateMultiplier) 0.02) false)
      (Pawn|Input|AddControllerYawInput (* (/ (* (- (Math|Vector|DotProduct (Math|Vector|Normalize (Math|Vector|MakeVector (stale Input|AxisEvents|InputAxisMoveLeft/Right AxisValue) AxisValue 0.0)) (Math|Vector|Normalize (Math|Vector|MakeVector (stale Input|AxisEvents|InputAxisAnalogLeft/Right AxisValue) (stale Input|AxisEvents|InputAxisAnalogUp/Down AxisValue) 0.0))) 1.0) (select (== (select (== _returnvalue 0.0) (Math|Float|Sign(Float) (stale Input|AxisEvents|InputAxisAnalogUp/Down AxisValue)) _returnvalue) 0.0) (select (== (Math|Float|Sign(Float) (stale Input|AxisEvents|InputAxisMoveLeft/Right AxisValue)) 0.0) (Math|Float|Sign(Float) (stale Input|AxisEvents|InputAxisAnalogLeft/Right AxisValue)) (Math|Float|Sign(Float) (stale Input|AxisEvents|InputAxisMoveLeft/Right AxisValue))) (select (== _returnvalue 0.0) (Math|Float|Sign(Float) (stale Input|AxisEvents|InputAxisAnalogUp/Down AxisValue)) _returnvalue))) 8.0) (Variables|Default|GetTurningRateMultiplier))))))

(event Input|AxisEvents|InputAxisAnalogUp/Down
  (params (AxisValue :type Float%20%28single-precision%29))
  (switch Utilities|FlowControl|Switch|SwitchonMovemode (Variables|Default|GetMovementMode)
    (:NewEnumerator1
      (if (> (Math|Vector|VectorLength (Math|Vector|Normalize (Math|Vector|MakeVector (stale Input|AxisEvents|InputAxisAnalogLeft/Right AxisValue) AxisValue 0.0))) 0.0)
        (bind _output_get (Variables|Default|SetDirection (Math|Vector|Normalize (Math|Vector|MakeVector (stale Input|AxisEvents|InputAxisAnalogLeft/Right AxisValue) AxisValue 0.0))))
        (Transformation|SetWorldRotation (Variables|Default|GetCenterRoot) (Class|KismetMathLibrary|RInterptoConstant (Transformation|GetWorldRotation (Variables|Default|GetCenterRoot)) (Math|Conversions|RotationFromXVector _output_get) (stale EventTick DeltaSeconds) (* (Variables|Default|GetTurningRateMultiplier) 1e+02)) false false)))
    (:NewEnumerator2
      (Pawn|Input|AddMovementInput (+ (Math|Vector|Normalize (Math|Vector|MakeVector (stale Input|AxisEvents|InputAxisMoveLeft/Right AxisValue) (stale Input|AxisEvents|InputAxisMoveUp/Down AxisValue) 0.0)) (Math|Vector|Normalize (Math|Vector|MakeVector (stale Input|AxisEvents|InputAxisAnalogLeft/Right AxisValue) AxisValue 0.0))) (* (Math|Vector|VectorLength (+ (Math|Vector|Normalize (Math|Vector|MakeVector (stale Input|AxisEvents|InputAxisMoveLeft/Right AxisValue) (stale Input|AxisEvents|InputAxisMoveUp/Down AxisValue) 0.0)) (Math|Vector|Normalize (Math|Vector|MakeVector (stale Input|AxisEvents|InputAxisAnalogLeft/Right AxisValue) AxisValue 0.0)))) (Variables|Default|GetMovingRateMultiplier) 0.02) false)
      (Pawn|Input|AddControllerYawInput (* (/ (* (- (Math|Vector|DotProduct (Math|Vector|Normalize (Math|Vector|MakeVector (stale Input|AxisEvents|InputAxisMoveLeft/Right AxisValue) (stale Input|AxisEvents|InputAxisMoveUp/Down AxisValue) 0.0)) (Math|Vector|Normalize (Math|Vector|MakeVector (stale Input|AxisEvents|InputAxisAnalogLeft/Right AxisValue) AxisValue 0.0))) 1.0) (select (== (select (== (Math|Float|Sign(Float) (stale Input|AxisEvents|InputAxisMoveUp/Down AxisValue)) 0.0) (Math|Float|Sign(Float) AxisValue) (Math|Float|Sign(Float) (stale Input|AxisEvents|InputAxisMoveUp/Down AxisValue))) 0.0) (select (== (Math|Float|Sign(Float) (stale Input|AxisEvents|InputAxisMoveLeft/Right AxisValue)) 0.0) (Math|Float|Sign(Float) (stale Input|AxisEvents|InputAxisAnalogLeft/Right AxisValue)) (Math|Float|Sign(Float) (stale Input|AxisEvents|InputAxisMoveLeft/Right AxisValue))) (select (== (Math|Float|Sign(Float) (stale Input|AxisEvents|InputAxisMoveUp/Down AxisValue)) 0.0) (Math|Float|Sign(Float) AxisValue) (Math|Float|Sign(Float) (stale Input|AxisEvents|InputAxisMoveUp/Down AxisValue))))) 8.0) (Variables|Default|GetTurningRateMultiplier))))))

(event Input|AxisEvents|InputAxisAnalogLeft/Right
  (params (AxisValue :type Float%20%28single-precision%29))
  (switch Utilities|FlowControl|Switch|SwitchonMovemode (Variables|Default|GetMovementMode)
    (:NewEnumerator1
      (if (> (Math|Vector|VectorLength (Math|Vector|Normalize (Math|Vector|MakeVector AxisValue (stale Input|AxisEvents|InputAxisAnalogUp/Down AxisValue) 0.0))) 0.0)
        (bind _output_get (Variables|Default|SetDirection (Math|Vector|Normalize (Math|Vector|MakeVector AxisValue (stale Input|AxisEvents|InputAxisAnalogUp/Down AxisValue) 0.0))))
        (Transformation|SetWorldRotation (Variables|Default|GetCenterRoot) (Class|KismetMathLibrary|RInterptoConstant (Transformation|GetWorldRotation (Variables|Default|GetCenterRoot)) (Math|Conversions|RotationFromXVector _output_get) (stale EventTick DeltaSeconds) (* (Variables|Default|GetTurningRateMultiplier) 1e+02)) false false)))
    (:NewEnumerator2
      (Pawn|Input|AddMovementInput (+ (Math|Vector|Normalize (Math|Vector|MakeVector (stale Input|AxisEvents|InputAxisMoveLeft/Right AxisValue) (stale Input|AxisEvents|InputAxisMoveUp/Down AxisValue) 0.0)) (Math|Vector|Normalize (Math|Vector|MakeVector AxisValue (stale Input|AxisEvents|InputAxisAnalogUp/Down AxisValue) 0.0))) (* (Math|Vector|VectorLength (+ (Math|Vector|Normalize (Math|Vector|MakeVector (stale Input|AxisEvents|InputAxisMoveLeft/Right AxisValue) (stale Input|AxisEvents|InputAxisMoveUp/Down AxisValue) 0.0)) (Math|Vector|Normalize (Math|Vector|MakeVector AxisValue (stale Input|AxisEvents|InputAxisAnalogUp/Down AxisValue) 0.0)))) (Variables|Default|GetMovingRateMultiplier) 0.02) false)
      (Pawn|Input|AddControllerYawInput (* (/ (* (- (Math|Vector|DotProduct (Math|Vector|Normalize (Math|Vector|MakeVector (stale Input|AxisEvents|InputAxisMoveLeft/Right AxisValue) (stale Input|AxisEvents|InputAxisMoveUp/Down AxisValue) 0.0)) (Math|Vector|Normalize (Math|Vector|MakeVector AxisValue (stale Input|AxisEvents|InputAxisAnalogUp/Down AxisValue) 0.0))) 1.0) (select (== (select (== (Math|Float|Sign(Float) (stale Input|AxisEvents|InputAxisMoveUp/Down AxisValue)) 0.0) (Math|Float|Sign(Float) (stale Input|AxisEvents|InputAxisAnalogUp/Down AxisValue)) (Math|Float|Sign(Float) (stale Input|AxisEvents|InputAxisMoveUp/Down AxisValue))) 0.0) (select (== (Math|Float|Sign(Float) (stale Input|AxisEvents|InputAxisMoveLeft/Right AxisValue)) 0.0) (Math|Float|Sign(Float) AxisValue) (Math|Float|Sign(Float) (stale Input|AxisEvents|InputAxisMoveLeft/Right AxisValue))) (select (== (Math|Float|Sign(Float) (stale Input|AxisEvents|InputAxisMoveUp/Down AxisValue)) 0.0) (Math|Float|Sign(Float) (stale Input|AxisEvents|InputAxisAnalogUp/Down AxisValue)) (Math|Float|Sign(Float) (stale Input|AxisEvents|InputAxisMoveUp/Down AxisValue))))) 8.0) (Variables|Default|GetTurningRateMultiplier))))))

(fn ConstructionScript
  (|CallParentFunction)
  (bind _output_get (Variables|Default|SetDistanceFromCenter (Math|Vector|Distance(Vector) "0, 0, 0" (Variables|/Script/Engine.SceneComponent|GetRelativeLocation (Variables|Default|GetcHero1)))))
  (Variables|Default|SetDistanceMultiplier _output_get)
  (Variables|Default|SetTurningRateMultiplier (Variables|Default|GetTurningRate))
  (Variables|Default|SetMovingRateMultiplier (Variables|Default|GetMovingRate))
  (Transformation|AttachComponentToComponent (Variables|Default|GetSpringArm) (Variables|Default|GetCapsuleComponent) "None" "KeepWorld" "KeepWorld" "KeepWorld" true)
  (Components|DestroyComponent (Variables|Default|GetCylinder)))

(fn SumRotationClamped
  (params (Add :type Float%20%28double-precision%29))
  (bind _output_get (Variables|Default|SetRotation (Math|Float|%(Float) (+ (Variables|Default|GetRotation) Add) 3.6e+02)))
  (return _output_get))