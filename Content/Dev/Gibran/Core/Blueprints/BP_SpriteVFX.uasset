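; BP_SpriteVFX is a short-lived Paper2D effect actor that shows a sprite or flipbook.
; Trigger events accept a sprite, a flipbook, or effect data directly or from a data table row.
; Effect data either plays timed flipbook steps in sequence or picks randomly, re-rolling per property read, with sound, transform and a global VFX event through the game mode.
; The actor removes itself by lifespan or when the sequence ends.
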(event Custom|TriggerEffect%28Sprite%29
  (params (Sprite :type Paper%20Sprite%20Object%20Reference) (Duration :type Float%20%28double-precision%29))
  (Rendering|Components|Sprite|SetSprite (Variables|Default|GetPaperSprite) Sprite)
  (Sprite|SetFlipbook (Variables|Default|GetPaperFlipbook))
  (Actor|SetLifeSpan Duration))

(event Custom|TriggerEffect%28Flipbook%29
  (params (Flipbook :type Paper%20Flipbook%20Object%20Reference) (TimeRate :type Float%20%28double-precision%29) (Looping :type Boolean))
  (bind _paperflipbook (Variables|Default|GetPaperFlipbook))
  (Components|Timeline|SetPlayRate _paperflipbook TimeRate)
  (Components|Timeline|SetLooping _paperflipbook Looping)
  (Sprite|SetFlipbook _paperflipbook Flipbook)
  (Sprite|SetSpriteColor (Variables|Default|GetPaperSprite) "(R=0.000000,G=0.000000,B=0.000000,A=0.000000)")
  (Actor|SetLifeSpan (Math|Float|Clamp(Float) (* (* (Class|PaperFlipbook|GetTotalDuration Flipbook) (/ 1.0 TimeRate)) 1.0) 0.01 1e+01)))

(event Custom|TriggerEffect%28DatatableRow%29
  (params (EffectDatatableRow :type Data%20Table%20Row%20Handle%20Structure))
  (bind (_datatable _rowname) (Utilities|Struct|BreakDataTableRowHandle EffectDatatableRow))
  (bind _returnvalue (Utilities|GetDataTableRow _datatable _rowname)
    (:then
      (CallFunction|TriggerEffect(Struct) _returnvalue))))

(event Custom|TriggerEffect%28Struct%29
  (params (EffectData :type S%20Sprite%20VFX%20Structure))
  (bind (_effectmode _effects) (Utilities|Struct|BreakS_SpriteVFX EffectData))
  (bind _paperflipbook (Variables|Default|GetPaperFlipbook))
  (bind _papersprite (Variables|Default|GetPaperSprite))
  (bind _paperflipbook_2 (Variables|Default|GetPaperFlipbook))
  (bind _outitem (Utilities|Array|Random _effects))
  (bind (_delaybeforenext _flipbook _sound _callvfxevent _relativetransform _looping) (Utilities|Struct|BreakS_SpriteVFXInstance _outitem))
  (switch Utilities|FlowControl|Switch|SwitchonE_SpriteVFXMode _effectmode
    (:NewEnumerator0
      (Variables|Default|SetFlipbookSequenceIndex 0)
      (if (Utilities|Array|IsValidIndex _effects (Variables|Default|GetFlipbookSequenceIndex)) :!label _label
        (Sprite|SetFlipbook (Variables|Default|GetPaperFlipbook) (.Flipbook (Utilities|Struct|BreakS_SpriteVFXInstance (Utilities|Array|Get(acopy) _effects (Variables|Default|GetFlipbookSequenceIndex)))))
        (Audio|PlaySoundatLocation (.Sound (Utilities|Struct|BreakS_SpriteVFXInstance (Utilities|Array|Get(acopy) _effects (Variables|Default|GetFlipbookSequenceIndex)))) (Transformation|GetActorLocation) "0, 0, 0" 1.0 1.0 0.0 0 0 0 0)
        (Default|CallGlobalVFXEvent (CallFunction|GetHeroesGameMode) self (.CallVFXEvent (Utilities|Struct|BreakS_SpriteVFXInstance (Utilities|Array|Get(acopy) _effects (Variables|Default|GetFlipbookSequenceIndex)))))
        (Transformation|SetRelativeTransform _papersprite (.RelativeTransform (Utilities|Struct|BreakS_SpriteVFXInstance (Utilities|Array|Get(acopy) _effects (Variables|Default|GetFlipbookSequenceIndex)))) false false)
        (Transformation|SetRelativeTransform _paperflipbook_2 (.RelativeTransform (Utilities|Struct|BreakS_SpriteVFXInstance (Utilities|Array|Get(acopy) _effects (Variables|Default|GetFlipbookSequenceIndex)))) false false)
        (Utilities|FlowControl|Delay (.DelayBeforeNext (Utilities|Struct|BreakS_SpriteVFXInstance (Utilities|Array|Get(acopy) _effects (Variables|Default|GetFlipbookSequenceIndex)))))
        (Math|Integer|IncrementInt (Variables|Default|GetFlipbookSequenceIndex)
          (:%20%20
            (goto _label)))
        (else
          (Actor|DestroyActor))))
    (:NewEnumerator1
      (Components|Timeline|SetLooping _paperflipbook _looping)
      (Sprite|SetFlipbook _paperflipbook _flipbook)
      (Audio|PlaySoundatLocation _sound (Transformation|GetActorLocation) "0, 0, 0" 1.0 1.0 0.0 0 0 0 0)
      (Default|CallGlobalVFXEvent (CallFunction|GetHeroesGameMode) self _callvfxevent)
      (Transformation|SetRelativeTransform _papersprite _relativetransform false false)
      (Transformation|SetRelativeTransform _paperflipbook_2 _relativetransform false false)
      (Actor|SetLifeSpan _delaybeforenext))))

(fn ConstructionScript)