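; Level generator that fills its Box bounds with a grid of Paper2D tilemap trees for a park.
; GenerateTrees clears earlier trees, then spawns flat-rotated tilemap actors at set spacing, with circular jitter and height rising per row plus slight randomness.
; Each tree gets a weighted random tilemap, optional random mirroring and a distortion or static material for animated leaves.
; Trees attach to the generator without collision or tick and are tracked for DeleteTrees.
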(event Custom|GenerateTrees
  (bind _box (Variables|Default|GetBox))
  (bind _distancebetweentrees (Variables|Default|GetDistanceBetweenTrees))
  (bind _distancebetweentrees_2 (Variables|Default|GetDistanceBetweenTrees))
  (bind (_origin _boxextent) (Collision|GetComponentBounds _box))
  (bind (_x _y) (Math|Vector|BreakVector _origin))
  (bind (_x_2 _y_2) (Math|Vector|BreakVector _boxextent))
  (CallFunction|DeleteTrees)
  (Variables|Default|SetOriginX (- _x (/ _x_2 1.0)))
  (Variables|Default|SetOriginY (- _y (/ _y_2 1.0)))
  (Variables|Default|SetNofTreesX (Math|Integer|Clamp(Integer) (.ReturnValue (Math|Float|Division(WholeandRemainder) (* _x_2 2.0) _distancebetweentrees_2)) 1 100))
  (Variables|Default|SetNofTreesY (Math|Integer|Clamp(Integer) (.ReturnValue (Math|Float|Division(WholeandRemainder) (* _y_2 2.0) _distancebetweentrees_2)) 1 100))
  (for _index (range 1 (Variables|Default|GetNofTreesY))
    (for _index_2 (range 1 (Variables|Default|GetNofTreesX))
      (bind _output_get (Variables|Default|SetNewTreeBaseLocation (Math|Vector|MakeVector (+ (Variables|Default|GetOriginX) (* _distancebetweentrees _index_2)) (+ (Variables|Default|GetOriginY) (* _distancebetweentrees _index)) (+ (+ (.z (Transformation|GetActorLocation)) (* (Variables|Default|GetMinHeightBetweenTrees) _index)) (Math|Random|RandomFloatinRange 1e+01 -1e+01)))))
      (bind _returnvalue (Game|SpawnActorfromClass "/Script/Paper2D.PaperTileMapActor" (Math|Transform|MakeTransform (CallFunction|RandomPointinCircle _output_get (Variables|Default|GetRandomDisplacement)) "0, 0,-90.000000" (Math|Vector|MakeVector (Math|Float|SelectFloat (Math|Float|SelectFloat 2.37 -2.37 (Math|Random|RandomBool)) 2.37 (Variables|Default|GetRandomFlipping)) 0.25 2.37)) "AlwaysSpawn" 0 0))
      (Transformation|AttachActorToActor _returnvalue self "None" "KeepWorld" "KeepWorld" "KeepWorld" true)
      (Class|PaperTileMapComponent|SetTileMap (Variables|/Script/Paper2D.PaperTileMapActor|GetRenderComponent _returnvalue) (Utilities|Array|Get(acopy) (Variables|Default|GetTreeTilemaps) (CallFunction|RandomWeightedInteger (Variables|Default|GetTilemapsWeights))))
      (Collision|SetActorEnableCollision _returnvalue false)
      (Utilities|Array|Add (Variables|Default|GetGeneratedTrees) _returnvalue)
      (Actor|Tick|SetActorTickEnabled _returnvalue)
      (if (Variables|Default|GetAnimatedLeaves)
        (Rendering|Material|SetMaterial (Variables|/Script/Paper2D.PaperTileMapActor|GetRenderComponent _returnvalue) 0 "/Game/Assets/Materials/M_SpriteMaterial_Distortion.M_SpriteMaterial_Distortion")
        (else
          (Rendering|Material|SetMaterial (Variables|/Script/Paper2D.PaperTileMapActor|GetRenderComponent _returnvalue) 0 "/Game/Assets/Materials/M_SpriteMaterial_NoDistortion.M_SpriteMaterial_NoDistortion"))))))

(event Custom|DeleteTrees
  (bind _generatedtrees (Variables|Default|GetGeneratedTrees))
  (for _array_element _generatedtrees
    (Actor|DestroyActor _array_element))
  (Utilities|Array|Clear _generatedtrees)
  (Utilities|Array|Resize _generatedtrees 0))

(fn ConstructionScript)