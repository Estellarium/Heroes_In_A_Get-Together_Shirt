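; Test actor for collision object types between itself and the projectiles it shoots.
; On BeginPlay it sets its mesh's object type, then loops every second, firing through BPShootingComponent and assigning each projectile's capsule object type and owner.
; Releasing Action 1 steps a MultiGate with no connected outputs, reset by a retriggerable delay after an input threshold.
; A disconnected branch holds unused flipbook attack-sequence logic.
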(event EventBeginPlay
  (Collision|SetCollisionObjectType (Variables|Default|GetStaticMesh) (Variables|Default|GetActorType))
  (Utilities|FlowControl|Delay 1.0 :!label _label)
  (bind _spawnedprojectiles (Default|FShootOnceProjectileClass (Variables|Default|GetBP_Shooting_Component)))
  (for _array_element _spawnedprojectiles
    (Collision|SetCollisionObjectType (Variables|/Game/Bin/Blueprints/Object/Projectiles/BP_Projectile.BP_Projectile_C|GetCapsule _array_element) (Variables|Default|GetProjectileType))
    (Variables|/Game/Bin/Blueprints/Object/Projectiles/BP_Projectile.BP_Projectile_C|SetOwnerRef _array_element self))
  (goto _label))

(event Input|ActionEvents|InputActionAction1
  (params (Key :type Key%20Structure :default "None"))
  (:Released
    (Utilities|FlowControl|Sequence
      (:then_0
        (Utilities|FlowControl|MultiGate false false -1 :!label _label))
      (:then_1
        (Utilities|FlowControl|RetriggerableDelay (Variables|Default|GetInputSequenceThreshold))
        (goto _label Reset)))))

(fn ConstructionScript)