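; Prototype test character that moves along its capsule's forward vector and uses left/right input to turn and reposition itself.
; Turning adds controller yaw and snaps the actor unswept to one of two side cylinders, with zero input counting as right.
; Overlaps on four collider components block the current turn direction; pushing into a block clears only the opposite one.
; Overlaps and hits print debug strings.
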(event OnComponentBeginOverlap(Coli4)
  (params (OverlappedComponent :type Primitive%20Component%20Object%20Reference) (OtherActor :type Actor%20Object%20Reference) (OtherComp :type Primitive%20Component%20Object%20Reference) (OtherBodyIndex :type Integer) (bFromSweep :type Boolean) (SweepResult :type Hit%20Result%20Structure%20%28by%20ref%29))
  (Development|PrintString (Utilities|GetDisplayName OtherActor) true true "(R=1.000000,G=0.000000,B=0.508881,A=1.000000)")
  (if (Variables|Default|GetMovingRight)
    (Variables|Default|SetBlockRight true)
    (elif (Variables|Default|GetMovingLeft)
      (Variables|Default|SetBlockLeft true))))

(event OnComponentBeginOverlap(Coli2)
  (params (OverlappedComponent :type Primitive%20Component%20Object%20Reference) (OtherActor :type Actor%20Object%20Reference) (OtherComp :type Primitive%20Component%20Object%20Reference) (OtherBodyIndex :type Integer) (bFromSweep :type Boolean) (SweepResult :type Hit%20Result%20Structure%20%28by%20ref%29))
  (Development|PrintString (Utilities|GetDisplayName OtherActor) true true "(R=1.000000,G=0.000000,B=0.508881,A=1.000000)")
  (if (Variables|Default|GetMovingRight)
    (Variables|Default|SetBlockRight true)
    (elif (Variables|Default|GetMovingLeft)
      (Variables|Default|SetBlockLeft true))))

(event OnComponentBeginOverlap(Capsule2)
  (params (OverlappedComponent :type Primitive%20Component%20Object%20Reference) (OtherActor :type Actor%20Object%20Reference) (OtherComp :type Primitive%20Component%20Object%20Reference) (OtherBodyIndex :type Integer) (bFromSweep :type Boolean) (SweepResult :type Hit%20Result%20Structure%20%28by%20ref%29))
  (Development|PrintString (Utilities|GetDisplayName OtherActor) true true "(R=1.000000,G=0.000000,B=0.508881,A=1.000000)")
  (if (Variables|Default|GetMovingRight)
    (Variables|Default|SetBlockRight true)
    (elif (Variables|Default|GetMovingLeft)
      (Variables|Default|SetBlockLeft true))))

(event OnComponentBeginOverlap(Capsule3)
  (params (OverlappedComponent :type Primitive%20Component%20Object%20Reference) (OtherActor :type Actor%20Object%20Reference) (OtherComp :type Primitive%20Component%20Object%20Reference) (OtherBodyIndex :type Integer) (bFromSweep :type Boolean) (SweepResult :type Hit%20Result%20Structure%20%28by%20ref%29))
  (Development|PrintString (Utilities|GetDisplayName OtherActor) true true "(R=1.000000,G=0.000000,B=0.508881,A=1.000000)")
  (if (Variables|Default|GetMovingRight)
    (Variables|Default|SetBlockRight true)
    (elif (Variables|Default|GetMovingLeft)
      (Variables|Default|SetBlockLeft true))))

(event OnComponentHit(Coli4)
  (params (HitComponent :type Primitive%20Component%20Object%20Reference) (OtherActor :type Actor%20Object%20Reference) (OtherComp :type Primitive%20Component%20Object%20Reference) (NormalImpulse :type Vector :default "0, 0, 0") (Hit :type Hit%20Result%20Structure%20%28by%20ref%29))
  (Development|PrintString "Hello"))

(event OnComponentHit(Coli2)
  (params (HitComponent :type Primitive%20Component%20Object%20Reference) (OtherActor :type Actor%20Object%20Reference) (OtherComp :type Primitive%20Component%20Object%20Reference) (NormalImpulse :type Vector :default "0, 0, 0") (Hit :type Hit%20Result%20Structure%20%28by%20ref%29))
  (Development|PrintString "Hello"))

(event OnComponentHit(Capsule2)
  (params (HitComponent :type Primitive%20Component%20Object%20Reference) (OtherActor :type Actor%20Object%20Reference) (OtherComp :type Primitive%20Component%20Object%20Reference) (NormalImpulse :type Vector :default "0, 0, 0") (Hit :type Hit%20Result%20Structure%20%28by%20ref%29))
  (Development|PrintString "Hello"))

(event OnComponentHit(Capsule3)
  (params (HitComponent :type Primitive%20Component%20Object%20Reference) (OtherActor :type Actor%20Object%20Reference) (OtherComp :type Primitive%20Component%20Object%20Reference) (NormalImpulse :type Vector :default "0, 0, 0") (Hit :type Hit%20Result%20Structure%20%28by%20ref%29))
  (Development|PrintString "Hello"))

(event Input|AxisEvents|InputAxisMoveLeft/Right
  (params (AxisValue :type Float%20%28single-precision%29))
  (if (>= AxisValue 0.0)
    (if (Variables|Default|GetBlockRight)
      (Variables|Default|SetBlockLeft false)
      (else
        (Variables|Default|SetMovingLeft false)
        (Variables|Default|SetMovingRight true)
        (Pawn|Input|AddControllerYawInput AxisValue)
        (bind _output_get (Variables|Default|SetTmpWorldLocation (Transformation|GetWorldLocation (Variables|Default|GetCylinder1))))
        (Transformation|SetActorLocation _output_get false false)))
    (elif (Variables|Default|GetBlockLeft)
      (Variables|Default|SetBlockRight false)
      (else
        (Variables|Default|SetMovingRight false)
        (Variables|Default|SetMovingLeft true)
        (Pawn|Input|AddControllerYawInput AxisValue)
        (bind _output_get_2 (Variables|Default|SetTmpWorldLocation (Transformation|GetWorldLocation (Variables|Default|GetCylinder))))
        (Transformation|SetActorLocation _output_get_2 false false)))))

(event Input|AxisEvents|InputAxisMoveUp/Down
  (params (AxisValue :type Float%20%28single-precision%29))
  (Pawn|Input|AddMovementInput (Math|Vector|GetForwardVector (Variables|Collision|GetCapsuleComponent)) AxisValue false))

(fn ConstructionScript)