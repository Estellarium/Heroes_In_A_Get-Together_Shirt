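; AccessibleTileMapActor is a tile map actor that exposes its RenderComponent's tile map, material and color to other code.
; Three events forward a new tile map, a material for element zero, or a color to the component.
; GetTileMap returns the component's current tile map, and the construction script is empty.
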(event EventSetTileMap
  (params (New%20Tile%20Map :type Paper%20Tile%20Map%20Object%20Reference))
  (Class|PaperTileMapComponent|SetTileMap (Variables|Default|GetRenderComponent) New%20Tile%20Map))

(event EventSetMaterial
  (params (New%20Material :type Material%20Interface%20Object%20Reference))
  (Rendering|Material|SetMaterial (Variables|Default|GetRenderComponent) 0 New%20Material))

(event EventSetColor
  (params (New%20Color :type Linear%20Color%20Structure))
  (Class|PaperTileMapComponent|SetTileMapColor (Variables|Default|GetRenderComponent) New%20Color))

(fn ConstructionScript)

(fn GetTileMap
  (return (Variables|/Script/Paper2D.PaperTileMapComponent|GetTileMap (Variables|Default|GetRenderComponent))))