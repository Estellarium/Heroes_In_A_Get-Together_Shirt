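; Bullet-hell game mode that spawns projectiles and tracks the live bullets.
; Projectiles spawn from a class or from a struct applied to an empty projectile, with an adjusted transform, and take their shooter as parent and its team before activating.
; Each spawn joins a list that destroys its oldest entry above MaxBullets, while death events remove and destroy bullets.
; A separate function toggles a debug mode flag.
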(event EventProjectileDied
  (params (Old%20Bullet :type BP%20Projectile%20Object%20Reference))
  (Utilities|IsValid Old%20Bullet
    (:Is%20Valid
      (Utilities|Array|RemoveItem (Variables|Default|GetAllBullets) Old%20Bullet)
      (Actor|DestroyActor Old%20Bullet))))

(event EventProjectileSpawned
  (params (New%20Bullet :type BP%20Projectile%20Object%20Reference))
  (bind _allbullets (Variables|Default|GetAllBullets))
  (bind _allbullets_2 (Variables|Default|GetAllBullets))
  (bind _output (Utilities|Array|Get(acopy) _allbullets_2))
  (Utilities|Array|AddUnique _allbullets New%20Bullet)
  (if (> (Utilities|Array|Length _allbullets) (Variables|Default|GetMaxBullets))
    (Utilities|IsValid _output
      (:Is%20Valid
        (Actor|DestroyActor _output))
      (:Is%20Not%20Valid
        _))
    (Utilities|Array|RemoveIndex _allbullets_2)))

(fn ConstructionScript)

(fn ToggleDebugMode
  (if (Variables|Default|GetDebugMode)
    (Variables|Default|SetDebugMode false)
    (else
      (Variables|Default|SetDebugMode true))))

(fn SpawnProjectilefromClass
  (params (Class :type BP%20Projectile%20Class%20Reference) (InitialTransform :type Transform) (Shooter :type Actor%20Object%20Reference))
  (bind _returnvalue (Game|SpawnActorfromClass Class (Math|Transform|ComposeTransforms InitialTransform (Variables|Default|GetModifySpawnTransform)) "AlwaysSpawn" 0 0))
  (bind _output_get (Variables|/Game/Bin/Blueprints/Object/Projectiles/BP_Projectile.BP_Projectile_C|SetParent _returnvalue Shooter))
  (bind _team (Class|BPIActorInteraction|GetTeam(Message) _output_get))
  (Variables|/Game/Bin/Blueprints/Object/Projectiles/BP_Projectile.BP_Projectile_C|SetTeam _returnvalue _team)
  (Default|Activate _returnvalue)
  (CallFunction|ProjectileSpawned _returnvalue)
  (return _returnvalue))

(fn SpawnProjectilefromStruct
  (params (Structure :type Struct%20Projectile%20Structure) (InitialTransform :type Transform) (Shooter :type Actor%20Object%20Reference))
  (bind _returnvalue (Game|SpawnActorfromClass "/Game/Bin/Blueprints/Object/Projectiles/BP_Projectile_Empty.BP_Projectile_Empty_C" (Math|Transform|ComposeTransforms InitialTransform (Variables|Default|GetModifySpawnTransform)) "AlwaysSpawn" 0 0))
  (bind _output_get (Variables|/Game/Bin/Blueprints/Object/Projectiles/BP_Projectile.BP_Projectile_C|SetParent _returnvalue Shooter))
  (bind _team (Class|BPIActorInteraction|GetTeam(Message) _output_get))
  (Variables|/Game/Bin/Blueprints/Object/Projectiles/BP_Projectile.BP_Projectile_C|SetTeam _returnvalue _team)
  (Default|SetVariables _returnvalue Structure)
  (Default|Activate _returnvalue)
  (CallFunction|ProjectileSpawned _returnvalue)
  (return _returnvalue))