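; BP_PickupBase is a base pickup actor that shows an item's sprite and gives that item to the heroes when interacted with.
; Construction and BeginPlay set the sprite from ItemData, which also supplies the localized name and icon for the interaction prompt.
; Interact calls an empty InteractionProcedure hook, then, unless the item name is None, adds ItemData to the heroes group inventory and destroys the pickup.
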(event Custom|InteractionProcedure)

(event EventBeginPlay
  (Rendering|Components|Sprite|SetSprite (Variables|Default|GetPickupSprite) (Utilities|Struct|BreakS_InventoryObject (Variables|Default|GetItemData)))
  (Variables|Default|SetHeroGroupRef (CallFunction|GetHeroesGroup)))

(event EventInteract
  (params (Instigator :type Actor%20Object%20Reference))
  (bind _itemdata (Variables|Default|GetItemData))
  (CallFunction|InteractionProcedure)
  (if (not (== (Utilities|Struct|BreakS_InventoryObject _itemdata) ""))
    (Utilities|Array|Add (Variables|/Game/Dev/Gibran/Core/Blueprints/Heroes/BP_HeroGroupRemake.BP_HeroGroupRemake_C|GetInventory (CallFunction|GetHeroesGroup)) _itemdata)
    (Actor|DestroyActor)))

(fn ConstructionScript
  (Rendering|Components|Sprite|SetSprite (Variables|Default|GetPickupSprite) (Utilities|Struct|BreakS_InventoryObject (Variables|Default|GetItemData))))

(fn GetInteractionPrompt
  (bind _itemdata (Variables|Default|GetItemData))
  (return (.locname _itemdata) (.icon _itemdata)))