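; BP_Prop is a prop actor drawn with a Paper2D tile map, with a Niagara petal effect.
; The construction script offsets the tile map from its dimensions and layers, then tints it.
; It feeds the petals height, radius, color and wind from a material parameter collection, then destroys that component.
; BeginPlay copies the tile map color to the petal effect.
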(event EventBeginPlay
  (Niagara|SetNiagaraVariable(LinearColor) (Variables|Default|GetNS_Petals) "Color" (Class|PaperTileMapComponent|GetTileMapColor (Variables|Default|GetPaperTileMap))))

(event Collision|EventActorBeginOverlap
  (params (OtherActor :type Actor%20Object%20Reference)))

(event EventTick
  (params (DeltaSeconds :type Float%20%28single-precision%29)))

(fn ConstructionScript
  (bind _papertilemap (Variables|Default|GetPaperTileMap))
  (bind _ns_petals (Variables|Default|GetNS_Petals))
  (bind _ns_petals_2 (Variables|Default|GetNS_Petals))
  (bind _color (Variables|Default|GetColor))
  (bind _returnvalue (Math|Conversions|ToLinearColor(Color) _color))
  (bind _tilemap (Variables|/Script/Paper2D.PaperTileMapComponent|GetTileMap _papertilemap))
  (bind _mapwidth (Variables|/Script/Paper2D.PaperTileMap|GetMapWidth _tilemap))
  (bind _tilewidth (Variables|/Script/Paper2D.PaperTileMap|GetTileWidth _tilemap))
  (bind _tileheight (Variables|/Script/Paper2D.PaperTileMap|GetTileHeight _tilemap))
  (bind _returnvalue_2 (Math|Conversions|ToFloat(Integer) _tileheight))
  (bind _returnvalue_3 (Math|Conversions|ToFloat(Integer) _tilewidth))
  (bind _returnvalue_4 (Math|Conversions|ToFloat(Integer) _mapwidth))
  (bind _returnvalue_5 (* _returnvalue_4 _returnvalue_3 -0.5))
  (Transformation|SetRelativeLocation (Variables|Default|GetPaperTileMap) (- (Math|Vector|MakeVector _returnvalue_5 0.0 (* (Math|Conversions|ToFloat(Integer) (Variables|/Script/Paper2D.PaperTileMap|GetMapHeight _tilemap)) _returnvalue_2)) (Math|Vector|MakeVector (/ _returnvalue_3 -2.0) (* (Variables|/Script/Paper2D.PaperTileMap|GetSeparationPerLayer _tilemap) (Utilities|Array|Length (Variables|/Script/Paper2D.PaperTileMap|GetTileLayers _tilemap)) -1.0) (/ _returnvalue_2 2.0))) false false)
  (Niagara|SetNiagaraVariable(Float) _ns_petals_2 "Height" (.z (Variables|/Script/Engine.SceneComponent|GetRelativeLocation (Variables|Default|GetPetalOrigin))))
  (Niagara|SetNiagaraVariable(Float) _ns_petals_2 "Radius" (Math|Float|Absolute(Float) _returnvalue_5))
  (bind _returnvalue_6 (Rendering|Material|GetVectorParameterValue "/Game/Assets/MPC_MaterialVariables.MPC_MaterialVariables" "WindDirectionStrength" :!class /Script/Engine.KismetMaterialLibrary))
  (Niagara|SetNiagaraVariable(Vector3) _ns_petals "Wind" (* (Math|Vector|Normalize (Math|Vector|MakeVector (.R (Math|Color|BreakColor _returnvalue_6)) (.G (Math|Color|BreakColor _returnvalue_6)) (.B (Math|Color|BreakColor _returnvalue_6)))) (.A (Math|Color|BreakColor _returnvalue_6))))
  (Niagara|SetNiagaraVariable(LinearColor) _ns_petals "Color" _returnvalue)
  (Class|PaperTileMapComponent|SetTileMapColor (Variables|Default|GetPaperTileMap) _returnvalue)
  (Components|DestroyComponent (Variables|Default|GetNS_Petals)))