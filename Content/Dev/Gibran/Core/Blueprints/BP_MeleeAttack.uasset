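; BP_MeleeAttack is a short-lived melee hitbox actor that damages and knocks back what it overlaps.
; TriggerAttack configures collision shape, profile, lifespan and damage from MeleeAttackData, plays a sound and spawns a BP_SpriteVFX effect from a struct or DataTable row.
; Overlaps with Hero, Enemy, Hero Shield or Destructible profiles send randomly varied damage with knockback directed away from the attack.
; Tick nudges the actor and mesh back and forth every frame.
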(event OnComponentBeginOverlap(CollisionMesh)
  (params (OverlappedComponent :type Primitive%20Component%20Object%20Reference) (OtherActor :type Actor%20Object%20Reference) (OtherComp :type Primitive%20Component%20Object%20Reference) (OtherBodyIndex :type Integer) (bFromSweep :type Boolean) (SweepResult :type Hit%20Result%20Structure%20%28by%20ref%29))
  (bind _returnvalue (Transformation|GetActorLocation OtherActor))
  (bind _defaultsceneroot (Variables|Default|GetDefaultSceneRoot))
  (bind _returnvalue_2 (Transformation|GetWorldLocation _defaultsceneroot))
  (bind _returnvalue_3 (Math|Rotator|FindLookatRotation _returnvalue_2 _returnvalue))
  (bind _returnvalue_4 (Math|Vector|GetForwardVector _returnvalue_3))
  (Development|PrintText (Utilities|Text|FormatText "attack direction: {ad}" (Utilities|Text|ToText(String) (Math|Vector|MakeVector (.x _returnvalue_4) (.y _returnvalue_4) 0.0))) true true "(R=0.000000,G=0.660000,B=1.000000,A=1.000000)" 2.0 "MeleeAttackDirection")
  (Development|PrintText (Utilities|Text|FormatText "Melee attack hit object of profile {pf} " (Collision|GetCollisionProfileName OtherComp)) true true "(R=1.000000,G=0.110224,B=0.000000,A=1.000000)" 5.0 "MeleeAttackHit")
  (switch name (Collision|GetCollisionProfileName OtherComp)
    (:Hero
      _)
    (:Enemy
      _)
    (:HeroShield
      _)
    (:Destructible
      _))
  (bind _output_get (Variables|Default|SetDisplacedDamage (CallFunction|ApplyRandomVariance (Variables|Default|GetBase%20Damage) (Variables|Default|GetDamage%20Variance))))
  (Class|BPIDamageableActor|TakeDamage(Message) OtherActor self 0 _output_get 2e+01 "NewEnumerator0" (Math|Vector|MakeVector (.x _returnvalue_4) (.y _returnvalue_4) 0.0)))

(event Custom|TriggerAttack
  (params (MeleeAttackData :type S%20Melee%20Attack%20Structure))
  (bind (_collisionshape _collisionprofile _duration _sound _effectsstruct _effectsdatatablerow _basedamage _damagevariance) (Utilities|Struct|BreakS_MeleeAttack MeleeAttackData))
  (bind _collisionmesh (Variables|Default|GetCollisionMesh))
  (Audio|PlaySoundatLocation _sound (Transformation|GetActorLocation) "0, 0, 0" 1.0 1.0 0.0 0 0 0 0)
  (Components|StaticMesh|SetStaticMesh _collisionmesh (Utilities|Select :Index _collisionshape :NewEnumerator0 "/Game/Dev/Gibran/TestAssets/Meshes/Coli1.Coli1" :NewEnumerator1 "/Game/Dev/Gibran/TestAssets/Meshes/Coli2.Coli2" :NewEnumerator2 "/Game/Dev/Gibran/TestAssets/Meshes/Coli5.Coli5" :NewEnumerator3 "/Game/Dev/Gibran/TestAssets/Meshes/Coli4.Coli4" :NewEnumerator4 "/Game/Dev/Gibran/TestAssets/Meshes/Coli3.Coli3"))
  (Collision|SetCollisionProfileName _collisionmesh _collisionprofile true :!class /Script/Engine.PrimitiveComponent)
  (Actor|SetLifeSpan _duration)
  (Development|PrintText (Utilities|Text|FormatText "Collision profile: {cp}" (Collision|GetCollisionProfileName (Variables|Default|GetCollisionMesh))))
  (Variables|Default|SetBase%20Damage _basedamage)
  (Variables|Default|SetDamage%20Variance _damagevariance)
  (bind _returnvalue (Game|SpawnActorfromClass "/Game/Dev/Gibran/Core/Blueprints/BP_SpriteVFX.BP_SpriteVFX_C" (Math|Transform|MakeTransform (Transformation|GetActorLocation) "0, 0,-90.000000" "1.000000,1.000000,1.000000") "AlwaysSpawn" 0 0))
  (if (Utilities|Array|IsEmpty (.Effects (Utilities|Struct|BreakS_SpriteVFX _effectsstruct)))
    (Default|TriggerEffect(DatatableRow) _returnvalue (Utilities|Struct|MakeDataTableRowHandle "/Game/Dev/Gibran/Core/DataTables/DT_SpriteVFXstructs.DT_SpriteVFXstructs" _effectsdatatablerow))
    (else
      (Default|TriggerEffect(Struct) _returnvalue _effectsstruct))))

(event EventBeginPlay)

(event EventTick
  (params (DeltaSeconds :type Float%20%28single-precision%29))
  (bind _collisionmesh (Variables|Default|GetCollisionMesh))
  (Utilities|FlowControl|FlipFlop
    (:A
      (Transformation|AddRelativeLocation _collisionmesh "1.000000, 0, 0" false false)
      (Transformation|AddActorLocalOffset "1.000000, 0, 0" false false))
    (:B
      (Transformation|AddRelativeLocation _collisionmesh "-1.000000, 0, 0" false false)
      (Transformation|AddActorLocalOffset "-1.000000, 0, 0" false false))))

(fn ConstructionScript)