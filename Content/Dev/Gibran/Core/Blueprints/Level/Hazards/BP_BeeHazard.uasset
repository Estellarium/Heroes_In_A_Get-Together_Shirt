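; A single bee hazard that roams around its beehive and damages heroes it touches.
; A looping timeline lerps it at random speeds from its current position to a random point within the hive's fly radius.
; A parallel delay loop randomly mirrors the sprite on X.
; Capsule overlaps with Hero-profile components deal random damage within a range looked up by current game difficulty.
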(event OnComponentBeginOverlap(Capsule)
  (params (OverlappedComponent :type Primitive%20Component%20Object%20Reference) (OtherActor :type Actor%20Object%20Reference) (OtherComp :type Primitive%20Component%20Object%20Reference) (OtherBodyIndex :type Integer) (bFromSweep :type Boolean) (SweepResult :type Hit%20Result%20Structure%20%28by%20ref%29))
  (bind _heroes_game_instance (CallFunction|GetHeroesGameInstance))
  (bind _beedamagemap (Variables|Default|GetBeeDamageMap))
  (bind _currentdifficulty (Variables|/Game/Dev/Gibran/Core/HeroesGameInstance.HeroesGameInstance_C|GetCurrentDifficulty _heroes_game_instance))
  (bind _value (Utilities|Map|Find (.damagevaluesperdifficulty _beedamagemap) _currentdifficulty))
  (bind (_basemindamage _basemaxdamage) (Utilities|Struct|BreakS_DamageDataValues _value))
  (switch name (Collision|GetCollisionProfileName OtherComp)
    (:Hero
      (Class|BPIDamageableActor|TakeDamage(Message) OtherActor self 0 (Math|Random|RandomFloatinRange _basemindamage _basemaxdamage) 0.0 "NewEnumerator0" "0, 0, 0"))))

(event EventBeginPlay
  (bind _beehiveref (Variables|Default|GetBeehiveRef))
  (bind _beesprite (Variables|Default|GetBeeSprite))
  (Utilities|FlowControl|Sequence
    (:then_0
      (Variables|Default|SetStartLocation (Transformation|GetActorLocation) :!label _label)
      (Variables|Default|SetTargetLocation (CallFunction|RandomPointinCircle (Transformation|GetWorldLocation (Variables|/Game/Dev/Gibran/Core/Blueprints/Level/Hazards/BP_BeehiveHazard.BP_BeehiveHazard_C|GetBeehiveSprite _beehiveref)) (Variables|/Game/Dev/Gibran/Core/Blueprints/Level/Hazards/BP_BeehiveHazard.BP_BeehiveHazard_C|GetBeesFlyRadius _beehiveref)))
      (Components|Timeline|SetPlayRate (Variables|Default|GetSpreadTimeline) (Math|Random|RandomFloatinRange 0.5 3.0))
      (bind _alpha (Timeline|SpreadTimeline PlayFromStart)
        (:Update
          (Transformation|SetActorLocation (Math|Vector|Lerp(Vector) (Variables|Default|GetStartLocation) (Variables|Default|GetTargetLocation) _alpha) false false))
        (:Finished
          (goto _label))))
    (:then_1
      (if (Math|Random|RandomBool) :!label _label_2
        (Transformation|SetRelativeScale3D _beesprite "1.000000,1.000000,1.000000")
        (else
          (Transformation|SetRelativeScale3D _beesprite "-1.000000,1.000000,1.000000")))
      (Utilities|FlowControl|Delay (Math|Random|RandomFloatinRange 0.1 2.0))
      (goto _label_2))))

(fn ConstructionScript)